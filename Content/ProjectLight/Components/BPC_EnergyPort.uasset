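; Energy port component that links its owning module to other ports and stores an energy volume clamped to a cap.
; Connections require an allowed connect state, a different port type and a matching energy type.
; Port priority comes from the owner's module type, and connected ports are kept in descending priority order through a midpoint-split insertion.
; Tick prints volume and connection count for debugging.
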(event `self.ReceiveBeginPlay`
  (bind _type (message `/Game/ProjectLight/Modules/BPI_Module.GetModuleType` (`self.GetOwner`)))
  (set `self.PortPriority` (`BlueprintMapLibrary.Map_Find` (`self.ModuleTypePriorities`) _type)))

(event `self.ReceiveTick`
  (params (DeltaSeconds :type "Float (single-precision)"))
  (`KismetSystemLibrary.PrintString` (`KismetStringLibrary.Concat_StrStr` (`KismetSystemLibrary.GetDisplayName` self) " " (`KismetStringLibrary.Conv_DoubleToString` (`self.CurrentVolume`)) " " (`KismetStringLibrary.Conv_IntToString` (`KismetArrayLibrary.Array_Length` (`self.ConnectedPorts`)))) true true (struct :`G` 0.66 :`B` 1.0 :`A` 1.0) 0.0))

(fn `ChangeEnergyVolume`
  (params (DeltaVolume :type "Float (double-precision)"))
  (set `self.CurrentVolume` (`KismetMathLibrary.FClamp` (+ (`self.CurrentVolume`) DeltaVolume) 0.0 (`self.VolumeCap`))))

(fn `ConnectError`)

(fn `ConnectStateIsOK`
  (params (OtherPort :type "/Game/ProjectLight/Components/BPC_EnergyPort Object Reference"))
  (returns (IsOK :type Boolean))
  (return (and (`|EnumInequality` (`self.ConnectState`) "NewEnumerator0") (not (`KismetArrayLibrary.Array_Contains` (`self.ConnectedPorts`) OtherPort)))))

(fn `LoseConnect`
  (params (OtherPort :type "/Game/ProjectLight/Components/BPC_EnergyPort Object Reference"))
  (bind _connectedports (`self.ConnectedPorts`))
  (if (`KismetArrayLibrary.Array_Contains` (`self.ConnectedPorts`) OtherPort)
    (`KismetArrayLibrary.Array_RemoveItem` _connectedports (`local.OtherPort`)))
  (if (`KismetArrayLibrary.Array_IsEmpty` _connectedports)
    (set `self.ConnectState` "NewEnumerator1")))

(fn `MakeConnect`
  (params (OtherPort :type "/Game/ProjectLight/Components/BPC_EnergyPort Object Reference"))
  (returns (ConncetSuccess :type Boolean))
  (if (and (`self.ConnectStateIsOK` OtherPort) (`|EnumInequality` (`self.PortType`) (`/Game/ProjectLight/Components/BPC_EnergyPort.PortType` OtherPort)) (`|EnumEquality` (`self.EnergyType`) (`/Game/ProjectLight/Components/BPC_EnergyPort.EnergyType` OtherPort)))
    (`self.RegisterNewPortToList` (`local.OtherPort`))
    (set `self.ConnectState` "NewEnumerator2")
    (return true)
    (else
      (return false))))

(fn `RegisterNewPortToList`
  (params (NewPort :type "/Game/ProjectLight/Components/BPC_EnergyPort Object Reference (by ref)"))
  (bind _connectedports (`self.ConnectedPorts`))
  (bind _connectedports_2 (`self.ConnectedPorts`))
  (bind _returnvalue (`KismetArrayLibrary.Array_Length` (`self.ConnectedPorts`)))
  (bind _portpriority (`/Game/ProjectLight/Components/BPC_EnergyPort.PortPriority` (`local.NewPort`)))
  (if (`KismetArrayLibrary.Array_IsEmpty` (`self.ConnectedPorts`))
    (`KismetArrayLibrary.Array_AddUnique` (`self.ConnectedPorts`) NewPort)
    (elif (>= _portpriority (`/Game/ProjectLight/Components/BPC_EnergyPort.PortPriority` (`|GetArrayItem` _connectedports)))
      (`KismetArrayLibrary.Array_Insert` (`self.ConnectedPorts`) (`local.NewPort`))
      (elif (<= _portpriority (`/Game/ProjectLight/Components/BPC_EnergyPort.PortPriority` (`|GetArrayItem` _connectedports (`KismetArrayLibrary.Array_LastIndex` _connectedports))))
        (`KismetArrayLibrary.Array_AddUnique` (`self.ConnectedPorts`) (`local.NewPort`))
        (elif (> (`/Game/ProjectLight/Components/BPC_EnergyPort.PortPriority` (`local.NewPort`)) (`/Game/ProjectLight/Components/BPC_EnergyPort.PortPriority` (`|GetArrayItem` _connectedports_2 (/ (`KismetArrayLibrary.Array_Length` _connectedports_2) 2))))
          ;[1 1 1] 大的话，从上往下查
          (for (_array_element _array_index) (`self.ConnectedPorts`)
            (if (>= (`/Game/ProjectLight/Components/BPC_EnergyPort.PortPriority` (`local.NewPort`)) (`/Game/ProjectLight/Components/BPC_EnergyPort.PortPriority` _array_element))
              (`KismetArrayLibrary.Array_Insert` (`self.ConnectedPorts`) (`local.NewPort`) _array_index)
              (break)))
          (else
            ;[1 1 1] 小的话，从中间开始查
            (for _index (range (/ _returnvalue 2) _returnvalue)
              (if (>= (`/Game/ProjectLight/Components/BPC_EnergyPort.PortPriority` (`local.NewPort`)) (`/Game/ProjectLight/Components/BPC_EnergyPort.PortPriority` (`|GetArrayItem` (`self.ConnectedPorts`) _index)))
                (`KismetArrayLibrary.Array_Insert` (`self.ConnectedPorts`) (`local.NewPort`) _index)
                (break)))))))))
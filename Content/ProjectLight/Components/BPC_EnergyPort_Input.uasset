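; Input energy port component, a child of a base port that adds the receiving side of energy transfer.
; Connecting binds its handler to the other port's energy-pass event once the parent connection succeeds, and disconnecting unbinds it, so passed volume feeds straight into ChangeEnergyVolume.
; A separate UDP-named event also changes the volume, but only when connection state and type allow receiving and the energy type matches.
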(event `/Game/ProjectLight/Components/Interfaces/BPI_Energy.EnergyPass_UDP`
  (params (EnergyInfo :type "/Game/ProjectLight/Components/Struct/FEnergyInfo Structure"))
  (bind (_type _volume) (break `/Game/ProjectLight/Components/Struct/FEnergyInfo` EnergyInfo))
  (if (`self.CanReceiveEnergy_UDP`)
    (if (`|EnumEquality` (`self.EnergyType`) _type)
      (`self.ChangeEnergyVolume` _volume))))

(fn `CanReceiveEnergy_UDP`
  (returns (CanReceive :type Boolean))
  (return (and (`|EnumInequality` (`self.ConnectState`) "NewEnumerator0") (`|EnumInequality` (`self.ConnectType`) "NewEnumerator0"))))

(fn `LoseConnect`
  (params (OtherPort :type "/Game/ProjectLight/Components/BPC_EnergyPort Object Reference"))
  (`parent.LoseConnect` OtherPort)
  (remove `self.OnConnectedEnergyPass` OtherPort (`|CreateDelegate` :!event `OnConnectedEnergyPassEvent`)))

(fn `MakeConnect`
  (params (OtherPort :type "/Game/ProjectLight/Components/BPC_EnergyPort Object Reference"))
  (returns (ConncetSuccess :type Boolean))
  (bind _conncetsuccess (`parent.MakeConnect` OtherPort))
  (if _conncetsuccess
    (add `self.OnConnectedEnergyPass` OtherPort (`|CreateDelegate` :!event `OnConnectedEnergyPassEvent`)))
  (return _conncetsuccess))

(fn `OnConnectedEnergyPassEvent`
  (params (Volume :type "Float (double-precision)"))
  (`self.ChangeEnergyVolume` Volume))
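; Actor component that gives a unit heat: received light raises it while living, and heat above the cap damages the owner.
; Base stats load from DT_HeatComponent by unit type, while curves over the heat-to-cap ratio scale light-to-heat and heat-to-damage conversion.
; Looping timers drive steady heat loss and, only while over the cap, damage.
; Assist effects edit a tag-keyed rate map, then recompute the heat cap.
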(event `self.ReceiveBeginPlay`
  (bind _unittype (message `/Game/ProjectLight/Blueprints/Interfaces/BPI_Common.GetUnitType` (`self.GetOwner`)))
  (bind _returnvalue (`|GetDataTableRow` "/Game/ProjectLight/Components/Data/DT_HeatComponent.DT_HeatComponent" (`KismetStringLibrary.Conv_StringToName` (`|GetEnumeratorNameAsString` _unittype)))
    (:`then`
      (`self.UpdateHeatComponentInfo` _returnvalue)
      (bind _returnvalue_2 (`KismetSystemLibrary.K2_SetTimerDelegate` (delegate `HeatLoss`) 0.1 true true))
      (set `self.HeatLossTimer` _returnvalue_2)
      (add `self.OnLightReceive` (`|CreateDelegate` :!event `ReceiveLight`))
      (add `self.OnHeatChange` (`|CreateDelegate` :!event `ChangeHeat`)))))

(event `HeatLoss`
  (`self.OnHeatChange` (* (`self.Rate_HeatLoss`) -0.1)))

(event `/Game/ProjectLight/Modules/InterfacesAndFunctions/BPI_AssistModule.ApplyAssistEffect`
  (params (AssistEffect :type "/Game/ProjectLight/Modules/Struct/FAssistEffectInfo Structure"))
  (`/Game/ProjectLight/Modules/InterfacesAndFunctions/BPL_AssistModule.ApplyAssist` AssistEffect (`self.AdjustRateMap`))
  (set `self.HeatCap` (`self.GetAttributeByTag` (struct :`TagName` "Component.Heat.HeatCap"))))

(event `/Game/ProjectLight/Modules/InterfacesAndFunctions/BPI_AssistModule.RemoveAssistEffect`
  (params (AssistEffect :type "/Game/ProjectLight/Modules/Struct/FAssistEffectInfo Structure"))
  (`/Game/ProjectLight/Modules/InterfacesAndFunctions/BPL_AssistModule.ApplyAssist` AssistEffect (`self.AdjustRateMap`) true)
  (set `self.HeatCap` (`self.GetAttributeByTag` (struct :`TagName` "Component.Heat.HeatCap"))))

(event `self.ReceiveTick`
  (params (DeltaSeconds :type "Float (single-precision)")))

(fn `ApplyDamageToOwner`
  (`GameplayStatics.ApplyDamage` (`self.GetOwner`) (* (`KismetMathLibrary.FClamp` (- (`self.CurrentHeat`) (`self.HeatCap`)) 0.0 10000.0) (`CurveFloat.GetFloatValue` (`self.Curve_HeatToDamage`) (/ (`self.CurrentHeat`) (`self.HeatCap`))))))

(fn `ChangeHeat`
  (params (Delta :type "Float (double-precision)"))
  (bind _damagetimer (`self.DamageTimer`))
  (bind _output_get (set `self.CurrentHeat` (`KismetMathLibrary.FClamp` (+ (`self.CurrentHeat`) Delta) 0.0 10000.0)))
  (if (> _output_get (`self.HeatCap`))
    (if (not (`KismetSystemLibrary.K2_IsValidTimerHandle` (`self.DamageTimer`)))
      (bind _returnvalue (`KismetSystemLibrary.K2_SetTimerDelegate` (`|CreateDelegate` :!event `ApplyDamageToOwner`) 0.1 true true))
      (set `self.DamageTimer` _returnvalue))
    (elif (`KismetSystemLibrary.K2_IsValidTimerHandle` _damagetimer)
      (`KismetSystemLibrary.K2_ClearAndInvalidateTimerHandle` _damagetimer))))

(fn `GetAttributeByTag`
  (params (AttributeTag :type "GameplayTag Structure"))
  (returns (AttributeReturn :type "Float (double-precision)"))
  (locals (AdjustRate_Local :type "Float (double-precision)"))
  (bind _adjustrate_local (`local.AdjustRate_Local`))
  (bind _adjustratemap (`self.AdjustRateMap`))
  (bind (_value _returnvalue) (`BlueprintMapLibrary.Map_Find` _adjustratemap AttributeTag))
  (set `local.AdjustRate_Local` _value)
  (if _returnvalue
    (`|SwitchGameplayTag` AttributeTag
      (:`Component.Heat.HeatCap`
        (return (* (`self.HeatCap`) _adjustrate_local)))
      (:`Component.Heat.LossRate`
        (return (* (`self.Rate_HeatLoss`) _adjustrate_local))))
    (else
      (`BlueprintMapLibrary.Map_Add` _adjustratemap AttributeTag 1.0)
      (return 1.0))))

(fn `ReceiveLight`
  (params (Volume :type "Float (double-precision)"))
  (bind _isliving (message `/Game/ProjectLight/Blueprints/Interfaces/BPI_Common.GetIsLiving` (`self.GetOwner`)))
  (if _isliving
    (`self.OnHeatChange` (* Volume (`CurveFloat.GetFloatValue` (`self.Curve_LightToHeat`) (/ (`self.CurrentHeat`) (`self.HeatCap`)))))))

(fn `UpdateHeatComponentInfo`
  (params (NewHeatComponentInfo :type "/Game/ProjectLight/Components/Struct/FHeatComponentInfo Structure"))
  (set `self.HeatCap` NewHeatComponentInfo_HeatCap_2_FE70B9E64FCC4C0DAE077089DE0BC890)
  (set `self.Rate_LightToHeat` NewHeatComponentInfo_Rate_LightToHeat_4_872D5CFB41D2FCA55F3B75A6EC2D5E1E)
  (set `self.Rate_HeatToDamage` NewHeatComponentInfo_Rate_HeatToDamage_6_F13E3F9E434E614789605F9BDC30193F)
  (set `self.Rate_HeatLoss` NewHeatComponentInfo_Rate_HeatLoss_8_6D76345344A733D60B6AE7830699814D))
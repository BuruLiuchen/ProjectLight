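; Output energy port component that pushes stored energy to connected ports at a set speed and interval.
; A looping timer starts on connect or open if a linked port is ready, and clears on close or last disconnect.
; SpreadEnergy serves eligible, non-full ports in list order from a per-interval budget, then deducts the amount given.
; When a receiver lacks room, CalVolumeToGive returns budget minus free space, not the free space.
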(fn `CalVolumeToGive`
  (params (TotalVolume :type "Float (double-precision)") (OtherPort :type "/Game/ProjectLight/Components/BPC_EnergyPort Object Reference"))
  (returns (EnergyToReceive :type "Float (double-precision)"))
  (locals (VolumeStorage :type "Float (double-precision)"))
  (bind _output_get (set `local.VolumeStorage` (- (`/Game/ProjectLight/Components/BPC_EnergyPort.VolumeCap` OtherPort) (`/Game/ProjectLight/Components/BPC_EnergyPort.CurrentVolume` OtherPort))))
  (if (>= _output_get (`local.TotalVolume`))
    (return (`local.TotalVolume`))
    (else
      (return (- (`local.TotalVolume`) (`local.VolumeStorage`))))))

(fn `ClosePort`
  (`parent.ClosePort`)
  (`KismetSystemLibrary.K2_ClearAndInvalidateTimerHandle` (`self.EnergySpreadTimer`)))

(fn `ConfirmTransportCondition`
  (params (OtherPort :type "/Game/ProjectLight/Components/BPC_EnergyPort Object Reference"))
  (returns (ReturnValue :type Boolean))
  (return (and (`|EnumEquality` (`/Game/ProjectLight/Components/BPC_EnergyPort.ConnectState` OtherPort) "NewEnumerator2") (not (`self.CurrentVolumeIsFull` OtherPort)))))

(fn `IsReadyToTransport`
  (returns (ReadyToTransport :type Boolean))
  (bind _connectedports (`self.ConnectedPorts`))
  (if (`KismetArrayLibrary.Array_IsNotEmpty` _connectedports)
    (for _array_element _connectedports
      (if (`|EnumEquality` (`/Game/ProjectLight/Components/BPC_EnergyPort.ConnectState` _array_element) "NewEnumerator2")
        (return true))))
  (return false))

(fn `LoseConnect`
  (params (OtherPort :type "/Game/ProjectLight/Components/BPC_EnergyPort Object Reference"))
  (bind _energyspreadtimer (`self.EnergySpreadTimer`))
  (`parent.LoseConnect` OtherPort)
  (if (`KismetArrayLibrary.Array_IsEmpty` (`self.ConnectedPorts`))
    (if (`KismetSystemLibrary.K2_IsValidTimerHandle` _energyspreadtimer)
      (`KismetSystemLibrary.K2_ClearAndInvalidateTimerHandle` _energyspreadtimer))))

(fn `MakeConnect`
  (params (OtherPort :type "/Game/ProjectLight/Components/BPC_EnergyPort Object Reference"))
  (returns (ConncetSuccess :type Boolean))
  (bind _conncetsuccess (`parent.MakeConnect` OtherPort))
  (if (not (`KismetSystemLibrary.K2_IsValidTimerHandle` (`self.EnergySpreadTimer`)))
    (`self.TryToStartEnergyTransport`))
  (return _conncetsuccess))

(fn `OnConncetStateChanged`
  (params (NewConnectState :type "/Game/ProjectLight/Components/Enum/EEnergyConnectState Enum" :default "NewEnumerator0"))
  (`parent.OnConncetStateChanged` NewConnectState))

(fn `OpenPort`
  (`parent.OpenPort`)
  (`self.TryToStartEnergyTransport`))

(fn `SpreadEnergy`
  (locals (VolumeToSpread :type "Float (double-precision)" :default 0.0) (RemainVolume :type "Float (double-precision)") (VolumeToGive :type "Float (double-precision)" :default 0.0))
  (bind (_energypassspeed _energypassinterval) (break `/Game/ProjectLight/CommonData/FEnergyPass` (`self.EnergyPassInfo`)))
  (bind _returnvalue (`KismetMathLibrary.FMin` (`self.CurrentVolume`) (* _energypassspeed _energypassinterval)))
  (if (not (`KismetArrayLibrary.Array_IsEmpty` (`self.ConnectedPorts`)))
    (set `local.VolumeToSpread` _returnvalue)
    (set `local.RemainVolume` _returnvalue)
    (for _array_element (`self.ConnectedPorts`)
      (if (`self.ConfirmTransportCondition` _array_element)
        (bind _output_get (set `local.VolumeToGive` (`self.CalVolumeToGive` (`local.RemainVolume`) _array_element)))
        (`self.ChangeEnergyVolume` _array_element _output_get)
        (bind _output_get_2 (set `local.RemainVolume` (`KismetMathLibrary.FClamp` (- (`local.RemainVolume`) (`local.VolumeToGive`)) 0.0 10000000.0)))
        (if (<= _output_get_2 0.0)
          (break))))
    (`self.ChangeEnergyVolume` (- (`local.RemainVolume`) (`local.VolumeToSpread`)))))

(fn `TryToStartEnergyTransport`
  (if (`self.IsReadyToTransport`)
    (bind _returnvalue (`KismetSystemLibrary.K2_SetTimerDelegate` (`|CreateDelegate` :!event `SpreadEnergy`) (`.EnergyPassInterval_5_E09C27724F5CB8BAEB93B6A4B60D5348` (break `/Game/ProjectLight/CommonData/FEnergyPass` (`self.EnergyPassInfo`))) true true))
    (set `self.EnergySpreadTimer` _returnvalue)))
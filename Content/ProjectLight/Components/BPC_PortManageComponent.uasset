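; Actor component that manages a unit's energy input and output ports and auto-links them to nearby units by proximity.
; Registered ports are sorted by direction and paired by energy type and connection state.
; Units with outputs get a runtime sense capsule, plus a one-shot trace for units already in range.
; Overlaps connect outputs to matching inputs on the other unit's port manager, and end overlaps call LoseConnect to break links.
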(event `OnSenseRangeBeginOverlap`
  (params (OverlappedComponent :type "PrimitiveComponent Object Reference") (OtherActor :type "Actor Object Reference") (OtherComp :type "PrimitiveComponent Object Reference") (OtherBodyIndex :type Integer) (bFromSweep :type Boolean) (SweepResult :type "HitResult Structure (by ref)"))
  (`self.TryConnectOtherUnit` OtherActor))

(event `OnSenseRangeEndOverlap`
  (params (OverlappedComponent :type "PrimitiveComponent Object Reference") (OtherActor :type "Actor Object Reference") (OtherComp :type "PrimitiveComponent Object Reference") (OtherBodyIndex :type Integer))
  (bind _returnvalue (`Actor.GetComponentByClass` OtherActor "BPC_PortManageComponent_C"))
  (for _array_element (`self.GetPortsHasConnected` "NewEnumerator1")
    (`/Engine/EditorBlueprintResources/StandardMacros.IsValid` _returnvalue
      (:`Is Valid`
        (for _array_element_2 (`self.GetPortsHasConnected` _returnvalue "NewEnumerator0")
          (`/Game/ProjectLight/Components/BPC_EnergyPort.LoseConnect` _array_element _array_element_2))))))

(event `self.ReceiveTick`
  (params (DeltaSeconds :type "Float (single-precision)")))

(fn `GetPortsByConnectType`
  (params (PortType :type "/Game/ProjectLight/Components/Enum/EEnergyPortType Enum" :default "NewEnumerator0") (ConnectType :type "/Game/ProjectLight/Components/Enum/EEnergyConnectType Enum" :default "NewEnumerator0"))
  (returns (SelectedPorts :type "Array of /Game/ProjectLight/Components/BPC_EnergyPort Object Reference"))
  (locals (PortsToReturn :type "Array of /Game/ProjectLight/Components/BPC_EnergyPort Object Reference"))
  (for _array_element (select `/Game/ProjectLight/Components/Enum/EEnergyPortType` PortType :`NewEnumerator0` (`self.InputPorts`) :`NewEnumerator1` (`self.Outputports`))
    (if (`|EnumEquality` (`local.ConnectType`) (`/Game/ProjectLight/Components/BPC_EnergyPort.ConnectType` _array_element))
      (`KismetArrayLibrary.Array_AddUnique` (`local.PortsToReturn`) _array_element)))
  (return (`local.PortsToReturn`)))

(fn `GetPortsByEnergyType`
  (params (PortType :type "/Game/ProjectLight/Components/Enum/EEnergyPortType Enum" :default "NewEnumerator0") (ConnectType :type "/Game/ProjectLight/Components/Enum/EEnergyConnectType Enum" :default "NewEnumerator0") (EnergyType :type "/Game/ProjectLight/Components/Enum/EEnergyType Enum" :default "NewEnumerator0"))
  (returns (SelectedPorts :type "Array of /Game/ProjectLight/Components/BPC_EnergyPort Object Reference"))
  (locals (PortsToReturn :type "Array of /Game/ProjectLight/Components/BPC_EnergyPort Object Reference"))
  (for _array_element (select `/Game/ProjectLight/Components/Enum/EEnergyPortType` PortType :`NewEnumerator0` (`self.InputPorts`) :`NewEnumerator1` (`self.Outputports`))
    (if (and (`|EnumEquality` (`local.ConnectType`) (`/Game/ProjectLight/Components/BPC_EnergyPort.ConnectType` _array_element)) (`|EnumEquality` (`local.EnergyType`) (`/Game/ProjectLight/Components/BPC_EnergyPort.EnergyType` _array_element)))
      (`KismetArrayLibrary.Array_AddUnique` (`local.PortsToReturn`) _array_element)))
  (return (`local.PortsToReturn`)))

(fn `GetPortsHasConnected`
  (params (PortType :type "/Game/ProjectLight/Components/Enum/EEnergyPortType Enum" :default "NewEnumerator0"))
  (returns (SelectedPorts :type "Array of /Game/ProjectLight/Components/BPC_EnergyPort Object Reference"))
  (locals (PortsToReturn :type "Array of /Game/ProjectLight/Components/BPC_EnergyPort Object Reference"))
  (for _array_element (select `/Game/ProjectLight/Components/Enum/EEnergyPortType` PortType :`NewEnumerator0` (`self.InputPorts`) :`NewEnumerator1` (`self.Outputports`))
    (`/Engine/EditorBlueprintResources/StandardMacros.IsValid` _array_element
      (:`Is Valid`
        (if (`|EnumEquality` (`/Game/ProjectLight/Components/BPC_EnergyPort.ConnectType` _array_element) "NewEnumerator0")
          (`KismetArrayLibrary.Array_AddUnique` (`local.PortsToReturn`) _array_element)))))
  (return (`local.PortsToReturn`)))

(fn `SenseOtherPortOnce`
  (bind _buildingsenserange (`self.BuildingSenseRange`))
  (bind _returnvalue (`Actor.K2_GetActorLocation` (`self.GetOwner`)))
  (bind _outhits (`KismetSystemLibrary.CapsuleTraceMultiForObjects` _returnvalue _returnvalue _buildingsenserange (+ _buildingsenserange 50.0) (`|MakeArray` "ObjectTypeQuery2" "ObjectTypeQuery3" :!type "EObjectTypeQuery Enum")))
  (if (`KismetArrayLibrary.Array_IsNotEmpty` _outhits)
    (for _array_element _outhits
      (`self.TryConnectOtherUnit` (`.HitActor` (`GameplayStatics.BreakHitResult` _array_element))))))

(fn `TryConnectOtherUnit`
  (params (OtherUnit :type "Actor Object Reference"))
  (bind _returnvalue (`Actor.GetComponentByClass` OtherUnit "BPC_PortManageComponent_C"))
  (for _array_element (`self.GetPortsByConnectType` "NewEnumerator1")
    (`/Engine/EditorBlueprintResources/StandardMacros.IsValid` _returnvalue
      (:`Is Valid`
        (bind _selectedports (`self.GetPortsByEnergyType` _returnvalue "NewEnumerator0" "NewEnumerator0" (`/Game/ProjectLight/Components/BPC_EnergyPort.EnergyType` _array_element)))
        (if (`KismetArrayLibrary.Array_IsNotEmpty` _selectedports)
          (for _array_element_2 _selectedports
            (`/Game/ProjectLight/Components/BPC_EnergyPort.MakeConnect` _array_element _array_element_2)))))))

(fn `UpdatePortsInfo`
  (params (EnergyPort :type "/Game/ProjectLight/Components/BPC_EnergyPort Object Reference"))
  (locals (EnergyType :type "/Game/ProjectLight/Components/Enum/EEnergyType Enum" :default "NewEnumerator0") (NewLocalVar :type "/Game/ProjectLight/Components/BPC_EnergyPort Object Reference"))
  (bind _energyport (`local.EnergyPort`))
  (bind _energyport_2 (`local.EnergyPort`))
  (set `local.EnergyType` (`/Game/ProjectLight/Components/BPC_EnergyPort.EnergyType` EnergyPort))
  (switch `/Game/ProjectLight/Components/Enum/EEnergyPortType` (`/Game/ProjectLight/Components/BPC_EnergyPort.PortType` EnergyPort)
    (:`NewEnumerator0`
      (`KismetArrayLibrary.Array_AddUnique` (`self.InputPorts`) (`local.EnergyPort`))
      (for _array_element (`self.GetPortsByEnergyType` "NewEnumerator1" "NewEnumerator0" (`local.EnergyType`))
        (if (!= (`self.GetOwner` _array_element) (`self.GetOwner` _energyport))
          (`/Game/ProjectLight/Components/BPC_EnergyPort.MakeConnect` _energyport _array_element))))
    (:`NewEnumerator1`
      (`KismetArrayLibrary.Array_AddUnique` (`self.Outputports`) (`local.EnergyPort`))
      (for _array_element_2 (`self.GetPortsByEnergyType` "NewEnumerator0" "NewEnumerator0" (`local.EnergyType`))
        (if (!= (`self.GetOwner` _array_element_2) (`self.GetOwner` _energyport_2))
          (`/Game/ProjectLight/Components/BPC_EnergyPort.MakeConnect` _energyport_2 _array_element_2))))))

(fn `UpdateSenseRange`
  (params (SenseRange :type "Float (double-precision)"))
  (bind _output_get (set `self.BuildingSenseRange` SenseRange))
  (`/Engine/EditorBlueprintResources/StandardMacros.IsValid` (`self.SenseRange`)
    (:`Is Valid`
      (`CapsuleComponent.SetCapsuleRadius` (`self.SenseRange`) _output_get true))
    (:`Is Not Valid`
      (if (`KismetArrayLibrary.Array_IsNotEmpty` (`self.Outputports`))
        (bind _returnvalue (`|AddComponentByClass` :`self` (`self.GetOwner`) :`Class` "/Script/Engine.CapsuleComponent"))
        (`CapsuleComponent.SetCapsuleHalfHeight` _returnvalue 1000.0 true)
        (`CapsuleComponent.SetCapsuleRadius` _returnvalue _output_get true)
        (bind _output_get_2 (set `self.SenseRange` _returnvalue))
        (`PrimitiveComponent.SetCollisionProfileName` _output_get_2 "EnergyConnect" true)
        (add `PrimitiveComponent.OnComponentBeginOverlap` _output_get_2 (`|CreateDelegate` :!event `OnSenseRangeBeginOverlap`))
        (add `PrimitiveComponent.OnComponentEndOverlap` _output_get_2 (`|CreateDelegate` :!event `OnSenseRangeEndOverlap`))
        (`self.SenseOtherPortOnce`)))))
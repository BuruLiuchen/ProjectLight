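; Base building actor that loads stats and modules from a data table, previews placement, builds over time, then joins the battle stage unit list.
; Modules attach by type sockets, can be installed or removed, and assist effects scale attributes such as max health.
; Received light boots or shuts down modules, while losing it starts recurring dark damage.
; It also handles resource-paid auto-repair, upgrades that carry over storage, and an info panel.
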(event `self.ReceiveBeginPlay`
  (`self.InitBuilding`)
  (`PrimitiveComponent.SetCollisionProfileName` (`self.Capsule`) "PreviewBuilding" true)
  (for _array_element (`self.AttachedModules`)
    (`/Game/ProjectLight/Modules/BP_Module_Base.RegisterModule` _array_element self))
  (`self.StartPreview`))

(event `BuildConfirm`
  (set `self.BuildProgress` 0.0)
  (`PrimitiveComponent.SetCollisionProfileName` (`self.Capsule`) "Building" true)
  (bind _returnvalue (`KismetSystemLibrary.K2_SetTimerDelegate` (delegate `Build`) (`self.BuildProcessInterval`) true true))
  (set `self.BuildTimer` _returnvalue))

(event `Build`
  (`self.BuildProcess`))

(event `BuildComplete`
  (`self.EndPreview`)
  (`PrimitiveComponent.SetCollisionProfileName` (`self.Capsule`) "Building" true)
  (set `self.IsLiving` true)
  (bind _asgm_battle_stage (cast `/Game/ProjectLight/BattleScene/GM_BattleStage` (`GameplayStatics.GetGameMode`)))
  (`/Game/ProjectLight/BattleScene/GM_BattleStage.RegisterToUnitList` _asgm_battle_stage self)
  (`KismetSystemLibrary.Delay` 0.2)
  (`self.InitMotionAndAssist`)
  (`/Game/ProjectLight/Components/BPC_PortManageComponent.UpdateSenseRange` (`self.BPC_PortManageComponent`) (`self.ConnectRange`))
  (if (`self.IsActive`)
    (`self.Boot`)
    (else
      (`self.ShutDown`)))
  (bind _buildinginfopanel (`self.BuildingInfoPanel`)
    (:`then`
      (`/Game/ProjectLight/UMG/Items/UMG_BuildingInfo_Window.CreateEquipmentSlots` _buildinginfopanel))
    (:`else`
      (bind _returnvalue (`|CreateWidget` "/Game/ProjectLight/UMG/Items/UMG_BuildingInfo_Window.UMG_BuildingInfo_Window_C"))
      (`/Game/ProjectLight/UMG/Items/UMG_BuildingInfo_Window.SetBuildingActor` _returnvalue self)
      (`WidgetComponent.SetWidget` (`self.Widget`) _returnvalue)
      (bind _output_get (set `self.BuildingInfoPanel` _returnvalue))
      (`Widget.SetVisibility` _output_get "Collapsed"))))

(event `self.ReceiveAnyDamage`
  (params (Damage :type "Float (single-precision)") (DamageType :type "DamageType Object Reference") (InstigatedBy :type "Controller Object Reference") (DamageCauser :type "Actor Object Reference"))
  (bind _output_get (set `self.HealthPoint` (`KismetMathLibrary.FClamp` (- (`self.HealthPoint`) Damage) 0.0 (`self.MaxHealthPoint`))))
  (if (<= _output_get 0.0)
    (`self.BuildingDie`)
    (else
      (`self.TryToStartRecovery`))))

(event `BuildingDie`
  (`self.K2_DestroyActor`))

(event `TryToStartRecovery`
  (bind _recoverytimer (`self.RecoveryTimer`))
  (`KismetSystemLibrary.K2_SetTimerDelegate` (delegate `StartRecovery`) (`self.RecoveryStartTime`))
  (if (`KismetSystemLibrary.K2_IsValidTimerHandle` _recoverytimer)
    (`KismetSystemLibrary.K2_ClearAndInvalidateTimerHandle` _recoverytimer)))

(event `self.ReceiveEndPlay`
  (params (EndPlayReason :type "EEndPlayReason Enum" :default "Destroyed"))
  (bind _darkdamagetimer (`self.DarkDamageTimer`))
  (for _array_element (`self.AttachedModules`)
    (`/Engine/EditorBlueprintResources/StandardMacros.IsValid` _array_element
      (:`Is Valid`
        (`self.K2_DestroyActor` _array_element))))
  (if (`KismetSystemLibrary.K2_IsValidTimerHandle` _darkdamagetimer)
    (`KismetSystemLibrary.K2_ClearAndInvalidateTimerHandle` _darkdamagetimer)))

(event `StartRecovery`
  (if (and (`self.AutoRecovery`) (< (`self.HealthPoint`) (`self.MaxHealthPoint`)))
    (bind _returnvalue (`KismetSystemLibrary.K2_SetTimerDelegate` (delegate `KeepRecovery`) 0.5 true true))
    (set `self.RecoveryTimer` _returnvalue)
    (else
      (`self.StopRecovery`))))

(event `KeepRecovery`
  (bind _resourcecomponent (`/Game/ProjectLight/Blueprints/FunctionLibrary/BML_Common.GetResourceComponent` (`GameplayStatics.GetPlayerCharacter` 0))
    (:`IsValid`
      (bind _consumesucess (`/Game/ProjectLight/Characters/Components/BPC_ResourceComponent.ConsumeStorageValue` _resourcecomponent "NewEnumerator2" 0.5))
      (if _consumesucess
        (bind _output_get (set `self.HealthPoint` (`KismetMathLibrary.FClamp` (+ (`self.HealthPoint`) 1.0) 0.0 (`self.MaxHealthPoint`))))
        (if (>= _output_get (`self.MaxHealthPoint`))
          (`self.StopRecovery`))))))

(event `/Game/ProjectLight/Blueprints/Interfaces/BPI_Common.OpenBuildingInfo`
  (`SceneComponent.SetVisibility` (`self.Widget`) true false)
  (bind _buildinginfopanel (`self.BuildingInfoPanel`)
    (:`then`
      (`/Game/ProjectLight/UMG/Items/UMG_BuildingInfo_Window.UpdateBuildingInfo` _buildinginfopanel)
      (`Widget.SetVisibility` _buildinginfopanel "Visible"))
    (:`else`)))

(event `/Game/ProjectLight/Blueprints/Interfaces/BPI_Common.CloseBuildingInfo`
  (`SceneComponent.SetVisibility` (`self.Widget`) false false)
  (bind _buildinginfopanel (`self.BuildingInfoPanel`)
    (:`then`
      (`Widget.SetVisibility` _buildinginfopanel "Collapsed"))
    (:`else`)))

(event `self.Capsule.OnComponentBeginOverlap`
  (params (OverlappedComponent :type "PrimitiveComponent Object Reference") (OtherActor :type "Actor Object Reference") (OtherComp :type "PrimitiveComponent Object Reference") (OtherBodyIndex :type Integer) (bFromSweep :type Boolean) (SweepResult :type "HitResult Structure (by ref)"))
  (if (and (!= OtherActor self) (`self.IsPreview`))
    (bind _buildcomponent (`/Game/ProjectLight/Blueprints/FunctionLibrary/BML_Common.GetBuildComponent` (`GameplayStatics.GetPlayerCharacter` 0))
      (:`IsValid`
        (`/Game/ProjectLight/Characters/Components/BPC_BuildComponent.SetOverlapedActors` _buildcomponent OtherActor false)))))

(event `self.Capsule.OnComponentEndOverlap`
  (params (OverlappedComponent :type "PrimitiveComponent Object Reference") (OtherActor :type "Actor Object Reference") (OtherComp :type "PrimitiveComponent Object Reference") (OtherBodyIndex :type Integer))
  (if (and (!= (stale `self.Capsule.OnComponentBeginOverlap` OtherActor) self) (`self.IsPreview`))
    (bind _buildcomponent (`/Game/ProjectLight/Blueprints/FunctionLibrary/BML_Common.GetBuildComponent` (`GameplayStatics.GetPlayerCharacter` 0))
      (:`IsValid`
        (`/Game/ProjectLight/Characters/Components/BPC_BuildComponent.SetOverlapedActors` _buildcomponent OtherActor true)))))

(event `/Game/ProjectLight/Components/Interfaces/BPI_Energy.EnergyPass_UDP`
  (params (EnergyInfo :type "/Game/ProjectLight/Components/Struct/FEnergyInfo Structure") (EnergySourceType :type "/Game/ProjectLight/Components/Enum/EEnergySourceType Enum" :default "NewEnumerator0"))
  (bind (_type _volume) (break `/Game/ProjectLight/Components/Struct/FEnergyInfo` EnergyInfo))
  (if (and (`|EnumEquality` _type "NewEnumerator0") (>= _volume (`self.MinLightRequest`)))
    (`/Game/ProjectLight/Blueprints/FunctionLibrary/BPL_Energy.ReceiveLight` self _volume)
    (`self.SetLightTakenNetural` (`|EnumEquality` EnergySourceType "NewEnumerator0"))
    (bind _returnvalue (`KismetSystemLibrary.K2_SetTimerDelegate` (delegate `ChangeLightState`) 5.0 false true))
    (set `self.LightCheckTimer` _returnvalue)
    (`self.LightTakenChange` true)
    (`/Game/ProjectLight/Blueprints/FunctionLibrary/BPL_Common.PauseTimer` (`self.DarkDamageTimer`) self)))

(event `ChangeLightState`
  (`self.LightTakenChange` false)
  (`self.NoLightTaken`))

(event `DarkDamage`
  (`/Game/ProjectLight/Blueprints/FunctionLibrary/BPL_Common.ApplyDarkDamage` self))

(event `/Game/ProjectLight/Modules/InterfacesAndFunctions/BPI_AssistModule.ApplyAssistEffect`
  (params (AssistEffect :type "/Game/ProjectLight/Modules/Struct/FAssistEffectInfo Structure"))
  (`/Game/ProjectLight/Modules/InterfacesAndFunctions/BPL_AssistModule.ApplyAssist` AssistEffect (`self.AdjustRateMap`))
  (`self.UpdateAssistEffect`))

(event `/Game/ProjectLight/Modules/InterfacesAndFunctions/BPI_AssistModule.RemoveAssistEffect`
  (params (AssistEffect :type "/Game/ProjectLight/Modules/Struct/FAssistEffectInfo Structure"))
  (`/Game/ProjectLight/Modules/InterfacesAndFunctions/BPL_AssistModule.ApplyAssist` AssistEffect (`self.AdjustRateMap`) true)
  (`self.UpdateAssistEffect`))

(fn `Boot`
  (locals (Module_Local :type "/Game/ProjectLight/Modules/BP_Module_Base Object Reference"))
  (if (`self.IsActive`)
    (if (`self.LightTaken_Netural`)
      (for _array_element (`self.AttachedModules`) :!label _label
        (set `local.Module_Local` _array_element)
        (bind _module_local (`local.Module_Local`)
          (:`then`
            (bind _moduletype (`/Game/ProjectLight/Modules/BP_Module_Base.ModuleType` _module_local))
            (if (`|EnumEquality` _moduletype "NewEnumerator4")
              _
              (elif (and (`|EnumEquality` _moduletype "NewEnumerator3") (`self.LightTaken_Netural`) (not (`/Game/ProjectLight/Modules/BP_Module_Base.ManualControll` _module_local)))
                (bind _module_local_2 (`local.Module_Local`)
                  (:`then`
                    (`/Game/ProjectLight/Modules/BP_Module_Base.CloseModule` _module_local_2))
                  (:`else`))
                (else
                  (bind _module_local_3 (`local.Module_Local`)
                    (:`then`
                      (`/Game/ProjectLight/Modules/BP_Module_Base.OpenModule` _module_local_3))
                    (:`else`))))))
          (:`else`)))
      (else
        (for _array_element_2 (`self.AttachedModules`)
          (if (and (`|EnumEquality` (`/Game/ProjectLight/Modules/BP_Module_Base.ModuleType` _array_element_2) "NewEnumerator3") (not (`/Game/ProjectLight/Modules/BP_Module_Base.ManualControll` _array_element_2)))
            (`/Game/ProjectLight/Modules/BP_Module_Base.OpenModule` _array_element_2)))))
    (else
      (set `self.IsActive` true)
      (goto _label))))

(fn `BuildProcess`
  (bind _output_get (set `self.BuildProgress` (+ (`self.BuildProgress`) (`self.BuildProcessInterval`))))
  (`self.PreviewStateChange` (/ _output_get (`.BuildTime_19_C1D51BA0490E9CB13D553D808D757649` (break `/Game/ProjectLight/Buildings/Struct/FBuildingInfo` (`self.BuildingInfo`)))))
  (if (>= _output_get (`.BuildTime_19_C1D51BA0490E9CB13D553D808D757649` (break `/Game/ProjectLight/Buildings/Struct/FBuildingInfo` (`self.BuildingInfo`))))
    (`KismetSystemLibrary.K2_ClearAndInvalidateTimerHandle` (`self.BuildTimer`))
    (`self.BuildComplete`)))

(fn `ChangeMaxHealth`
  (params (NewMaxHealth :type "Float (double-precision)") (ResetHealth :type Boolean))
  (bind _output_get (set `self.MaxHealthPoint` NewMaxHealth))
  (if ResetHealth
    (set `self.HealthPoint` (`self.MaxHealthPoint`))
    (else
      (bind _output_get_2 (set `self.HealthPoint` (`KismetMathLibrary.FMin` _output_get (`self.HealthPoint`))))
      (if (< _output_get_2 (`self.MaxHealthPoint`))
        (`self.TryToStartRecovery`)))))

(fn `EndPreview`
  (for (_array_element _array_index) (`self.DefaultMaterials`)
    (`PrimitiveComponent.SetMaterial` (`self.StaticMesh`) _array_index _array_element))
  (for _array_element_2 (`self.AttachedModules`)
    (`/Game/ProjectLight/Modules/BP_Module_Base.EndPreview` _array_element_2))
  (set `self.IsPreview` false))

(fn `GetAttributeByTag`
  (params (AttributeTag :type "GameplayTag Structure"))
  (returns (AttributeReturn :type "Float (double-precision)"))
  (locals (AdjustRate_Local :type "Float (double-precision)"))
  (bind _adjustrate_local (`local.AdjustRate_Local`))
  (bind _adjustratemap (`self.AdjustRateMap`))
  (bind (_value _returnvalue) (`BlueprintMapLibrary.Map_Find` _adjustratemap AttributeTag))
  (set `local.AdjustRate_Local` _value)
  (if (not _returnvalue)
    (`BlueprintMapLibrary.Map_Add` _adjustratemap AttributeTag 1.0)
    (set `local.AdjustRate_Local` 1.0))
  (`|SwitchGameplayTag` AttributeTag
    (:`Unit.Base.MaxHealth`
      (return (* (`self.MaxHealthPoint`) _adjustrate_local)))
    (:`Building.Base.ConnectRange`
      (return (* (`self.ConnectRange`) _adjustrate_local)))))

(fn `GetBuildingType`
  (returns (BuildingType :type "/Game/ProjectLight/Buildings/EBuildingType Enum"))
  (return (`self.BuildingType`)))

(fn `GetIsActive`
  (returns (IsActive :type Boolean))
  (return (`self.IsActive`)))

(fn `GetIsLiving`
  (returns (IsLiving :type Boolean))
  (return (`self.IsLiving`)))

(fn `GetName`
  (returns (ReturnName :type Name))
  (return (`self.BuildingName`)))

(fn `GetUnitType`
  (returns (UnitType :type "/Game/ProjectLight/Blueprints/Enums/EUnitType Enum"))
  (return "NewEnumerator2"))

(fn `GetVolumeForDispaly`
  (returns (Volume :type "Float (double-precision)") (MaxVolume :type "Float (double-precision)"))
  (return (`self.HealthPoint`) (`self.MaxHealthPoint`)))

(fn `InitBuilding`
  (bind _returnvalue (`|GetDataTableRow` (`self.BuildingData`) (`self.BuildingName`))
    (:`then`
      (bind _output_get (set `self.BuildingInfo` _returnvalue))
      (bind (_displayname _buildingtype _size _maxhealthpoint _assistmodulelimit _attachedmodules _connectrange) (break `/Game/ProjectLight/Buildings/Struct/FBuildingInfo` _output_get))
      (`self.ChangeMaxHealth` _maxhealthpoint true)
      (set `self.BuildingType` _buildingtype)
      (set `self.ConnectRange` _connectrange)
      (set `self.AssistModuleLimit` _assistmodulelimit)
      (for (_array_element _array_index) _attachedmodules
        (bind _spawnedmodule (`self.SpawnModuleActor` _array_element _array_index))
        (bind _asbp_module_storage (cast `/Game/ProjectLight/Modules/BP_Module_Storage` _spawnedmodule))
        (bind (_value _returnvalue_2) (`BlueprintMapLibrary.Map_Find` (`self.TempStorage`) (`/Game/ProjectLight/Blueprints/FunctionLibrary/BPL_Common.GetUnitNameAndLevel` (`KismetStringLibrary.Conv_NameToString` (`/Game/ProjectLight/Modules/BP_Module_Base.ModuleName` _asbp_module_storage)))))
        (if _returnvalue_2
          (`/Game/ProjectLight/Modules/BP_Module_Storage.ChangeStorage` _asbp_module_storage _value))))))

(fn `InitMotionAndAssist`
  (bind _assistmodules (`self.AssistModules`))
  (`|ExecutionSequence`
    (:`then_0`
      (bind _module_motion (`self.Module Motion`)
        (:`then`
          (for _array_element (`self.AttachedModules`)
            (if (!= _array_element _module_motion)
              (`|ExecutionSequence`
                (:`then_0`
                  (`self.K2_AttachToComponent` _array_element (`/Game/ProjectLight/Modules/BP_Module_Base.StaticMesh` (`self.Module Motion`)) (`BlueprintMapLibrary.Map_Find` (`self.ModuleTypeSocketName`) (`/Game/ProjectLight/Modules/BP_Module_Base.ModuleType` _array_element)) "KeepRelative" "SnapToTarget" "KeepWorld" true))
                (:`then_1`
                  (bind _asbp_module_battle (cast `/Game/ProjectLight/Modules/BP_Module_Battle` _array_element))
                  (`/Game/ProjectLight/Modules/BP_Module_Battle.RegisterMotionModule` _asbp_module_battle (`self.Module Motion`)))))))
        (:`else`)))
    (:`then_1`
      (if (`KismetArrayLibrary.Array_IsNotEmpty` _assistmodules)
        (for _array_element_2 _assistmodules
          (`/Game/ProjectLight/Modules/InterfacesAndFunctions/BPL_AssistModule.LinkAssistModule` _array_element_2 (`self.AttachedModules`) self))))))

(fn `InstallNewModule`
  (params (ModuleInfo :type "/Game/ProjectLight/Modules/Struct/FModuleBaseInfo Structure"))
  (returns (InstallSuccess :type Boolean))
  (bind _spawnedmodule (`self.SpawnModuleActor` ModuleInfo))
  (`/Game/ProjectLight/Modules/BP_Module_Base.RegisterModule` _spawnedmodule self)
  (`/Game/ProjectLight/Modules/BP_Module_Base.InstallModule` _spawnedmodule self)
  (`self.OnModuleInstall` (`/Game/ProjectLight/Modules/BP_Module_Base.ModuleType` _spawnedmodule))
  (return true))

(fn `LightTakenChange`
  (params (NewLightTaken :type Boolean))
  (bind _lightchecktimer (`self.LightCheckTimer`))
  (if (!= NewLightTaken (`self.LightTaken`))
    (bind _output_get (set `self.LightTaken` NewLightTaken))
    (if _output_get
      (`self.Boot`)
      (`/Game/ProjectLight/Blueprints/FunctionLibrary/BPL_Common.PauseTimer` (`self.DarkDamageTimer`) self)
      (else
        (`self.ShutDown`)
        (if (`KismetSystemLibrary.K2_IsValidTimerHandle` _lightchecktimer)
          (`KismetSystemLibrary.K2_ClearAndInvalidateTimerHandle` _lightchecktimer))))))

(fn `NoLightTaken`
  (bind _darkdamageinfo_darkdamageinterval (break `/Game/ProjectLight/Blueprints/Struct/FDarkDamageInfo` (`self.DarkDamageInfo`)))
  (bind _darkdamagetimer (`self.DarkDamageTimer`))
  (if (`KismetSystemLibrary.K2_IsValidTimerHandle` _darkdamagetimer)
    (`/Game/ProjectLight/Blueprints/FunctionLibrary/BPL_Common.UnpauseTimer` _darkdamagetimer self)
    (elif (`|EnumInequality` (`self.BuildingType`) "NewEnumerator4")
      (bind _returnvalue (`KismetSystemLibrary.K2_SetTimerDelegate` (`|CreateDelegate` :!event `DarkDamage`) _darkdamageinfo_darkdamageinterval true true 2.0))
      (set `self.DarkDamageTimer` _returnvalue))))

(fn `PreviewStateChange`
  (params (TransPercent :type "Float (double-precision)"))
  (`MaterialInstanceDynamic.SetScalarParameterValue` (`self.PreviewMaterial`) "TransPercenet" TransPercent)
  (for _array_element (`self.AttachedModules`)
    (`/Game/ProjectLight/Modules/BP_Module_Base.PreviewStateChange` _array_element TransPercent))
  (set `self.IsPreview` false))

(fn `RegisterModuleToList`
  (params (NewModule :type "/Game/ProjectLight/Modules/BP_Module_Base Object Reference"))
  (bind _asbp_module_assist (cast `/Game/ProjectLight/Modules/BP_Module_Assist` NewModule)
    (:`then`
      (`KismetArrayLibrary.Array_AddUnique` (`self.AssistModules`) _asbp_module_assist))
    (:`CastFailed`
      (`KismetArrayLibrary.Array_AddUnique` (`self.AttachedModules`) NewModule)
      (`/Game/ProjectLight/Modules/BP_Module_Base.CloseModule` NewModule)
      (bind _asbp_module_motion (cast `/Game/ProjectLight/Modules/BP_Module_Motion` NewModule))
      (set `self.Module Motion` _asbp_module_motion))))

(fn `SetAutoRepairCheck`
  (params (New :type Boolean))
  (bind _output_get (set `self.AutoRecovery` New))
  (if _output_get
    (`self.TryToStartRecovery`)
    (else
      (`self.StopRecovery`))))

(fn `SetLightTakenNetural`
  (params (NewLightTaken_Netural :type Boolean))
  (if (!= NewLightTaken_Netural (`self.LightTaken_Netural`))
    (bind _output_get (set `self.LightTaken_Netural` NewLightTaken_Netural))
    (if _output_get
      (`self.Boot`)
      (else
        (`self.ShutDown`)))))

(fn `ShutDown`
  (set `self.IsActive` (select `bool` (`|EnumEquality` (`self.BuildingType`) "NewEnumerator4") :`true` true))
  (for _array_element (`self.AttachedModules`)
    (`/Engine/EditorBlueprintResources/StandardMacros.IsValid` _array_element
      (:`Is Valid`
        (bind _moduletype (`/Game/ProjectLight/Modules/BP_Module_Base.ModuleType` _array_element))
        (if (and (or (`|EnumEquality` _moduletype "NewEnumerator2") (`|EnumEquality` _moduletype "NewEnumerator3")) (not (`/Game/ProjectLight/Modules/BP_Module_Base.ManualControll` _array_element)) (`self.IsActive`))
          (`/Game/ProjectLight/Modules/BP_Module_Base.OpenModule` _array_element)
          (else
            (`/Game/ProjectLight/Modules/BP_Module_Base.CloseModule` _array_element)))))))

(fn `SpawnModuleActor`
  (params (FModuleInfo :type "/Game/ProjectLight/Modules/Struct/FModuleBaseInfo Structure (by ref)") (Index :type Integer))
  (returns (SpawnedModule :type "/Game/ProjectLight/Modules/BP_Module_Base Object Reference"))
  (locals (ModuleSpawned :type "/Game/ProjectLight/Modules/BP_Module_Base Object Reference"))
  (bind (_moduleclass _modulename _moduletype) (break `/Game/ProjectLight/Modules/Struct/FModuleBaseInfo` FModuleInfo))
  (bind _modulespawned (`local.ModuleSpawned`))
  (bind _returnvalue (`|SpawnActorFromClass` _moduleclass (`KismetMathLibrary.MakeTransform` (`KismetMathLibrary.MakeVector` 0.0 0.0 (`KismetMathLibrary.Conv_IntToDouble` (* Index 20)))) "Undefined" "MultiplyWithRoot" null _modulename _moduletype null))
  (bind _output_get (set `local.ModuleSpawned` _returnvalue))
  (`self.K2_AttachToComponent` _output_get (`self.StaticMesh`) (`BlueprintMapLibrary.Map_Find` (`self.ModuleTypeSocketName`) _moduletype) "KeepRelative" "SnapToTarget" "KeepWorld" true)
  (`self.RegisterModuleToList` _modulespawned)
  (return _modulespawned))

(fn `StartDestory`
  (for _array_element (`self.AttachedModules`)
    (`self.UninstallModule` _array_element true))
  (for _array_element_2 (`self.AssistModules`)
    (`self.UninstallModule` _array_element_2 true))
  (`self.SetLifeSpan` 0.2))

(fn `StartPreview`
  (bind _staticmesh (`self.StaticMesh`))
  (set `self.IsPreview` true)
  (set `self.DefaultMaterials` (`MeshComponent.GetMaterials` (`self.StaticMesh`)))
  (`PrimitiveComponent.SetMaterial` _staticmesh 0 "/Game/ProjectLight/Buildings/Materials/MI_PreviewBuilding.MI_PreviewBuilding")
  (bind _returnvalue (`PrimitiveComponent.CreateDynamicMaterialInstance` _staticmesh 0 (`PrimitiveComponent.GetMaterial` _staticmesh 0) "None"))
  (bind _output_get (set `self.PreviewMaterial` _returnvalue))
  (`PrimitiveComponent.SetMaterial` _staticmesh 0 _output_get)
  (for _array_element (`self.AttachedModules`)
    (`/Game/ProjectLight/Modules/BP_Module_Base.StartPreview` _array_element)))

(fn `StopRecovery`
  (bind _recoverytimer (`self.RecoveryTimer`))
  (if (`KismetSystemLibrary.K2_IsValidTimerHandle` _recoverytimer)
    (`KismetSystemLibrary.K2_ClearAndInvalidateTimerHandle` _recoverytimer)))

(fn `UninstallModule`
  (params (ModuleToUninstall :type "/Game/ProjectLight/Modules/BP_Module_Base Object Reference") (Discard :type Boolean))
  (bind _moduletype (`/Game/ProjectLight/Modules/BP_Module_Base.ModuleType` ModuleToUninstall))
  (`/Game/ProjectLight/Modules/BP_Module_Base.UninstallModule` ModuleToUninstall self true)
  (`self.UnregisterModule` ModuleToUninstall)
  (`self.OnModuleUninstall` _moduletype)
  (if (not Discard)
    (bind _inventorycomponent (`/Game/ProjectLight/Blueprints/FunctionLibrary/BML_Common.GetInventoryComponent` (`GameplayStatics.GetPlayerCharacter` 0))
      (:`IsValid`
        (`/Game/ProjectLight/Characters/Components/BPC_InventoryComponent.ChangeModuleStock` _inventorycomponent (make `/Game/ProjectLight/Modules/Struct/FModuleBasicInfo` (`/Game/ProjectLight/Modules/BP_Module_Base.ModuleName` ModuleToUninstall) _moduletype) 1)))))

(fn `UnregisterModule`
  (params (ModuleToUninstall :type "/Game/ProjectLight/Modules/BP_Module_Base Object Reference"))
  (bind _asbp_module_assist (cast `/Game/ProjectLight/Modules/BP_Module_Assist` ModuleToUninstall)
    (:`then`
      (`KismetArrayLibrary.Array_RemoveItem` (`self.AssistModules`) _asbp_module_assist))
    (:`CastFailed`
      (`KismetArrayLibrary.Array_RemoveItem` (`self.AttachedModules`) ModuleToUninstall))))

(fn `UpdateAssistEffect`
  (`self.ChangeMaxHealth` (`self.GetAttributeByTag` (struct :`TagName` "Unit.Base.MaxHealth"))))

(fn `UpgradeBuilding`
  (params (NewBuildingName :type Name))
  (bind _attachedmodules (`self.AttachedModules`))
  (set `self.BuildingName` NewBuildingName)
  (for _array_element _attachedmodules
    (bind _asbp_module_storage (cast `/Game/ProjectLight/Modules/BP_Module_Storage` _array_element)
      (:`then`
        (`BlueprintMapLibrary.Map_Add` (`self.TempStorage`) (`/Game/ProjectLight/Blueprints/FunctionLibrary/BPL_Common.GetUnitNameAndLevel` (`KismetStringLibrary.Conv_NameToString` (`/Game/ProjectLight/Modules/BP_Module_Base.ModuleName` _asbp_module_storage))) (`/Game/ProjectLight/Modules/BP_Module_Storage.CurrentStorage` _asbp_module_storage)))
      (:`CastFailed`
        _))
    (`/Game/ProjectLight/Modules/BP_Module_Base.UninstallModule` _array_element self true))
  (`KismetArrayLibrary.Array_Clear` _attachedmodules)
  (for _array_element_2 (`self.AssistModules`)
    (`/Game/ProjectLight/Modules/BP_Module_Base.UninstallModule` _array_element_2 self false))
  (`self.InitBuilding`)
  (`PrimitiveComponent.SetCollisionProfileName` (`self.Capsule`) "PreviewBuilding" true)
  (for _array_element_3 (`self.AttachedModules`)
    (`/Game/ProjectLight/Modules/BP_Module_Base.RegisterModule` _array_element_3 self))
  (if (== (`GameplayStatics.GetObjectClass` self) "/Game/ProjectLight/Buildings/BP_Building_MainTower.BP_Building_MainTower_C")
    (`self.BuildComplete`)
    (else
      (`self.StartPreview`)
      (`self.BuildConfirm`))))

(fn `UserConstructionScript`)
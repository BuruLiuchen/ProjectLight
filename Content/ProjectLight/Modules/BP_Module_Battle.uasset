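; Battle module that turns a parent unit's energy into spotlight attacks, passing light energy to the actors it hits.
; A looping timer consumes energy and runs the data-table mode: cone traces, surround sphere trace, or charge that bursts on close and sends overcharge to heat.
; Players control it manually, while other units follow Dusk/Day phases.
; Assist effects rescale attributes, and an attached motion module adds energy cost and follows work state.
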(event `TryToStartLight`
  (if (`self.ManualControll`)
    (bind _returnvalue (`KismetSystemLibrary.K2_SetTimerDelegate` (delegate `KeepLight`) (`self.GetAttributeByTag` (struct :`TagName` "Module.Battle.AttackInterval")) true true :!label _label))
    (bind _output_get (set `self.LightTimer` _returnvalue))
    (`KismetArrayLibrary.Array_AddUnique` (`self.WorkingTimers`) _output_get)
    (elif (not (`BlueprintGameplayTagLibrary.MatchesTag` (`self.CurrentPhase`) (struct :`TagName` "Gameplay.Phase.Day")))
      (goto _label)
      (else
        (`self.CloseModule`)))))

(event `KeepLight`
  (`self.EnergyConsume` 0.0
    (:`CanWork`
      (`self.ChangeWorkState` "NewEnumerator2" (`self.ManualControll`))
      (switch `/Game/ProjectLight/Modules/Enum/EAttackMode` (`.AttackMode_2_E8E6633B4AC0E7B8BF1CA59D88094C30` (break `/Game/ProjectLight/Modules/Struct/FModuleInfo_Battle` (`self.BattleModuleInfo`)))
        (:`NewEnumerator0`
          (`self.ApplyConeLight` 0.0))
        (:`NewEnumerator1`
          (`self.Change Light Volume Charged` 0.0))
        (:`NewEnumerator2`
          (`self.ApplySurroundLight` 0.0))))
    (:`NotWork`
      (`/Game/ProjectLight/Blueprints/FunctionLibrary/BPL_Common.PauseTimer` (`self.LightTimer`) self)
      (`self.ChangeWorkState` "NewEnumerator4"))))

(event `self.ReceiveBeginPlay`
  (bind _returnvalue (`|GetDataTableRow` (`self.DataTable`) (`self.ModuleName`))
    (:`then`
      (bind _output_get (set `self.BattleModuleInfo` _returnvalue))
      (bind (_basicinfo _workcondition) (break `/Game/ProjectLight/Modules/Struct/FModuleInfo_Battle` _output_get))
      (set `self.BasicInfo` _basicinfo)
      (`self.SetWorkCondition` _workcondition)
      (`self.SetInputVolumeCap`)
      (`parent.ReceiveBeginPlay`)
      (`KismetSystemLibrary.Delay` 0.2)
      (`self.SetLightInfo`)
      (bind _parentactor (`self.ParentActor`)
        (:`then`
          (bind _unittype (message `/Game/ProjectLight/Blueprints/Interfaces/BPI_Common.GetUnitType` _parentactor))
          (if (`|EnumEquality` _unittype "NewEnumerator0")
            (set `self.ManualControll` true)
            (else
              (bind _asgm_battle_stage (cast `/Game/ProjectLight/BattleScene/GM_BattleStage` (`GameplayStatics.GetGameMode`)))
              (add `/Game/ProjectLight/BattleScene/GM_BattleStage.OnPhaseChange` _asgm_battle_stage (delegate `OnPhaseChange`)))))
        (:`else`)))))

(event `OnPhaseChange`
  (params (NewPhase :type "GameplayTag Structure"))
  (bind _output_get (set `self.CurrentPhase` NewPhase))
  (if (not (`self.ManualControll`))
    (`|SwitchGameplayTag` _output_get
      (:`Gameplay.Phase.Day`
        (`self.CloseModule`))
      (:`Gameplay.Phase.Dusk`
        (`self.OpenModule`)))))

(event `self.ReceiveTick`
  (params (DeltaSeconds :type "Float (single-precision)")))

(event `self.BPC_EnergyPort_Input.OnCurrentVolumeChange`
  (if (not (`/Game/ProjectLight/Components/BPC_EnergyPort.CurrentVolumeIsEmpty` (`self.BPC_EnergyPort_Input`)))
    (bind _unittype (message `/Game/ProjectLight/Blueprints/Interfaces/BPI_Common.GetUnitType` (`self.ParentActor`)))
    (if (`|EnumEquality` _unittype "NewEnumerator2")
      (`self.ChangeWorkState` "NewEnumerator2")
      (`/Game/ProjectLight/Blueprints/FunctionLibrary/BPL_Common.UnpauseTimer` (`self.LightTimer`) self))))

(event `/Game/ProjectLight/Modules/InterfacesAndFunctions/BPI_AssistModule.ApplyAssistEffect`
  (params (AssistEffect :type "/Game/ProjectLight/Modules/Struct/FAssistEffectInfo Structure"))
  (`/Game/ProjectLight/Modules/InterfacesAndFunctions/BPL_AssistModule.ApplyAssist` AssistEffect (`self.AdjustRateMap`))
  (`self.SetInputVolumeCap`)
  (`self.SetLightInfo`))

(event `/Game/ProjectLight/Modules/InterfacesAndFunctions/BPI_AssistModule.RemoveAssistEffect`
  (params (AssistEffect :type "/Game/ProjectLight/Modules/Struct/FAssistEffectInfo Structure"))
  (`/Game/ProjectLight/Modules/InterfacesAndFunctions/BPL_AssistModule.ApplyAssist` AssistEffect (`self.AdjustRateMap`) true)
  (`self.SetInputVolumeCap`)
  (`self.SetLightInfo`))

(fn `ApplyConeLight`
  (params (DeltaTime :type "Float (double-precision)"))
  (locals (HitActors :type "Array of Actor Object Reference"))
  (bind _attributereturn (`self.GetAttributeByTag` (struct :`TagName` "Module.Battle.AttackAngle")))
  (bind _deltatime (`local.DeltaTime`))
  (bind _parentactor (`self.ParentActor`))
  (bind (_asbp_character_hero _bsuccess) (cast `/Game/ProjectLight/Characters/Hero/BP_Character_Hero` _parentactor :!pure true))
  (bind _outhits (`/Game/ProjectLight/Blueprints/FunctionLibrary/BPL_Light.ConeLineTrace` (select `bool` _bsuccess :`false` self :`true` _asbp_character_hero :!type "Actor Object Reference") (`|MakeArray` _parentactor) (* (/ _attributereturn 10.0) 2) 90.0 20.0 _attributereturn (`self.GetAttributeByTag` (struct :`TagName` "Module.Battle.AttackRange"))))
  (for _array_element _outhits
    (`KismetArrayLibrary.Array_AddUnique` (`local.HitActors`) (`.HitActor` (`GameplayStatics.BreakHitResult` _array_element))))
  (for _array_element_2 (`local.HitActors`)
    (bind _unittype (message `/Game/ProjectLight/Blueprints/Interfaces/BPI_Common.GetUnitType` (`self.ParentActor`)))
    (message `/Game/ProjectLight/Components/Interfaces/BPI_Energy.EnergyPass_UDP` _array_element_2 (make `/Game/ProjectLight/Components/Struct/FEnergyInfo` "NewEnumerator0" (* (`self.GetAttributeByTag` (struct :`TagName` "Module.Battle.LightPower")) (select `bool` (> _deltatime 0.0) :`false` (`self.GetAttributeByTag` (struct :`TagName` "Module.Battle.AttackInterval")) :`true` _deltatime))) (select `/Game/ProjectLight/Blueprints/Enums/EUnitType` _unittype :`NewEnumerator0` "NewEnumerator2" :`NewEnumerator1` "NewEnumerator3" :`NewEnumerator2` "NewEnumerator1" :`NewEnumerator3` "NewEnumerator1" :!type "/Game/ProjectLight/Components/Enum/EEnergySourceType Enum"))))

(fn `ApplySurroundLight`
  (params (DeltaTime :type "Float (double-precision)"))
  (locals (HitActors :type "Array of Actor Object Reference"))
  (bind _deltatime (`local.DeltaTime`))
  (bind _parentactor (`self.ParentActor`))
  (bind _returnvalue (`self.K2_GetActorLocation` _parentactor))
  (bind _outhits (`KismetSystemLibrary.SphereTraceMulti` _returnvalue _returnvalue (`self.GetAttributeByTag` (struct :`TagName` "Module.Battle.AttackRange")) "TraceTypeQuery5" false (`|MakeArray` _parentactor)))
  (for _array_element _outhits
    (`KismetArrayLibrary.Array_AddUnique` (`local.HitActors`) (`.HitActor` (`GameplayStatics.BreakHitResult` _array_element))))
  (for _array_element_2 (`local.HitActors`)
    (bind _unittype (message `/Game/ProjectLight/Blueprints/Interfaces/BPI_Common.GetUnitType` (`self.ParentActor`)))
    (message `/Game/ProjectLight/Components/Interfaces/BPI_Energy.EnergyPass_UDP` _array_element_2 (make `/Game/ProjectLight/Components/Struct/FEnergyInfo` "NewEnumerator0" (* (`self.GetAttributeByTag` (struct :`TagName` "Module.Battle.LightPower")) (select `bool` (> _deltatime 0.0) :`false` (`self.GetAttributeByTag` (struct :`TagName` "Module.Battle.AttackInterval")) :`true` _deltatime))) (select `/Game/ProjectLight/Blueprints/Enums/EUnitType` _unittype :`NewEnumerator0` "NewEnumerator2" :`NewEnumerator1` "NewEnumerator3" :`NewEnumerator2` "NewEnumerator1" :`NewEnumerator3` "NewEnumerator1" :!type "/Game/ProjectLight/Components/Enum/EEnergySourceType Enum"))))

(fn `BurstLight`
  (`self.ApplyConeLight` (* (/ (`self.LightVolumeCharged`) (`self.GetAttributeByTag` (struct :`TagName` "Module.Battle.LightChargeCap"))) (`self.GetAttributeByTag` (struct :`TagName` "Module.Battle.LightPower"))))
  (`self.Change Light Volume Charged` (* (`self.LightVolumeCharged`) -1.0)))

(fn `Change Light Volume Charged`
  (params (DeltaTime :type "Float (double-precision)"))
  (locals (LightOverCharged :type "Float (double-precision)"))
  (bind _attributereturn (`self.GetAttributeByTag` (struct :`TagName` "Module.Battle.LightChargeCap")))
  (bind _output_get (set `self.LightVolumeCharged` (`KismetMathLibrary.FClamp` (+ (`self.LightVolumeCharged`) (* (select `bool` (> DeltaTime 0.0) :`false` (`self.GetAttributeByTag` (struct :`TagName` "Module.Battle.AttackInterval")) :`true` DeltaTime) (`self.GetAttributeByTag` (struct :`TagName` "Module.Battle.LightChargeRate")))) 0.0 (select `bool` (`.AllowOverload_11_DF094AB0445C855CC122E091FEC42A13` (break `/Game/ProjectLight/Modules/Struct/FModuleInfo_Base` (`.BasicInfo_6_414C61A04DE72DB98E7CADA74C6A4198` (break `/Game/ProjectLight/Modules/Struct/FModuleInfo_Battle` (`self.BattleModuleInfo`))))) :`false` _attributereturn :`true` (* _attributereturn 1.5)))))
  (bind _output_get_2 (set `local.LightOverCharged` (- _output_get (`self.GetAttributeByTag` (struct :`TagName` "Module.Battle.LightChargeCap")))))
  (if (> _output_get_2 0.0)
    (bind _heatcomponent (`/Game/ProjectLight/Blueprints/FunctionLibrary/BML_Common.GetHeatComponent` (`self.ParentActor`))
      (:`IsValid`
        (`/Game/ProjectLight/Components/BPC_HeatComponent.ReceiveLight` _heatcomponent (`local.LightOverCharged`))))))

(fn `ChangeWorkState`
  (params (NewWorkState :type "/Game/ProjectLight/Modules/Enum/EWorkState Enum" :default "NewEnumerator0") (ForceSwitch :type Boolean))
  (bind _workstate (`self.WorkState`))
  (bind _spotlight (`self.SpotLight`))
  (bind _changed (`parent.ChangeWorkState` NewWorkState ForceSwitch))
  (if _changed
    (bind _motionmoduleattached (`self.MotionModuleAttached`)
      (:`then`
        (`self.ChangeWorkState` _motionmoduleattached _workstate false))
      (:`else`
        _))
    (switch `/Game/ProjectLight/Modules/Enum/EWorkState` _workstate
      (:`NewEnumerator0`
        (`SceneComponent.SetVisibility` _spotlight false false :!label _label))
      (:`NewEnumerator4`
        (goto _label))
      (:`NewEnumerator2`
        (`SceneComponent.SetVisibility` _spotlight true false)))))

(fn `CloseModule`
  (bind _workingtimers (`self.WorkingTimers`))
  (`parent.CloseModule`)
  (if (`|EnumEquality` (`.AttackMode_2_E8E6633B4AC0E7B8BF1CA59D88094C30` (break `/Game/ProjectLight/Modules/Struct/FModuleInfo_Battle` (`self.BattleModuleInfo`))) "NewEnumerator1")
    (`self.BurstLight`))
  (if (`KismetArrayLibrary.Array_IsNotEmpty` _workingtimers)
    (for _array_element _workingtimers
      (if (`KismetSystemLibrary.K2_IsValidTimerHandle` _array_element)
        (`KismetSystemLibrary.K2_ClearAndInvalidateTimerHandle` _array_element)))
    (`KismetArrayLibrary.Array_Clear` (`self.WorkingTimers`))))

(fn `GetAttributeByTag`
  (params (AttributeTag :type "GameplayTag Structure"))
  (returns (AttributeReturn :type "Float (double-precision)"))
  (locals (AdjustRate_Local :type "Float (double-precision)"))
  (bind _adjustrate_local (`local.AdjustRate_Local`))
  (bind ((`EnergyConsumePerSecond_27_B0D9AA454100F1724F25F2B243581B42` _energyconsumepersecond) (`AttackInterval_12_6EFD5F3A46C3E751D7B394A027EE9BC9` _attackinterval) (`LightPower_29_3D539A304D3CA8686D02B6BE6E81787E` _lightpower) (`AttackAngle_16_F01804FE4543C69B946D9BBA7E3701D7` _attackangle) (`AttackRange_22_1AF10EBC49359C72F6B79599AD3EE562` _attackrange) (`LightChargePerSecond_30_AC4C27EE49BD3AA4C5F241BBBEE90BEA` _lightchargepersecond) (`LightVolumeCap_18_392CD6A34823CD25B4170B84EC349C8F` _lightvolumecap)) (break `/Game/ProjectLight/Modules/Struct/FModuleInfo_Battle` (`self.BattleModuleInfo`)))
  (set `local.AdjustRate_Local` (`parent.GetAttributeByTag` AttributeTag))
  (`|SwitchGameplayTag` AttributeTag
    (:`Module.Battle.AttackAngle`
      (return (`KismetMathLibrary.FClamp` (* _attackangle _adjustrate_local) 1.0 89.0)))
    (:`Module.Battle.AttackInterval`
      (return (* _attackinterval _adjustrate_local)))
    (:`Module.Battle.AttackRange`
      (return (* _attackrange _adjustrate_local)))
    (:`Module.Battle.EnergyConsumeRate`
      (return (* _energyconsumepersecond _adjustrate_local)))
    (:`Module.Battle.LightChargeCap`
      (return (* _lightvolumecap _adjustrate_local)))
    (:`Module.Battle.LightChargeRate`
      (return (* _lightchargepersecond _adjustrate_local)))
    (:`Module.Battle.LightPower`
      (return (* _lightpower _adjustrate_local)))))

(fn `GetEnergyConsume`
  (returns (EnergyConsumeValue :type "Float (double-precision)"))
  (bind _attributereturn (`self.GetAttributeByTag` (struct :`TagName` "Module.Battle.EnergyConsumeRate")))
  (bind _motionmoduleattached (`self.MotionModuleAttached`)
    (:`then`
      (return (+ _attributereturn (`self.GetAttributeByTag` _motionmoduleattached (struct :`TagName` "Module.Battle.EnergyConsumeRate")))))
    (:`else`
      (return _attributereturn))))

(fn `GetSurroundLightInfo`
  (returns (AttenuationRadius :type "Float (double-precision)") (ConeAngle :type "Float (double-precision)"))
  (locals (Radius :type "Float (double-precision)" :default 0.0))
  (bind _output_get (set `local.Radius` (`KismetMathLibrary.Sqrt` (+ (`KismetMathLibrary.Square` (.z (`SceneComponent.K2_GetComponentLocation` (`self.SpotLight`)))) (`KismetMathLibrary.Square` (`self.GetAttributeByTag` (struct :`TagName` "Module.Battle.AttackRange")))))))
  (return _output_get (`KismetMathLibrary.DegAsin` (/ (`self.GetAttributeByTag` (struct :`TagName` "Module.Battle.AttackRange")) (`local.Radius`)))))

(fn `OpenModule`
  (returns (OpenSuccess :type Boolean))
  (bind _opensuccess (`parent.OpenModule`))
  (if _opensuccess
    (`self.StartAttack` 0.0)
    (bind _motionmoduleattached (`self.MotionModuleAttached`)
      (:`then`
        (if (not (`/Game/ProjectLight/Modules/BP_Module_Base.ManualControll` _motionmoduleattached))
          (bind _opensuccess_2 (`self.OpenModule` _motionmoduleattached))
          (return _opensuccess_2)
          (else
            _)))
      (:`else`
        _))
    (return true)
    (else
      (return false))))

(fn `RegisterMotionModule`
  (params (MotionModule :type "/Game/ProjectLight/Modules/BP_Module_Motion Object Reference"))
  (set `self.MotionModuleAttached` MotionModule)
  (`self.SetInputVolumeCap`))

(fn `SetInputVolumeCap`
  (`/Game/ProjectLight/Components/BPC_EnergyPort.SetVolumeCap` (`self.BPC_EnergyPort_Input`) (`KismetMathLibrary.Conv_IntToDouble` (`KismetMathLibrary.FCeil` (* (`self.GetEnergyConsume`) (`self.GetAttributeByTag` (struct :`TagName` "Module.Battle.AttackInterval")))))))

(fn `SetLightInfo`
  (bind _spotlight (`self.SpotLight`))
  (bind _spotlight_2 (`self.SpotLight`))
  (bind _spotlight_3 (`self.SpotLight`))
  (bind _returnvalue (/ (`self.GetAttributeByTag` (struct :`TagName` "Module.Battle.AttackAngle")) 2.0))
  (`LightComponent.SetIntensity` (`self.SpotLight`) (* (`self.GetAttributeByTag` (struct :`TagName` "Module.Battle.LightPower")) (select `/Game/ProjectLight/Modules/Enum/EAttackMode` (`.AttackMode_2_E8E6633B4AC0E7B8BF1CA59D88094C30` (break `/Game/ProjectLight/Modules/Struct/FModuleInfo_Battle` (`self.BattleModuleInfo`))) :`NewEnumerator0` 30.0 :`NewEnumerator1` 60.0 :`NewEnumerator2` 1.0)))
  (switch `/Game/ProjectLight/Modules/Enum/EAttackMode` (`.AttackMode_2_E8E6633B4AC0E7B8BF1CA59D88094C30` (break `/Game/ProjectLight/Modules/Struct/FModuleInfo_Battle` (`self.BattleModuleInfo`)))
    (:`NewEnumerator0`
      (`LocalLightComponent.SetAttenuationRadius` _spotlight_2 (+ (`self.GetAttributeByTag` (struct :`TagName` "Module.Battle.AttackRange")) 200.0) :!label _label)
      (`SpotLightComponent.SetInnerConeAngle` _spotlight_2 _returnvalue)
      (`SpotLightComponent.SetOuterConeAngle` _spotlight_2 _returnvalue)
      (bind _asbp_character_hero (cast `/Game/ProjectLight/Characters/Hero/BP_Character_Hero` (`self.ParentActor`)))
      (`SceneComponent.K2_SetRelativeLocation` _spotlight_3 (0.0 0.0 0.0) false false)
      (`SceneComponent.K2_AttachToComponent` _spotlight_3 (`Character.Mesh` _asbp_character_hero) "spotlight" "SnapToTarget" "SnapToTarget" "KeepRelative" true))
    (:`NewEnumerator1`
      (goto _label))
    (:`NewEnumerator2`
      (`SceneComponent.K2_SetRelativeLocationAndRotation` (`self.SpotLight`) (0.0 0.0 1000.0) (struct :`Pitch` -90.0 :`Roll` 90.0) false false)
      (bind (_attenuationradius _coneangle) (`self.GetSurroundLightInfo`))
      (`LocalLightComponent.SetAttenuationRadius` _spotlight _attenuationradius)
      (`SpotLightComponent.SetInnerConeAngle` _spotlight _coneangle)
      (`SpotLightComponent.SetOuterConeAngle` _spotlight _coneangle))))

(fn `SetStaticMesh`
  (params (NewMesh :type "StaticMesh Object Reference"))
  (locals (SpawnedStaticMesh :type "StaticMeshComponent Object Reference"))
  (bind _spawnedstaticmesh (`local.SpawnedStaticMesh`))
  (bind _staticmesh (`self.StaticMesh`))
  (switch `/Game/ProjectLight/Blueprints/Enums/EUnitType` (`self.ParentUnitType`)
    (:`NewEnumerator0`
      (`parent.SetStaticMesh` NewMesh))
    (:`NewEnumerator2`
      (bind _returnvalue (`AddComponent|NODE_AddStaticMeshComponent-0` :`RelativeTransform` (`KismetMathLibrary.MakeTransform` (0.0 0.0 0.0))))
      (bind _output_get (set `local.SpawnedStaticMesh` _returnvalue))
      (`PrimitiveComponent.SetCollisionProfileName` _output_get "NoCollision" true)
      (`StaticMeshComponent.SetStaticMesh` _output_get (`local.NewMesh`))
      (`SceneComponent.K2_AttachToComponent` (`local.SpawnedStaticMesh`) (`self.StaticMesh`) "LightSocket" "SnapToTarget" "SnapToTarget" "KeepRelative" true)
      (`BlueprintMapLibrary.Map_Add` (`self.MeshDefaultMaterials`) _spawnedstaticmesh (make `/Game/ProjectLight/Modules/Struct/FMaterialArray` (`MeshComponent.GetMaterials` _spawnedstaticmesh)))
      (`BlueprintMapLibrary.Map_Add` (`self.MeshDefaultMaterials`) _staticmesh (make `/Game/ProjectLight/Modules/Struct/FMaterialArray` (`MeshComponent.GetMaterials` _staticmesh))))))

(fn `StartAttack`
  (params (DeltaTime :type "Float (double-precision)"))
  (bind _deltatime (`local.DeltaTime`))
  (if (> DeltaTime 0.0)
    (`self.EnergyConsume` _deltatime
      (:`CanWork`
        (switch `/Game/ProjectLight/Modules/Enum/EAttackMode` (`.AttackMode_2_E8E6633B4AC0E7B8BF1CA59D88094C30` (break `/Game/ProjectLight/Modules/Struct/FModuleInfo_Battle` (`self.BattleModuleInfo`)))
          (:`NewEnumerator0`
            (`self.ApplyConeLight` _deltatime))
          (:`NewEnumerator1`
            (`self.Change Light Volume Charged` _deltatime))
          (:`NewEnumerator2`
            (`self.ApplySurroundLight` _deltatime)))))
    (else
      (`self.TryToStartLight`))))

(fn `UserConstructionScript`
  (`parent.UserConstructionScript`))
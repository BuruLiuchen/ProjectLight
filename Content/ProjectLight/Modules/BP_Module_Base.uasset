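; Base actor for energy modules attached to buildings or other parent actors.
; On BeginPlay or RegisterModule it loads basic info, registers its ports with the parent's port manager, creates an info widget and joins the building's module list or parent's inventory.
; Work checks derive efficiency from input energy and free output space, while helpers spread consumption and charging across ports.
; Opening or closing toggles ports and work state, gated by parent activity.
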(event `RegisterModule`
  (params (ParentActor :type "Actor Object Reference"))
  (bind _parentactor (`self.ParentActor`))
  (bind _returnvalue (`self.GetComponentByClass` _parentactor "/Game/ProjectLight/Characters/Components/BPC_InventoryComponent.BPC_InventoryComponent_C"))
  (set `self.ParentActor` ParentActor)
  (`/Engine/EditorBlueprintResources/StandardMacros.IsValid` (`self.ParentActor`) :!label _label
    (:`Is Valid`
      (`self.InitBasicInfo`)
      (`self.InitPortsInfo`)
      (bind _returnvalue_2 (`|CreateWidget` "/Game/ProjectLight/UMG/UMG_ModuleInfoDisplay.UMG_ModuleInfoDisplay_C" null self))
      (`WidgetComponent.SetWidget` (`self.Widget`) _returnvalue_2)
      (bind _asbp_building_base (cast `/Game/ProjectLight/Buildings/BP_Building_Base` _parentactor)
        (:`then`
          (`KismetArrayLibrary.Array_AddUnique` (`/Game/ProjectLight/Buildings/BP_Building_Base.AttachedModules` _asbp_building_base) self))
        (:`CastFailed`
          (`/Engine/EditorBlueprintResources/StandardMacros.IsValid` _returnvalue
            (:`Is Valid`
              (`/Game/ProjectLight/Characters/Components/BPC_InventoryComponent.UpdateModuleList` _returnvalue self))))))))

(event `self.ReceiveBeginPlay`
  (set `self.ParentActor` (`self.GetAttachParentActor`))
  (goto _label))

(fn `ChangeWorkState`
  (params (NewWorkState :type "/Game/ProjectLight/Modules/Enum/EWorkState Enum" :default "NewEnumerator0"))
  (locals (BuildingIsActive :type Boolean :default false))
  (bind _parentactor (`self.ParentActor`)
    (:`then`
      (bind _isactive (message `/Game/ProjectLight/Blueprints/Interfaces/BPI_Common.GetIsActive` _parentactor))
      (bind _output_get (set `local.BuildingIsActive` _isactive))
      (if _output_get
        (set `self.WorkState` (`local.NewWorkState`))
        (else
          (set `self.WorkState` "NewEnumerator0"))))
    (:`else`)))

(fn `ChargeOutputVolume`
  (params (EnergyType :type "/Game/ProjectLight/Components/Enum/EEnergyType Enum" :default "NewEnumerator0") (Volume :type "Float (double-precision)"))
  (locals (VolumeNeedToCharge :type "Float (double-precision)") (VolumeHasCharged :type "Float (double-precision)"))
  (set `local.VolumeNeedToCharge` Volume)
  (for _array_element (`/Game/ProjectLight/Blueprints/FunctionLibrary/BPL_Port.GetPortsByTypeAndEnergy` self "NewEnumerator1" EnergyType)
    (bind _output_get (set `local.VolumeHasCharged` (`KismetMathLibrary.FMin` (- (`/Game/ProjectLight/Components/BPC_EnergyPort.VolumeCap` _array_element) (`/Game/ProjectLight/Components/BPC_EnergyPort.CurrentVolume` _array_element)) (`local.VolumeNeedToCharge`))))
    (`/Game/ProjectLight/Components/BPC_EnergyPort.ChangeEnergyVolume` _array_element _output_get)
    (bind _output_get_2 (set `local.VolumeNeedToCharge` (- (`local.VolumeNeedToCharge`) (`local.VolumeHasCharged`))))
    (if (<= _output_get_2 0.0)
      (break))))

(fn `CheckWorkCondition`
  (returns (CanWork :type Boolean))
  (locals (InputVolume :type "Float (double-precision)" :default 0.0))
  (bind _inputvolume (`local.InputVolume`))
  (bind (_norequest _energytype _volumefornormalwork) (break `/Game/ProjectLight/Modules/Struct/FWorkCondition` (`self.WorkCondition`)))
  (if (and (`self.OutputIsNotAllFull`) (`|EnumInequality` (`self.WorkState`) "NewEnumerator0"))
    (if _norequest
      (set `self.WorkEfficiency` 1.0)
      (return true)
      (else
        (set `local.InputVolume` (`self.GetInputVolumeByEnergyType` _energytype))
        (if (>= _inputvolume _volumefornormalwork)
          (set `self.WorkEfficiency` 1.0)
          (elif (> _inputvolume 0.0)
            (set `self.WorkEfficiency` 0.5)
            (else
              (return false))))
        (return true)))
    (else
      (return false))))

(fn `CloseModule`
  (for _array_element (`self.K2_GetComponentsByClass` "/Game/ProjectLight/Components/BPC_EnergyPort.BPC_EnergyPort_C")
    (`/Game/ProjectLight/Components/BPC_EnergyPort.ClosePort` _array_element))
  (`self.ChangeWorkState` "NewEnumerator0")
  (`self.OnModuleClose`))

(fn `ConsumeInputVolume`
  (params (EnergyType :type "/Game/ProjectLight/Components/Enum/EEnergyType Enum" :default "NewEnumerator0") (Volume :type "Float (double-precision)"))
  (returns (VolumeConsumed :type "Float (double-precision)"))
  (locals (VolumeNeedToConsume :type "Float (double-precision)") (VolumeHasConsumed :type "Float (double-precision)"))
  (set `local.VolumeNeedToConsume` Volume)
  (for _array_element (`/Game/ProjectLight/Blueprints/FunctionLibrary/BPL_Port.GetPortsByTypeAndEnergy` self "NewEnumerator0" EnergyType)
    (bind _output_get (set `local.VolumeHasConsumed` (* (`KismetMathLibrary.FMin` (`/Game/ProjectLight/Components/BPC_EnergyPort.CurrentVolume` _array_element) (`local.VolumeNeedToConsume`)) -1.0)))
    (`/Game/ProjectLight/Components/BPC_EnergyPort.ChangeEnergyVolume` _array_element _output_get)
    (bind _output_get_2 (set `local.VolumeNeedToConsume` (+ (`local.VolumeNeedToConsume`) (`local.VolumeHasConsumed`))))
    (if (<= _output_get_2 0.0)
      (break)))
  (return (- (`local.Volume`) (`local.VolumeNeedToConsume`))))

(fn `GetAttributeByTag`
  (params (AttributeTag :type "GameplayTag Structure"))
  (returns (AttributeReturn :type "Float (double-precision)"))
  (locals (AdjustRate_Local :type "Float (double-precision)"))
  (bind _adjustratemap (`self.AdjustRateMap`))
  (bind (_value _returnvalue) (`BlueprintMapLibrary.Map_Find` _adjustratemap AttributeTag))
  (if _returnvalue
    (set `local.AdjustRate_Local` _value)
    (else
      (`BlueprintMapLibrary.Map_Add` _adjustratemap AttributeTag 1.0)
      (set `local.AdjustRate_Local` 1.0)))
  (return (`local.AdjustRate_Local`)))

(fn `GetInputVolumeByEnergyType`
  (params (EnergyType :type "/Game/ProjectLight/Components/Enum/EEnergyType Enum" :default "NewEnumerator0"))
  (returns (TotalVolume :type "Float (double-precision)"))
  (locals (VolumeReturn :type "Float (double-precision)"))
  (for _array_element (`/Game/ProjectLight/Blueprints/FunctionLibrary/BPL_Port.GetPortsByTypeAndEnergy` self "NewEnumerator0" EnergyType)
    (set `local.VolumeReturn` (+ (`local.VolumeReturn`) (`/Game/ProjectLight/Components/BPC_EnergyPort.CurrentVolume` _array_element))))
  (return (`local.VolumeReturn`)))

(fn `GetModuleParentActor`
  (returns (ModuleParentActor :type "Actor Object Reference"))
  (return (`self.ParentActor`)))

(fn `GetModuleType`
  (returns (Type :type "/Game/ProjectLight/Modules/EModuleType Enum"))
  (return (`self.ModuleType`)))

(fn `InitBasicInfo`
  (bind (_size _rarity _moduletype _basicworkheat _allowoverload) (break `/Game/ProjectLight/Modules/Struct/FModuleInfo_Base` (`self.BasicInfo`)))
  (set `self.Size` _size)
  (set `self.ModuleType` _moduletype)
  (set `self.BasicWorkHeat` _basicworkheat)
  (set `self.Allow Overload` _allowoverload))

(fn `InitPortsInfo`
  (bind _parentactor (`self.ParentActor`))
  (bind _returnvalue (`self.GetComponentByClass` _parentactor "/Game/ProjectLight/Components/BPC_PortManageComponent.BPC_PortManageComponent_C"))
  (`/Engine/EditorBlueprintResources/StandardMacros.IsValid` _parentactor
    (:`Is Valid`
      (`/Engine/EditorBlueprintResources/StandardMacros.IsValid` _returnvalue
        (:`Is Valid`
          (for _array_element (`self.K2_GetComponentsByClass` "/Game/ProjectLight/Components/BPC_EnergyPort.BPC_EnergyPort_C")
            (`/Game/ProjectLight/Components/BPC_PortManageComponent.UpdatePortsInfo` _returnvalue _array_element)))))))

(fn `InstallModule`
  (params (ContextObject :type "Object Object Reference")))

(fn `OpenModule`
  (returns (OpenSuccess :type Boolean))
  (for _array_element (`self.K2_GetComponentsByClass` "/Game/ProjectLight/Components/BPC_EnergyPort.BPC_EnergyPort_C")
    (`/Game/ProjectLight/Components/BPC_EnergyPort.OpenPort` _array_element))
  (`self.ChangeWorkState` "NewEnumerator4")
  (`self.OnModuleOpen`)
  (return true))

(fn `OutputIsNotAllFull`
  (returns (NotAllFull :type Boolean))
  (bind _returnvalue (`self.K2_GetComponentsByClass` "/Game/ProjectLight/Components/BPC_EnergyPort_Output.BPC_EnergyPort_Output_C"))
  (if (`KismetArrayLibrary.Array_IsNotEmpty` _returnvalue)
    (for _array_element _returnvalue
      (if (not (`/Game/ProjectLight/Components/BPC_EnergyPort.CurrentVolumeIsFull` _array_element))
        (return true)))
    (return false)
    (else
      (return true))))

(fn `SetWorkCondition`
  (params (NewWorkCondition :type "/Game/ProjectLight/Modules/Struct/FWorkCondition Structure"))
  (bind _returnvalue (`self.GetComponentByClass` "/Game/ProjectLight/Components/BPC_EnergyPort_Input.BPC_EnergyPort_Input_C"))
  (bind _output_get (set `self.WorkCondition` NewWorkCondition))
  (`/Engine/EditorBlueprintResources/StandardMacros.IsValid` _returnvalue
    (:`Is Valid`
      (set `/Game/ProjectLight/Components/BPC_EnergyPort.EnergyType` (`.EnergyType_3_7D5E4D4A49DC81D3E274729DA9D08D31` (break `/Game/ProjectLight/Modules/Struct/FWorkCondition` _output_get)) _returnvalue))))

(fn `UninstallModule`
  (params (ContextObject :type "Object Object Reference")))

(fn `UserConstructionScript`)
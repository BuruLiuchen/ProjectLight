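; Motion module that yaws itself every tick while powered, using a data-table mode: oscillating angle, constant spin or homing.
; Homing uses cone traces to pick the nearest living enemy, with a looping sense timer that pauses while locked on and resumes when the target dies.
; Assist effects rescale speed, angle, sensing and energy-rate attributes by gameplay tag.
; An energy-consumption routine exists but is not wired into execution.
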(event `self.ReceiveBeginPlay`
  (bind _returnvalue (`|GetDataTableRow` (`self.DataTable`) (`self.ModuleName`))
    (:`then`
      (bind _output_get (set `self.ModuleInfo_Motion` _returnvalue))
      (bind (_basicinfo _workcondition) (break `/Game/ProjectLight/Modules/Struct/FModuleInfo_Motion` _output_get))
      (set `self.BasicInfo` _basicinfo)
      (`self.SetWorkCondition` _workcondition)
      (`self.InitAttributes`)
      (`parent.ReceiveBeginPlay`))))

(event `MotionProcess`
  (params (Interval :type "Float (double-precision)"))
  (`self.ChangeWorkState` "NewEnumerator2")
  (switch `/Game/ProjectLight/Modules/Enum/EMotionType` (`.MotionMode_32_E8E6633B4AC0E7B8BF1CA59D88094C30` (break `/Game/ProjectLight/Modules/Struct/FModuleInfo_Motion` (`self.ModuleInfo_Motion`)))
    (:`NewEnumerator0`
      (`self.RepeatAngleMove` Interval))
    (:`NewEnumerator1`
      (`self.RotationMove` Interval))
    (:`NewEnumerator2`
      (bind _homingtarget (`self.HomingTarget`)
        (:`then`
          (`self.RotateToTarget` _homingtarget Interval)
          (`/Game/ProjectLight/Blueprints/FunctionLibrary/BPL_Common.PauseTimer` (`self.HomingSenseTimer`) self)
          (add `/Game/ProjectLight/Characters/BP_Character_Base.OnCharacterDie` (`self.HomingTarget`) (delegate `TargetDie`)))
        (:`else`)))))

(event `TargetDie`
  (set `self.HomingTarget` null)
  (if (`KismetSystemLibrary.K2_IsValidTimerHandle` (`self.HomingSenseTimer`))
    (`/Game/ProjectLight/Blueprints/FunctionLibrary/BPL_Common.UnpauseTimer` (`self.HomingSenseTimer`) self)))

(event `self.ReceiveTick`
  (params (DeltaSeconds :type "Float (single-precision)"))
  (switch `/Game/ProjectLight/Modules/Enum/EWorkState` (`self.WorkState`)
    (:`NewEnumerator1`
      _)
    (:`NewEnumerator2`
      _)
    (:`NewEnumerator3`
      _))
  (`self.MotionProcess` DeltaSeconds))

(event `FindNextTarget`
  (bind _outhits (`/Game/ProjectLight/Blueprints/FunctionLibrary/BPL_Light.ConeLineTrace` :`Actor` (`self.ParentActor`) :`OuterAngle` (`self.SenseAngle`) :`OuterDistance` (`self.SenseDistance`)))
  (`self.FindNearstEnemy` _outhits))

(event `/Game/ProjectLight/Modules/InterfacesAndFunctions/BPI_AssistModule.ApplyAssistEffect`
  (params (AssistEffect :type "/Game/ProjectLight/Modules/Struct/FAssistEffectInfo Structure"))
  (`/Game/ProjectLight/Modules/InterfacesAndFunctions/BPL_AssistModule.ApplyAssist` AssistEffect (`self.AdjustRateMap`))
  (`self.SetAttributesAfterAssist` AssistEffect))

(event `/Game/ProjectLight/Modules/InterfacesAndFunctions/BPI_AssistModule.RemoveAssistEffect`
  (params (AssistEffect :type "/Game/ProjectLight/Modules/Struct/FAssistEffectInfo Structure"))
  (`/Game/ProjectLight/Modules/InterfacesAndFunctions/BPL_AssistModule.ApplyAssist` AssistEffect (`self.AdjustRateMap`))
  (`self.SetAttributesAfterAssist` AssistEffect))

(fn `ChangeWorkState`
  (params (NewWorkState :type "/Game/ProjectLight/Modules/Enum/EWorkState Enum" :default "NewEnumerator0") (ForceSwitch :type Boolean))
  (bind _homingsensetimer (`self.HomingSenseTimer`))
  (`parent.ChangeWorkState` NewWorkState ForceSwitch)
  (switch `/Game/ProjectLight/Modules/Enum/EWorkState` (`self.WorkState`)
    (:`NewEnumerator0`
      (`/Game/ProjectLight/Blueprints/FunctionLibrary/BPL_Common.PauseTimer` _homingsensetimer self :!label _label))
    (:`NewEnumerator4`
      (goto _label))
    (:`NewEnumerator2`
      (if (`KismetSystemLibrary.K2_IsValidTimerHandle` (`self.HomingSenseTimer`))
        (`/Game/ProjectLight/Blueprints/FunctionLibrary/BPL_Common.UnpauseTimer` _homingsensetimer self)
        (else
          (bind _returnvalue (`KismetSystemLibrary.K2_SetTimerDelegate` (`|CreateDelegate` :!event `FindNextTarget`) 0.5 true true))
          (set `self.HomingSenseTimer` _returnvalue))))))

(fn `CloseModule`
  (bind _homingsensetimer (`self.HomingSenseTimer`))
  (`parent.CloseModule`)
  (if (`KismetSystemLibrary.K2_IsValidTimerHandle` _homingsensetimer)
    (`KismetSystemLibrary.K2_ClearAndInvalidateTimerHandle` _homingsensetimer)))

(fn `FindNearstEnemy`
  (params (Array :type "Array of HitResult Structure"))
  (locals (MinDistance :type "Float (double-precision)" :default -1.0) (NearestEnemy :type "/Game/ProjectLight/Characters/Enemy/BP_Character_Enemy Object Reference") (CurrentDistance :type "Float (single-precision)" :default 0.0))
  (for _array_element Array
    (bind (_bblockinghit _binitialoverlap _time _distance _location _impactpoint _normal _impactnormal _physmat _hitactor) (`GameplayStatics.BreakHitResult` _array_element))
    (set `local.CurrentDistance` (`self.GetDistanceTo` _hitactor (`self.ParentActor`)))
    (bind _asbp_character_enemy (cast `/Game/ProjectLight/Characters/Enemy/BP_Character_Enemy` _hitactor))
    (if (and (`/Game/ProjectLight/Characters/BP_Character_Base.IsLiving` _asbp_character_enemy) (or (<= (`local.MinDistance`) -1.0) (< (`local.CurrentDistance`) (`local.MinDistance`))))
      (set `local.NearestEnemy` _asbp_character_enemy)
      (set `local.MinDistance` (`local.CurrentDistance`))))
  (set `self.HomingTarget` (`local.NearestEnemy`)))

(fn `GetAttributeByTag`
  (params (AttributeTag :type "GameplayTag Structure"))
  (returns (AttributeReturn :type "Float (double-precision)"))
  (locals (AdjustRate_Local :type "Float (double-precision)"))
  (bind _adjustrate_local (`local.AdjustRate_Local`))
  (bind ((`EnergyConsumePerSecond_27_B0D9AA454100F1724F25F2B243581B42` _energyconsumepersecond) (`RotateSpeed_33_6EFD5F3A46C3E751D7B394A027EE9BC9` _rotatespeed) (`RepeatAngle_34_3D539A304D3CA8686D02B6BE6E81787E` _repeatangle) (`SenseAngle_40_25142CFA4500660395053492031C5C79` _senseangle) (`SenseDistance_42_40886C7E469AC616F694F8A2F160558C` _sensedistance)) (break `/Game/ProjectLight/Modules/Struct/FModuleInfo_Motion` (`self.ModuleInfo_Motion`)))
  (set `local.AdjustRate_Local` (`parent.GetAttributeByTag` AttributeTag))
  (`|SwitchGameplayTag` AttributeTag
    (:`Module.Motion.EnergyConsumeRate`
      (return (* _energyconsumepersecond _adjustrate_local)))
    (:`Module.Motion.RepeatAngle`
      (return (* _repeatangle _adjustrate_local)))
    (:`Module.Motion.RotateSpeed`
      (return (* _rotatespeed _adjustrate_local)))
    (:`Module.Motion.SenseAngle`
      (return (* _senseangle _adjustrate_local)))
    (:`Module.Motion.SenseDistance`
      (return (* _sensedistance _adjustrate_local)))))

(fn `InitAttributes`
  (locals (ValueToSet :type "Float (double-precision)" :default 0.0))
  (bind ((`EnergyConsumePerSecond_27_B0D9AA454100F1724F25F2B243581B42` _energyconsumepersecond) (`RotateSpeed_33_6EFD5F3A46C3E751D7B394A027EE9BC9` _rotatespeed) (`RepeatAngle_34_3D539A304D3CA8686D02B6BE6E81787E` _repeatangle) (`SenseAngle_40_25142CFA4500660395053492031C5C79` _senseangle) (`SenseDistance_42_40886C7E469AC616F694F8A2F160558C` _sensedistance)) (break `/Game/ProjectLight/Modules/Struct/FModuleInfo_Motion` (`self.ModuleInfo_Motion`)))
  (`|ExecutionSequence`
    (:`then_0`
      (set `self.Energy Consume Per Second` _energyconsumepersecond))
    (:`then_1`
      (set `self.Repeat Angle` _repeatangle))
    (:`then_2`
      (set `self.Rotate Speed` _rotatespeed))
    (:`then_3`
      (set `self.SenseAngle` _senseangle))
    (:`then_4`
      (set `self.SenseDistance` _sensedistance))))

(fn `RepeatAngleMove`
  (params (Interval :type "Float (double-precision)"))
  (locals (RotateSpeed :type "Float (double-precision)"))
  (bind _returnvalue (* (`self.AngleDirection`) (`local.RotateSpeed`)))
  (set `local.RotateSpeed` (* Interval (`self.Rotate Speed`)))
  (if (>= (`KismetMathLibrary.Abs` (`self.AngleRotated`)) (`self.Repeat Angle`))
    (set `self.AngleDirection` (* (`self.AngleDirection`) -1.0)))
  (set `self.AngleRotated` (+ (`self.AngleRotated`) _returnvalue))
  (`self.K2_AddActorWorldRotation` (`KismetMathLibrary.MakeRotator` 0.0 0.0 _returnvalue)))

(fn `RotateToTarget`
  (params (Target :type "Actor Object Reference") (DeltaTime :type "Float (single-precision)"))
  (`self.K2_SetActorRotation` (`KismetMathLibrary.RInterpTo` (`self.K2_GetActorRotation`) (`KismetMathLibrary.MakeRotator` (.roll (`self.K2_GetActorRotation`)) (.pitch (`self.K2_GetActorRotation`)) (.yaw (`KismetMathLibrary.FindLookAtRotation` (`self.K2_GetActorLocation`) (`self.K2_GetActorLocation` Target)))) DeltaTime (* DeltaTime (`self.Rotate Speed`)))))

(fn `RotationMove`
  (params (Interval :type "Float (double-precision)"))
  (bind _returnvalue (* Interval (`self.Rotate Speed`)))
  (`self.K2_AddActorWorldRotation` (`KismetMathLibrary.MakeRotator` 0.0 0.0 (select `bool` (`self.IsClockwise`) :`false` (* _returnvalue -1.0) :`true` _returnvalue :!type "Float (single-precision)"))))

(fn `SetAttributesAfterAssist`
  (params (AssistEffect :type "/Game/ProjectLight/Modules/Struct/FAssistEffectInfo Structure"))
  (locals (ValueToSet :type "Float (double-precision)" :default 0.0))
  (bind _effecttypetag (break `/Game/ProjectLight/Modules/Struct/FAssistEffectInfo` AssistEffect))
  (bind _valuetoset (`local.ValueToSet`))
  (set `local.ValueToSet` (`self.GetAttributeByTag` _effecttypetag))
  (`|SwitchGameplayTag` _effecttypetag
    (:`Module.Motion.EnergyConsumeRate`
      (set `self.Energy Consume Per Second` _valuetoset))
    (:`Module.Motion.RepeatAngle`
      (set `self.Repeat Angle` _valuetoset))
    (:`Module.Motion.RotateSpeed`
      (set `self.Rotate Speed` _valuetoset))
    (:`Module.Motion.SenseAngle`
      (set `self.SenseAngle` _valuetoset))
    (:`Module.Motion.SenseDistance`
      (set `self.SenseDistance` _valuetoset))))

(fn `UserConstructionScript`
  (`parent.UserConstructionScript`))
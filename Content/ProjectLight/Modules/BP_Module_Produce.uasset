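; Producer module that converts one energy type into another, configured from a data table row looked up by module name.
; A looping timer consumes input energy scaled by work efficiency and charges the output port by the transform efficiency.
; The timer pauses when work conditions fail, including a full output, and resumes on port volume changes.
; Assist effects adjust the interval and efficiency through gameplay-tagged attributes.
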(event `self.ReceiveBeginPlay`
  (bind _returnvalue (`|GetDataTableRow` (`self.DataTable`) (`self.ModuleName`))
    (:`then`
      (bind _output_get (set `self.ModuleInfo_Produce` _returnvalue))
      (bind (_basicinfo _workcondition _inputenergy _outputenergy) (break `/Game/ProjectLight/Modules/Struct/FModuleInfo_Produce` _output_get))
      (set `self.BasicInfo` _basicinfo)
      (set `self.WorkCondition` _workcondition)
      (set `/Game/ProjectLight/Components/BPC_EnergyPort.EnergyType` _inputenergy (`self.BPC_EnergyPort_Input`))
      (set `/Game/ProjectLight/Components/BPC_EnergyPort.EnergyType` _outputenergy (`self.BPC_EnergyPort_Output`))
      (`parent.ReceiveBeginPlay`)
      (`self.TryToStartProduce`))))

(event `TryToStartProduce`
  (bind _returnvalue (`KismetSystemLibrary.K2_SetTimerDelegate` (delegate `ProduceProcess`) (`self.GetAttributeByTag` (struct :`TagName` "Module.Produce.ProduceInterval")) true))
  (set `self.ProduceTimer` _returnvalue))

(event `ProduceProcess`
  (bind (_basicinfo _workcondition _inputenergy _outputenergy _transformefficiency _volumeinputonetime) (break `/Game/ProjectLight/Modules/Struct/FModuleInfo_Produce` (`self.ModuleInfo_Produce`)))
  (bind _canwork (`self.CheckWorkCondition`))
  (if _canwork
    (`self.ChangeWorkState` "NewEnumerator2")
    (bind _volumeconsumed (`self.ConsumeInputVolume` _inputenergy (* _volumeinputonetime (`self.WorkEfficiency`))))
    (`self.ChargeOutputVolume` _outputenergy (* _volumeconsumed (`self.GetAttributeByTag` (struct :`TagName` "Module.Produce.TransformEfficiency"))))
    (else
      (`/Game/ProjectLight/Blueprints/FunctionLibrary/BPL_Common.PauseTimer` (`self.ProduceTimer`) self)
      (`self.ChangeWorkState` "NewEnumerator4"))))

(event `self.BPC_EnergyPort_Output.OnCurrentVolumeChange`
  (if (not (`/Game/ProjectLight/Components/BPC_EnergyPort.CurrentVolumeIsEmpty` (`self.BPC_EnergyPort_Input`)))
    (`/Game/ProjectLight/Blueprints/FunctionLibrary/BPL_Common.UnpauseTimer` (`self.ProduceTimer`) self :!label _label)))

(event `self.BPC_EnergyPort_Input.OnCurrentVolumeChange`
  (if (not (`/Game/ProjectLight/Components/BPC_EnergyPort.CurrentVolumeIsFull` (`self.BPC_EnergyPort_Output`)))
    (goto _label)))

(event `/Game/ProjectLight/Modules/InterfacesAndFunctions/BPI_AssistModule.ApplyAssistEffect`
  (params (AssistEffect :type "/Game/ProjectLight/Modules/Struct/FAssistEffectInfo Structure"))
  (`/Game/ProjectLight/Modules/InterfacesAndFunctions/BPL_AssistModule.ApplyAssist` AssistEffect (`self.AdjustRateMap`)))

(event `/Game/ProjectLight/Modules/InterfacesAndFunctions/BPI_AssistModule.RemoveAssistEffect`
  (params (AssistEffect :type "/Game/ProjectLight/Modules/Struct/FAssistEffectInfo Structure"))
  (`/Game/ProjectLight/Modules/InterfacesAndFunctions/BPL_AssistModule.ApplyAssist` AssistEffect (`self.AdjustRateMap`) true))

(fn `CheckWorkCondition`
  (returns (CanWork :type Boolean))
  (bind _canwork (`parent.CheckWorkCondition`))
  (return (and _canwork (not (`/Game/ProjectLight/Components/BPC_EnergyPort.CurrentVolumeIsFull` (`self.BPC_EnergyPort_Output`))))))

(fn `CloseModule`
  (`parent.CloseModule`)
  (`KismetSystemLibrary.K2_ClearAndInvalidateTimerHandle` (`self.ProduceTimer`)))

(fn `GetAttributeByTag`
  (params (AttributeTag :type "GameplayTag Structure"))
  (returns (AttributeReturn :type "Float (double-precision)"))
  (locals (AdjustRate_Local :type "Float (double-precision)"))
  (bind _adjustrate_local (`local.AdjustRate_Local`))
  (bind ((`TransformEfficiency_8_851798684E1C3FCF8E5A92A5B4705664` _transformefficiency) (`ProduceInterval_14_2FFD068047E8FB66A1AD48B290AF564A` _produceinterval)) (break `/Game/ProjectLight/Modules/Struct/FModuleInfo_Produce` (`self.ModuleInfo_Produce`)))
  (set `local.AdjustRate_Local` (`parent.GetAttributeByTag` AttributeTag))
  (`|SwitchGameplayTag` AttributeTag
    (:`Module.Produce.ProduceInterval`
      (return (/ _produceinterval _adjustrate_local)))
    (:`Module.Produce.TransformEfficiency`
      (return (* _transformefficiency _adjustrate_local)))))

(fn `OpenModule`
  (`parent.OpenModule`)
  (`self.TryToStartProduce`))

(fn `UserConstructionScript`
  (`parent.UserConstructionScript`))
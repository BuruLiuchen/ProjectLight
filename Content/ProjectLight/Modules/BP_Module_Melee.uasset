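; Melee weapon module that loads its stats and attack montage from a data table, scaled by assist-effect rate adjustments.
; Opening it checks work conditions, snaps the weapon to the hand socket, spends energy and plays the montage.
; Between attack start and end events, box overlaps damage each qualifying unit once, excluding the owner.
; Closing waits for any active montage to end before returning the weapon to its module socket.
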(event `self.ReceiveBeginPlay`
  (bind (_basicinfo _workcondition) (break `/Game/ProjectLight/Modules/Struct/FModuleInfo_Melee` (`self.ModuleInfo_Melee`)))
  (bind _returnvalue (`|GetDataTableRow` (`self.DataTable`) (`self.ModuleName`))
    (:`then`
      (set `self.ModuleInfo_Melee` _returnvalue)
      (`/Game/ProjectLight/Components/BPC_EnergyPort.SetVolumeCap` (`self.BPC_EnergyPort_Input`) (`self.GetAttributeByTag` (struct :`TagName` "Module.Melee.EnergyConsumeRate")))
      (set `self.BasicInfo` _basicinfo)
      (set `self.WorkCondition` _workcondition)
      (`parent.ReceiveBeginPlay`))))

(event `StartMeleeAttack`
  (`KismetArrayLibrary.Array_Clear` (`self.HitActors`))
  (set `self.IsAttacking` true))

(event `EndMeleeAttack`
  (`KismetArrayLibrary.Array_Clear` (`self.HitActors`))
  (set `self.IsAttacking` false))

(event `self.Box.OnComponentBeginOverlap`
  (params (OverlappedComponent :type "PrimitiveComponent Object Reference") (OtherActor :type "Actor Object Reference") (OtherComp :type "PrimitiveComponent Object Reference") (OtherBodyIndex :type Integer) (bFromSweep :type Boolean) (SweepResult :type "HitResult Structure (by ref)"))
  (`self.MeleeAttackProcess` OtherActor))

(event `self.Box.OnComponentEndOverlap`
  (params (OverlappedComponent :type "PrimitiveComponent Object Reference") (OtherActor :type "Actor Object Reference") (OtherComp :type "PrimitiveComponent Object Reference") (OtherBodyIndex :type Integer))
  (`self.MeleeAttackProcess` OtherActor))

(event `/Game/ProjectLight/Modules/InterfacesAndFunctions/BPI_AssistModule.ApplyAssistEffect`
  (params (AssistEffect :type "/Game/ProjectLight/Modules/Struct/FAssistEffectInfo Structure"))
  (`/Game/ProjectLight/Modules/InterfacesAndFunctions/BPL_AssistModule.ApplyAssist` AssistEffect (`self.AdjustRateMap`))
  (`/Game/ProjectLight/Components/BPC_EnergyPort.SetVolumeCap` (`self.BPC_EnergyPort_Input`) (`self.GetAttributeByTag` (struct :`TagName` "Module.Melee.EnergyConsumeRate"))))

(event `/Game/ProjectLight/Modules/InterfacesAndFunctions/BPI_AssistModule.RemoveAssistEffect`
  (params (AssistEffect :type "/Game/ProjectLight/Modules/Struct/FAssistEffectInfo Structure"))
  (`/Game/ProjectLight/Modules/InterfacesAndFunctions/BPL_AssistModule.ApplyAssist` AssistEffect (`self.AdjustRateMap`) true)
  (`/Game/ProjectLight/Components/BPC_EnergyPort.SetVolumeCap` (`self.BPC_EnergyPort_Input`) (`self.GetAttributeByTag` (struct :`TagName` "Module.Melee.EnergyConsumeRate"))))

(fn `CloseModule`
  (bind _returnvalue (`SkeletalMeshComponent.GetAnimInstance` (`self.GetComponentByClass` (`self.ParentActor`) "/Script/Engine.SkeletalMeshComponent")))
  (`/Engine/EditorBlueprintResources/StandardMacros.IsValid` (`AnimInstance.GetCurrentActiveMontage` _returnvalue)
    (:`Is Valid`
      (add `AnimInstance.OnMontageEnded` _returnvalue (`|CreateDelegate` :!event `OnMontageEnded`)))
    (:`Is Not Valid`
      (`self.ResetWeaponLocation`)
      (remove `AnimInstance.OnMontageEnded` _returnvalue (`|CreateDelegate` :!event `OnMontageEnded`))
      (`parent.CloseModule`))))

(fn `GetAttributeByTag`
  (params (AttributeTag :type "GameplayTag Structure"))
  (returns (AttributeReturn :type "Float (double-precision)"))
  (locals (AdjustRate_Local :type "Float (double-precision)"))
  (bind _adjustrate_local (`local.AdjustRate_Local`))
  (bind ((`EnergyConsumeOneTime_30_B0D9AA454100F1724F25F2B243581B42` _energyconsumeonetime) (`AttackSpeed_31_6EFD5F3A46C3E751D7B394A027EE9BC9` _attackspeed) (`AttackPower_32_3D539A304D3CA8686D02B6BE6E81787E` _attackpower)) (break `/Game/ProjectLight/Modules/Struct/FModuleInfo_Melee` (`self.ModuleInfo_Melee`)))
  (set `local.AdjustRate_Local` (`parent.GetAttributeByTag` AttributeTag))
  (`|SwitchGameplayTag` AttributeTag
    (:`Module.Melee.AttackPower`
      (return (* _attackpower _adjustrate_local)))
    (:`Module.Melee.AttackSpeed`
      (return (* _attackspeed _adjustrate_local)))
    (:`Module.Melee.EnergyConsumeRate`
      (return (* _energyconsumeonetime _adjustrate_local)))))

(fn `MeleeAttackProcess`
  (params (OverlapedActor :type "Actor Object Reference"))
  (bind _overlapedactor (`local.OverlapedActor`))
  (bind _overlapedactor_2 (`local.OverlapedActor`))
  (bind _unittype (message `/Game/ProjectLight/Blueprints/Interfaces/BPI_Common.GetUnitType` OverlapedActor))
  (if (`|EnumEquality` _unittype "NewEnumerator1")
    (if (`self.IsAttacking`)
      (if (`KismetMathLibrary.BooleanNOR` (== _overlapedactor (`self.ParentActor`)) (`KismetArrayLibrary.Array_Contains` (`self.HitActors`) _overlapedactor))
        (`KismetArrayLibrary.Array_AddUnique` (`self.HitActors`) _overlapedactor_2)
        (`GameplayStatics.ApplyDamage` _overlapedactor_2 (`self.GetAttributeByTag` (struct :`TagName` "Module.Melee.AttackPower")))))))

(fn `OnMontageEnded`
  (params (Montage :type "AnimMontage Object Reference") (bInterrupted :type Boolean))
  (`self.CloseModule`))

(fn `OpenModule`
  (returns (OpenSuccess :type Boolean))
  (bind (_workcondition_norequest _workcondition_energytype) (break `/Game/ProjectLight/Modules/Struct/FWorkCondition` (`self.WorkCondition`)))
  (bind _returnvalue (`self.GetComponentByClass` (`self.ParentActor`) "/Script/Engine.SkeletalMeshComponent"))
  (`parent.OpenModule`)
  (bind _canwork (`self.CheckWorkCondition`))
  (if _canwork
    (if (not (`self.WeaponInHand`))
      (`self.K2_AttachToComponent` _returnvalue "Weapon_R" "SnapToTarget" "SnapToTarget" "KeepWorld"))
    (`/Engine/EditorBlueprintResources/StandardMacros.IsValid` (`AnimInstance.GetCurrentActiveMontage` (`SkeletalMeshComponent.GetAnimInstance` _returnvalue))
      (:`Is Not Valid`
        (`self.ConsumeInputVolume` _workcondition_energytype (`self.GetAttributeByTag` (struct :`TagName` "Module.Melee.EnergyConsumeRate")))
        (message `/Game/ProjectLight/Characters/Interfaces/BPI_Character.PlayMontage` (`self.ParentActor`) (`.AttackMontage_34_F01804FE4543C69B946D9BBA7E3701D7` (break `/Game/ProjectLight/Modules/Struct/FModuleInfo_Melee` (`self.ModuleInfo_Melee`))) (`self.GetAttributeByTag` (struct :`TagName` "Module.Melee.AttackSpeed")))
        (return true)))
    (else
      (return false))))

(fn `ResetWeaponLocation`
  (`self.K2_AttachToComponent` (`self.GetComponentByClass` (`self.ParentActor`) "/Script/Engine.SkeletalMeshComponent") "module_melee" "SnapToTarget" "SnapToTarget" "KeepWorld"))

(fn `UserConstructionScript`
  (`parent.UserConstructionScript`))
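; Energy storage module that buffers one energy type between an input port and an output port, configured from a data table row.
; Two looping timers drain input into storage and charge output from it, pausing when blocked and unpausing on port volume changes.
; Assist effects update a rate map and re-read the capacity through GetAttributeByTag, which returns zero here with its scaling multiply unconnected.
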(event `self.ReceiveBeginPlay`
  (bind _returnvalue (`|GetDataTableRow` (`self.DataTable`) (`self.ModuleName`))
    (:`then`
      (bind _output_get (set `self.ModuleInfo_Storage` _returnvalue))
      (bind (_basicinfo _workcondition _storageenergy _storagecap) (break `/Game/ProjectLight/Modules/Struct/FModuleInfo_Storage` _output_get))
      (set `self.BasicInfo` _basicinfo)
      (set `self.WorkCondition` _workcondition)
      (set `self.Storage Energy` _storageenergy)
      (set `self.Storage Cap` _storagecap)
      (`self.InitStorageModulePorts`)
      (`parent.ReceiveBeginPlay`)
      (bind _returnvalue_2 (`KismetSystemLibrary.K2_SetTimerDelegate` (delegate `StoreEnergy`) (`self.StoreInterval`) true true))
      (set `self.StoreTimer` _returnvalue_2)
      (bind _returnvalue_3 (`KismetSystemLibrary.K2_SetTimerDelegate` (delegate `ChargeOutput`) (`self.StoreInterval`) true true))
      (set `self.ChargeTimer` _returnvalue_3))))

(event `StoreEnergy`
  (`self.StoreToStorage` (`self.StoreInterval`)))

(event `ChargeOutput`
  (`self.ChargeToOutput` (`self.StoreInterval`)))

(event `StoreToStorage`
  (params (Interval :type "Float (double-precision)"))
  (if (`/Game/ProjectLight/Components/BPC_EnergyPort.CurrentVolumeIsEmpty` (`self.BPC_EnergyPort_Input`))
    (`/Game/ProjectLight/Blueprints/FunctionLibrary/BPL_Common.PauseTimer` (`self.StoreTimer`) self :!label _label)
    (elif (>= (`self.CurrentStorage`) (`self.Storage Cap`))
      (goto _label)
      (else
        (bind _volumeconsumed (`self.ConsumeInputVolume` (`self.Storage Energy`) (* Interval (`self.StoreVolumePerSecond`))))
        (`self.ChangeStorage` _volumeconsumed)))))

(event `ChargeToOutput`
  (params (Interval :type "Float (double-precision)"))
  (bind _returnvalue (* Interval (`self.StoreVolumePerSecond`)))
  (if (`/Game/ProjectLight/Components/BPC_EnergyPort.CurrentVolumeIsFull` (`self.BPC_EnergyPort_Output`))
    (`/Game/ProjectLight/Blueprints/FunctionLibrary/BPL_Common.PauseTimer` (`self.ChargeTimer`) self :!label _label_2)
    (elif (<= (`self.CurrentStorage`) 0.0)
      (goto _label_2)
      (else
        (`self.ChangeStorage` (* _returnvalue -1.0))
        (`self.ChargeOutputVolume` (`self.Storage Energy`) _returnvalue)))))

(event `self.BPC_EnergyPort_Output.OnCurrentVolumeChange`
  (`|ExecutionSequence` :!label _label_3
    (:`then_0`
      (if (>= (`self.CurrentStorage`) 0.0)
        (`/Game/ProjectLight/Blueprints/FunctionLibrary/BPL_Common.UnpauseTimer` (`self.ChargeTimer`) self)))
    (:`then_1`
      (if (< (`self.CurrentStorage`) (`self.Storage Cap`))
        (`/Game/ProjectLight/Blueprints/FunctionLibrary/BPL_Common.UnpauseTimer` (`self.StoreTimer`) self)))))

(event `self.BPC_EnergyPort_Input.OnCurrentVolumeChange`
  (goto _label_3))

(event `/Game/ProjectLight/Modules/InterfacesAndFunctions/BPI_AssistModule.ApplyAssistEffect`
  (params (AssistEffect :type "/Game/ProjectLight/Modules/Struct/FAssistEffectInfo Structure"))
  (`/Game/ProjectLight/Modules/InterfacesAndFunctions/BPL_AssistModule.ApplyAssist` AssistEffect (`self.AdjustRateMap`))
  (set `self.Storage Cap` (`self.GetAttributeByTag` (struct :`TagName` "Module.Storage.StorageCap"))))

(event `/Game/ProjectLight/Modules/InterfacesAndFunctions/BPI_AssistModule.RemoveAssistEffect`
  (params (AssistEffect :type "/Game/ProjectLight/Modules/Struct/FAssistEffectInfo Structure"))
  (`/Game/ProjectLight/Modules/InterfacesAndFunctions/BPL_AssistModule.ApplyAssist` AssistEffect (`self.AdjustRateMap`) true)
  (set `self.Storage Cap` (`self.GetAttributeByTag` (struct :`TagName` "Module.Storage.StorageCap"))))

(fn `ChangeStorage`
  (params (DeltaVolume :type "Float (double-precision)"))
  (bind _output_get (set `self.CurrentStorage` (`KismetMathLibrary.FClamp` (+ (`self.CurrentStorage`) DeltaVolume) 0.0 (`self.Storage Cap`))))
  (if (< _output_get (`self.Storage Cap`))
    _))

(fn `GetAttributeByTag`
  (params (AttributeTag :type "GameplayTag Structure"))
  (returns (AttributeReturn :type "Float (double-precision)"))
  (locals (AdjustRate_Local :type "Float (double-precision)"))
  (bind (_value _returnvalue) (`BlueprintMapLibrary.Map_Find` (`self.AdjustRateMap`) AttributeTag))
  (set `local.AdjustRate_Local` _value)
  (if _returnvalue
    (`|SwitchGameplayTag` AttributeTag
      (:`Module.Storage.StorageCap`
        (return 0.0)))
    (else
      (`BlueprintMapLibrary.Map_Add` (`self.AdjustRateMap`) AttributeTag 1.0)
      (return 0.0))))

(fn `InitStorageModulePorts`
  (set `/Game/ProjectLight/Components/BPC_EnergyPort.EnergyType` (`self.Storage Energy`) (`self.BPC_EnergyPort_Input`))
  (set `/Game/ProjectLight/Components/BPC_EnergyPort.EnergyType` (`self.Storage Energy`) (`self.BPC_EnergyPort_Output`)))

(fn `UserConstructionScript`
  (`parent.UserConstructionScript`))
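; Assist module Blueprint that grants data-driven assist effects to the objects it is installed on.
; BeginPlay loads its row by ModuleName, setting basic info and work condition; parent BeginPlay runs only if found.
; Installing adds the context to LinkedObjects and sends every effect to all linked objects, including earlier ones.
; Uninstalling removes the effects from all linked objects and clears the list, regardless of context.
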(event `self.ReceiveBeginPlay`
  (bind _returnvalue (`|GetDataTableRow` (`self.DataTable`) (`self.ModuleName`))
    (:`then`
      (bind _output_get (set `self.ModuleInfo_Assist` _returnvalue))
      (bind (_basicinfo _workcondition) (break `/Game/ProjectLight/Modules/Struct/FModuleInfo_Assist` _output_get))
      (set `self.BasicInfo` _basicinfo)
      (`self.SetWorkCondition` _workcondition)
      (`parent.ReceiveBeginPlay`))))

(fn `InstallModule`
  (params (ContextObject :type "Object Object Reference"))
  (`parent.InstallModule` ContextObject)
  (`KismetArrayLibrary.Array_AddUnique` (`self.LinkedObjects`) ContextObject)
  (for _array_element (`.EffectList_27_08B5289E48878F41BFCA57A4E1A6AC60` (break `/Game/ProjectLight/Modules/Struct/FModuleInfo_Assist` (`self.ModuleInfo_Assist`)))
    (for _array_element_2 (`self.LinkedObjects`)
      (message `/Game/ProjectLight/Modules/InterfacesAndFunctions/BPI_AssistModule.ApplyAssistEffect` _array_element_2 _array_element))))

(fn `UninstallModule`
  (params (ContextObject :type "Object Object Reference"))
  (`parent.UninstallModule` ContextObject)
  (for _array_element (`.EffectList_27_08B5289E48878F41BFCA57A4E1A6AC60` (break `/Game/ProjectLight/Modules/Struct/FModuleInfo_Assist` (`self.ModuleInfo_Assist`)))
    (for _array_element_2 (`self.LinkedObjects`)
      (message `/Game/ProjectLight/Modules/InterfacesAndFunctions/BPI_AssistModule.RemoveAssistEffect` _array_element_2 _array_element)))
  (`KismetArrayLibrary.Array_Clear` (`self.LinkedObjects`)))

(fn `UserConstructionScript`
  (`parent.UserConstructionScript`))
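; Base character Blueprint for battle-stage units, handling health, movement speed, death and an overhead info display.
; On BeginPlay it registers with GM_BattleStage's unit list and gives its info widget component a UMG display bound to itself.
; Damage clamps health and triggers hit or death events, with death playing a montage, switching collision and hiding the widget.
; It also receives light through energy-pass events and resolves tag-keyed attributes as base values times adjustable rates.
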(event `self.ReceiveBeginPlay`
  (set `CharacterMovementComponent.MaxWalkSpeed` (`self.InitalMovementSpeed`) (`self.CharacterMovement`))
  (bind _asgm_battle_stage (cast `/Game/ProjectLight/BattleScene/GM_BattleStage` (`GameplayStatics.GetGameMode`)))
  (`/Game/ProjectLight/BattleScene/GM_BattleStage.RegisterToUnitList` _asgm_battle_stage self)
  (bind _returnvalue (`|CreateWidget` "/Game/ProjectLight/UMG/Items/UMG_BasicInfoDisplay.UMG_BasicInfoDisplay_C" null (`self.UnitType`) self))
  (`WidgetComponent.SetWidget` (`self.BaseInfoWidget`) _returnvalue))

(event `/Game/ProjectLight/Characters/Interfaces/BPI_Character.SetMovementSpeedRate`
  (params (NewSpeedRate :type "Float (double-precision)"))
  (set `CharacterMovementComponent.MaxWalkSpeed` (* NewSpeedRate (`self.InitalMovementSpeed`)) (`self.CharacterMovement`)))

(event `self.ReceiveAnyDamage`
  (params (Damage :type "Float (single-precision)") (DamageType :type "DamageType Object Reference") (InstigatedBy :type "Controller Object Reference") (DamageCauser :type "Actor Object Reference"))
  (if (`self.IsLiving`)
    (bind _output_get (set `self.HealthPoint` (`KismetMathLibrary.FClamp` (- (`self.HealthPoint`) Damage) 0.0 (`self.MaxHealthPoint`))))
    (if (<= _output_get 0.0)
      (set `self.IsLiving` false)
      (`self.CharacterDie`)
      (else
        (`self.CharacterDamaged`)))))

(event `CharacterDamaged`)

(event `CharacterDie`
  (`|PlayMontage` (`self.Mesh`) (`self.DeathMontage`)
    (:`then`
      (`PrimitiveComponent.SetCollisionProfileName` (`self.CapsuleComponent`) "DeadCharacter" true)
      (`SceneComponent.SetVisibility` (`self.BaseInfoWidget`) false false)
      (`self.OnCharacterDie`))))

(event `/Game/ProjectLight/Components/Interfaces/BPI_Energy.EnergyPass_UDP`
  (params (EnergyInfo :type "/Game/ProjectLight/Components/Struct/FEnergyInfo Structure") (EnergySourceType :type "/Game/ProjectLight/Components/Enum/EEnergySourceType Enum" :default "NewEnumerator0"))
  (bind (_type _volume) (break `/Game/ProjectLight/Components/Struct/FEnergyInfo` EnergyInfo))
  (if (`|EnumEquality` _type "NewEnumerator0")
    (`/Game/ProjectLight/Blueprints/FunctionLibrary/BPL_Energy.ReceiveLight` self _volume)
    (`self.LightTaken`)))

(event `NoLightTake`)

(event `LightTaken`)

(fn `ChangeMaxHealth`
  (params (NewMaxHealth :type "Float (double-precision)") (ResetHealth :type Boolean))
  (bind _output_get (set `self.MaxHealthPoint` NewMaxHealth))
  (if ResetHealth
    (set `self.HealthPoint` (`self.MaxHealthPoint`))
    (else
      (set `self.HealthPoint` (`KismetMathLibrary.FMin` _output_get (`self.HealthPoint`))))))

(fn `GetAttributeByTag`
  (params (AttributeTag :type "GameplayTag Structure"))
  (returns (AttributeReturn :type "Float (double-precision)"))
  (locals (AdjustRate_Local :type "Float (double-precision)"))
  (bind (_characterbaseinfo_maxhealth _characterbaseinfo_movespeed _characterbaseinfo_pickrange) (break `/Game/ProjectLight/Characters/Hero/Struct/FCharacterInfo` (`self.CharacterBaseInfo`)))
  (bind _adjustrate_local (`local.AdjustRate_Local`))
  (bind _adjustratemap (`self.AdjustRateMap`))
  (bind (_value _returnvalue) (`BlueprintMapLibrary.Map_Find` _adjustratemap AttributeTag))
  (set `local.AdjustRate_Local` _value)
  (if (not _returnvalue)
    (`BlueprintMapLibrary.Map_Add` _adjustratemap AttributeTag 1.0)
    (set `local.AdjustRate_Local` 1.0))
  (`|SwitchGameplayTag` AttributeTag
    (:`Unit.Base.MaxHealth`
      (return (* _characterbaseinfo_maxhealth _adjustrate_local)))
    (:`Player.Base.MoveSpeed`
      (return (* _characterbaseinfo_movespeed _adjustrate_local)))
    (:`Player.Base.PickRange`
      (return (* _characterbaseinfo_pickrange _adjustrate_local)))))

(fn `GetBuildingType`
  (returns (BuildingType :type "/Game/ProjectLight/Buildings/EBuildingType Enum"))
  (return "NewEnumerator0"))

(fn `GetIsActive`
  (returns (IsActive :type Boolean))
  (return true))

(fn `GetIsLiving`
  (returns (IsLiving :type Boolean))
  (return (`self.IsLiving`)))

(fn `GetName`
  (returns (ReturnName :type Name))
  (return (`self.CharacterName`)))

(fn `GetUnitType`
  (returns (UnitType :type "/Game/ProjectLight/Blueprints/Enums/EUnitType Enum"))
  (return "NewEnumerator1"))

(fn `GetVolumeForDispaly`
  (returns (Volume :type "Float (double-precision)") (MaxVolume :type "Float (double-precision)"))
  (return (`self.HealthPoint`) (`self.MaxHealthPoint`)))

(fn `UserConstructionScript`)
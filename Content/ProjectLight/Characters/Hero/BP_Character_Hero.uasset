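; BP_Character_Hero is the player hero, with data-table stats and upgrades that grant modules and buildings.
; It spawns socket-attached modules, links assist modules from its inventory, and recomputes tagged health, speed and pickup radius when assist effects change.
; A pickup sphere collects resources on overlap.
; Timers drive looping darkness damage after light is lost and delayed health recovery that consumes stored energy.
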(event `self.ReceiveBeginPlay`
  (bind _bpc_inventorycomponent (`self.BPC_InventoryComponent`))
  (`self.UpdatePlayerBaseInfo` (`self.CharacterName`))
  (`parent.ReceiveBeginPlay`)
  (`/Game/ProjectLight/Characters/Components/BPC_InventoryComponent.SetHeroCharacter` _bpc_inventorycomponent self)
  (`/Game/ProjectLight/Characters/Components/BPC_InventoryComponent.InitDefaultEquipment` _bpc_inventorycomponent)
  (`KismetSystemLibrary.Delay` 0.2)
  (`self.InitAssistModules`)
  (`/Game/ProjectLight/Components/BPC_PortManageComponent.UpdateSenseRange` (`self.BPC_PortManageComponent`) (`self.SenseRange`)))

(event `CharacterUpgrade`
  (`self.UpdatePlayerBaseInfo` (`self.CharacterName`)))

(event `/Game/ProjectLight/Characters/Interfaces/BPI_Character.PlayMontage`
  (params (MontageToPlay :type "AnimMontage Object Reference") (PlayRate :type "Float (double-precision)"))
  (`/Engine/EditorBlueprintResources/StandardMacros.IsValid` (`self.GetCurrentMontage`)
    (:`Is Not Valid`
      (`|PlayMontage` (`self.Mesh`) MontageToPlay PlayRate))))

(event `/Game/ProjectLight/Modules/InterfacesAndFunctions/BPI_AssistModule.ApplyAssistEffect`
  (params (AssistEffect :type "/Game/ProjectLight/Modules/Struct/FAssistEffectInfo Structure"))
  (`/Game/ProjectLight/Modules/InterfacesAndFunctions/BPL_AssistModule.ApplyAssist` AssistEffect (`self.AdjustRateMap`))
  (`self.UpdateAttribute`))

(event `/Game/ProjectLight/Modules/InterfacesAndFunctions/BPI_AssistModule.RemoveAssistEffect`
  (params (AssistEffect :type "/Game/ProjectLight/Modules/Struct/FAssistEffectInfo Structure"))
  (`/Game/ProjectLight/Modules/InterfacesAndFunctions/BPL_AssistModule.ApplyAssist` AssistEffect (`self.AdjustRateMap`) true)
  (`self.UpdateAttribute`))

(event `self.PickRangeSphere.OnComponentBeginOverlap`
  (params (OverlappedComponent :type "PrimitiveComponent Object Reference") (OtherActor :type "Actor Object Reference") (OtherComp :type "PrimitiveComponent Object Reference") (OtherBodyIndex :type Integer) (bFromSweep :type Boolean) (SweepResult :type "HitResult Structure (by ref)"))
  (bind _asbp_resource_base (cast `/Game/ProjectLight/Blueprints/BP_Resource_Base` OtherActor))
  (`/Game/ProjectLight/Blueprints/BP_Resource_Base.PickedUp` _asbp_resource_base self))

(event `self.LightTaken`
  (bind _darkdamagetimer (`self.DarkDamageTimer`))
  (bind _returnvalue (`KismetSystemLibrary.K2_SetTimerDelegate` (delegate `LightLose`) 1.0 false true))
  (set `self.LightCheckTimer` _returnvalue)
  (if (`KismetSystemLibrary.K2_IsValidTimerHandle` _darkdamagetimer)
    (`KismetSystemLibrary.K2_ClearAndInvalidateTimerHandle` _darkdamagetimer)))

(event `LightLose`
  (bind _lightchecktimer (`self.LightCheckTimer`))
  (`self.NoLightTake`)
  (if (`KismetSystemLibrary.K2_IsValidTimerHandle` _lightchecktimer)
    (`KismetSystemLibrary.K2_ClearAndInvalidateTimerHandle` _lightchecktimer)))

(event `self.NoLightTake`
  (bind _darkdamageinfo_darkdamageinterval (break `/Game/ProjectLight/Blueprints/Struct/FDarkDamageInfo` (`self.DarkDamageInfo`)))
  (bind _returnvalue (`KismetSystemLibrary.K2_SetTimerDelegate` (`|CreateDelegate` :!event `DarkDamage`) _darkdamageinfo_darkdamageinterval true true))
  (set `self.DarkDamageTimer` _returnvalue))

(event `DarkDamage`
  (`/Game/ProjectLight/Blueprints/FunctionLibrary/BPL_Common.ApplyDarkDamage` self))

(event `self.BPC_InventoryComponent.OnModuleInstall`
  (params (InstalledModule :type "/Game/ProjectLight/Modules/BP_Module_Base Object Reference"))
  (`self.InitAssistModules`))

(event `self.CharacterDamaged`
  (`self.TryToStartRecovery`))

(event `TryToStartRecovery`
  (bind _recoverytimer (`self.RecoveryTimer`))
  (`KismetSystemLibrary.K2_SetTimerDelegate` (delegate `StartRecovery`) (`self.RecoveryStartTime`))
  (if (`KismetSystemLibrary.K2_IsValidTimerHandle` _recoverytimer)
    (`KismetSystemLibrary.K2_ClearAndInvalidateTimerHandle` _recoverytimer)))

(event `StartRecovery`
  (if (and (not (`self.IsRecoverying`)) (< (`self.HealthPoint`) (`self.MaxHealthPoint`))) :!label _label
    (bind _returnvalue (`KismetSystemLibrary.K2_SetTimerDelegate` (delegate `KeepRecovery`) 0.5 true true))
    (set `self.RecoveryTimer` _returnvalue)
    (set `self.IsRecoverying` true)))

(event `self.BPC_ResourceComponent.OnCurrentStorageChange`
  (goto _label))

(event `KeepRecovery`
  (bind _recoverytimer (`self.RecoveryTimer`))
  (bind _resourcecomponent (`/Game/ProjectLight/Blueprints/FunctionLibrary/BML_Common.GetResourceComponent` (`GameplayStatics.GetPlayerCharacter` 0))
    (:`IsValid`
      (bind _consumesucess (`/Game/ProjectLight/Characters/Components/BPC_ResourceComponent.ConsumeStorageValue` _resourcecomponent "NewEnumerator2" 0.5))
      (if _consumesucess
        (bind _output_get (set `self.HealthPoint` (`KismetMathLibrary.FClamp` (+ (`self.HealthPoint`) 1.0) 0.0 (`self.MaxHealthPoint`))))
        (if (>= _output_get (`self.MaxHealthPoint`))
          (if (`KismetSystemLibrary.K2_IsValidTimerHandle` _recoverytimer)
            (`KismetSystemLibrary.K2_ClearAndInvalidateTimerHandle` _recoverytimer)
            (set `self.IsRecoverying` false)))))))

(fn `GetUnitType`
  (returns (UnitType :type "/Game/ProjectLight/Blueprints/Enums/EUnitType Enum"))
  (return "NewEnumerator0"))

(fn `InitAssistModules`
  (bind _bpc_inventorycomponent (`self.BPC_InventoryComponent`))
  (bind _assistmodules (`/Game/ProjectLight/Characters/Components/BPC_InventoryComponent.AssistModules` _bpc_inventorycomponent))
  (if (`KismetArrayLibrary.Array_IsNotEmpty` _assistmodules)
    (for _array_element _assistmodules
      (bind _asbp_module_assist (cast `/Game/ProjectLight/Modules/BP_Module_Assist` _array_element))
      (`/Game/ProjectLight/Modules/InterfacesAndFunctions/BPL_AssistModule.LinkAssistModule` _asbp_module_assist (`/Game/ProjectLight/Characters/Components/BPC_InventoryComponent.GetAllModules` _bpc_inventorycomponent false) self))))

(fn `SetParentActor`
  (params (Module :type "ChildActorComponent Object Reference"))
  (bind _asbp_module_base (cast `/Game/ProjectLight/Modules/BP_Module_Base` (`ChildActorComponent.ChildActor` Module)))
  (set `/Game/ProjectLight/Modules/BP_Module_Base.ParentActor` self _asbp_module_base))

(fn `SpawnModuleActor`
  (params (ModuleInfo :type "/Game/ProjectLight/Modules/Struct/FModuleBaseInfo Structure"))
  (returns (SpwanedModule :type "/Game/ProjectLight/Modules/BP_Module_Base Object Reference"))
  (locals (ModuleSpawned :type "/Game/ProjectLight/Modules/BP_Module_Base Object Reference"))
  (bind (_moduleclass _modulename _moduletype) (break `/Game/ProjectLight/Modules/Struct/FModuleBaseInfo` ModuleInfo))
  (bind _returnvalue (`|SpawnActorFromClass` _moduleclass (`KismetMathLibrary.MakeTransform` (0.0 0.0 0.0) (struct) (select `bool` (`|EnumEquality` _moduletype "NewEnumerator0") :`false` (0.1 0.1 0.1) :`true` (1.0 1.0 1.0) :!type "Vector Structure")) "Undefined" "MultiplyWithRoot" null _modulename _moduletype null))
  (set `local.ModuleSpawned` _returnvalue)
  (bind _moduletype_2 (`/Game/ProjectLight/Modules/BP_Module_Base.ModuleType` _returnvalue))
  (`self.K2_AttachToComponent` _returnvalue (`self.Mesh`) (`BlueprintMapLibrary.Map_Find` (`self.ModuleSocketName`) _moduletype_2) "SnapToTarget" "SnapToTarget" "KeepWorld" true)
  (`/Game/ProjectLight/Modules/BP_Module_Base.RegisterModule` _returnvalue self)
  (if (or (`|EnumEquality` _moduletype_2 "NewEnumerator3") (`|EnumEquality` _moduletype_2 "NewEnumerator0"))
    (`/Game/ProjectLight/Modules/BP_Module_Base.CloseModule` _returnvalue)
    (else
      (`/Game/ProjectLight/Modules/BP_Module_Base.OpenModule` _returnvalue)))
  (return (`local.ModuleSpawned`)))

(fn `UpdateAttribute`
  (`self.ChangeMaxHealth` (`self.GetAttributeByTag` (struct :`TagName` "Unit.Base.MaxHealth")))
  (set `CharacterMovementComponent.MaxWalkSpeed` (`self.GetAttributeByTag` (struct :`TagName` "Player.Base.MoveSpeed")) (`self.CharacterMovement`))
  (`self.UpdatePickRange` (`self.GetAttributeByTag` (struct :`TagName` "Player.Base.PickRange"))))

(fn `UpdatePickRange`
  (params (NewPickRange :type "Float (double-precision)"))
  (bind _output_get (set `self.PickRange` NewPickRange))
  (`SphereComponent.SetSphereRadius` (`self.PickRangeSphere`) _output_get true))

(fn `UpdatePlayerBaseInfo`
  (params (NewName :type Name))
  (locals (BuildingToUnlock :type "Array of Name") (ModuleToReceive :type "Array of /Game/ProjectLight/Modules/Struct/FModuleBasicInfo Structure"))
  (bind _bpc_inventorycomponent (`self.BPC_InventoryComponent`))
  (bind ((`StorageLimit_25_8D3F70BF401ECA8173E05A8B1C496D2D` _storagelimit) (`AssistLimit_27_B2B10402456CCDF3E48E46BA658B7770` _assistlimit)) (break `/Game/ProjectLight/Characters/Hero/Struct/FCharacterInfo` (`self.CharacterBaseInfo`)))
  (bind _returnvalue (`|GetDataTableRow` "/Game/ProjectLight/Characters/Hero/Data/DT_PlayerBaseData.DT_PlayerBaseData" NewName)
    (:`then`
      (set `self.CharacterBaseInfo` _returnvalue)
      (bind ((`MaxHealth_2_ECA93A9D43604CD930735AA6685F69C0` _maxhealth) (`MoveSpeed_4_6AAAA5D74DD97F4ADEC2EA877A54DF8D` _movespeed) (`StorageLimit_25_8D3F70BF401ECA8173E05A8B1C496D2D` _storagelimit_2) (`AssistLimit_27_B2B10402456CCDF3E48E46BA658B7770` _assistlimit_2) (`GachaTime_29_2B458DA544B33B86C938A588B550CAE0` _gachatime) (`BuildingToUnlock_11_4AEDBBD940ADB18A499DFC8F1A1B1B53` _buildingtounlock) (`UpgradeModule_22_41F7308B4CEC19A88136A3BE088FB27C` _upgrademodule)) (break `/Game/ProjectLight/Characters/Hero/Struct/FCharacterInfo` _returnvalue))
      (`self.ChangeMaxHealth` _maxhealth true)
      (set `self.InitalMovementSpeed` _movespeed)
      (set `local.BuildingToUnlock` _buildingtounlock)
      (set `local.ModuleToReceive` _upgrademodule)
      (`self.UpdateAttribute`)
      (`|ExecutionSequence`
        (:`then_0`
          (`self.BPC_InventoryComponent`
            (:`then`
              (`|ExecutionSequence`
                (:`then_0`
                  (if (`KismetArrayLibrary.Array_IsNotEmpty` (`local.ModuleToReceive`))
                    (for _array_element (`local.ModuleToReceive`)
                      (`/Game/ProjectLight/Characters/Components/BPC_InventoryComponent.ChangeModuleStock` (`self.BPC_InventoryComponent`) _array_element 1))))
                (:`then_1`
                  (if (`KismetArrayLibrary.Array_IsNotEmpty` (`local.BuildingToUnlock`))
                    (`KismetArrayLibrary.Array_Append` (`/Game/ProjectLight/Characters/Components/BPC_InventoryComponent.BuildingsCanBuild` (`self.BPC_InventoryComponent`)) (`local.BuildingToUnlock`))))
                (:`then_2`
                  (set `/Game/ProjectLight/Characters/Components/BPC_InventoryComponent.StorageLimit` _storagelimit _bpc_inventorycomponent)
                  (set `/Game/ProjectLight/Characters/Components/BPC_InventoryComponent.AssistLimit` _assistlimit _bpc_inventorycomponent))))
            (:`else`)))
        (:`then_1`
          (bind _bpc_upgradecomponent (`self.BPC_UpgradeComponent`)
            (:`then`
              (set `/Game/ProjectLight/Characters/Components/BPC_UpgradeComponent.MaxGachaNum` (+ (`.GachaTime_29_2B458DA544B33B86C938A588B550CAE0` (break `/Game/ProjectLight/Characters/Hero/Struct/FCharacterInfo` (`self.CharacterBaseInfo`))) 1) _bpc_upgradecomponent))
            (:`else`)))
        (:`then_2`
          (bind _bpc_upgradecomponent_2 (`self.BPC_UpgradeComponent`)
            (:`then`
              (`/Game/ProjectLight/Characters/Components/BPC_UpgradeComponent.OnUpgradeSuccess` _bpc_upgradecomponent_2))
            (:`else`)))))))

(fn `UserConstructionScript`
  (`parent.UserConstructionScript`))
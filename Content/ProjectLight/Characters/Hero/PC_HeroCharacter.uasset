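; Player controller for the hero character, adding the battle input mapping and driving movement, camera and combat input.
; Movement follows control rotation; view rotates while a trigger is held, and a quick double tap resets it to a downward angle.
; Focus and melee inputs open inventory battle or melee modules; success makes the pawn face the cursor via a trace, changes its speed rate and sets the hero's focus state.
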(event `self.ReceiveBeginPlay`
  (`self.SetControlRotation` (`KismetMathLibrary.MakeRotator` 0.0 -45.0)))

(event `self.ReceiveTick`
  (params (DeltaSeconds :type "Float (single-precision)"))
  (bind (_rotation_roll _rotation_pitch _rotation_yaw) (`KismetMathLibrary.BreakRotator` (`self.GetRotationCharacterToCursor`)))
  (bind _returnvalue (`self.K2_GetPawn`))
  (bind (_returnvalue_roll _returnvalue_pitch) (`KismetMathLibrary.BreakRotator` (`self.K2_GetActorRotation` _returnvalue)))
  (if (`self.FocusOnMouse`)
    (`self.K2_SetActorRotation` _returnvalue (`KismetMathLibrary.MakeRotator` _returnvalue_roll _returnvalue_pitch _rotation_yaw) false)))

(event `self.ReceivePossess`
  (params (PossessedPawn :type "Pawn Object Reference"))
  (`EnhancedInputSubsystemInterface.AddMappingContext` (subsystem `EnhancedInputLocalPlayerSubsystem`) "/Game/ProjectLight/Characters/Hero/Input/IMC_BattleControll.IMC_BattleControll" 0 (struct))
  (set `self.bShowMouseCursor` true)
  (bind _asbp_character_hero (cast `/Game/ProjectLight/Characters/Hero/BP_Character_Hero` PossessedPawn))
  (set `self.HeroCharacter` _asbp_character_hero))

(event `EnhancedInput|/Game/ProjectLight/Characters/Hero/Input/IA_Move`
  (params (ActionValue :type "Vector2D Structure") (ElapsedSeconds :type "Float (double-precision)") (TriggeredSeconds :type "Float (double-precision)") (InputAction :type "InputAction Object Reference" :default "/Game/ProjectLight/Characters/Hero/Input/IA_Move.IA_Move"))
  (bind (_x _y) (`KismetMathLibrary.BreakVector2D` ActionValue))
  (bind _returnvalue (`self.GetControlRotation`))
  (:`Triggered`
    (`KismetSystemLibrary.PrintString` (`KismetStringLibrary.Conv_Vector2dToString` ActionValue) true true (struct :`G` 0.66 :`B` 1.0 :`A` 1.0) 0.0)
    (`Pawn.AddMovementInput` (`self.K2_GetPawn`) (+ (* _y (`KismetMathLibrary.GetForwardVector` _returnvalue)) (* _x (`KismetMathLibrary.GetRightVector` _returnvalue))) 1.0 false)))

(event `EnhancedInput|/Game/ProjectLight/Characters/Hero/Input/IA_ViewControll`
  (params (ActionValue :type "Vector2D Structure") (ElapsedSeconds :type "Float (double-precision)") (TriggeredSeconds :type "Float (double-precision)") (InputAction :type "InputAction Object Reference" :default "/Game/ProjectLight/Characters/Hero/Input/IA_ViewControll.IA_ViewControll"))
  (bind _returnvalue (`self.K2_GetPawn`))
  (bind (_x _y) (`KismetMathLibrary.BreakVector2D` ActionValue))
  (:`Triggered`
    (if (`self.ViewControllIsOn`)
      (`Pawn.AddControllerYawInput` _returnvalue _y)
      (`Pawn.AddControllerPitchInput` _returnvalue _x))))

(event `EnhancedInput|/Game/ProjectLight/Characters/Hero/Input/IA_ViewControllTrigger`
  (params (ActionValue :type Boolean) (ElapsedSeconds :type "Float (double-precision)") (TriggeredSeconds :type "Float (double-precision)") (InputAction :type "InputAction Object Reference" :default "/Game/ProjectLight/Characters/Hero/Input/IA_ViewControllTrigger.IA_ViewControllTrigger"))
  (:`Triggered`
    (set `self.ViewControllIsOn` true))
  (:`Completed`
    (set `self.ViewControllIsOn` false)
    (if (`self.CanResetView`)
      (`self.SetControlRotation` (`KismetMathLibrary.MakeRotator` 0.0 -45.0))
      (set `self.CanResetView` false)
      (else
        (set `self.CanResetView` true)
        (bind _returnvalue (`KismetSystemLibrary.K2_SetTimerDelegate` (delegate `TimeOut`) 0.2))
        (set `self.ViewControllTriggerTimer` _returnvalue)))))

(event `TimeOut`
  (set `self.CanResetView` false)
  (`KismetSystemLibrary.K2_ClearAndInvalidateTimerHandle` (`self.ViewControllTriggerTimer`)))

(event `EnhancedInput|/Game/ProjectLight/Characters/Hero/Input/IA_FocusLookTrigger`
  (params (ActionValue :type Boolean) (ElapsedSeconds :type "Float (double-precision)") (TriggeredSeconds :type "Float (double-precision)") (InputAction :type "InputAction Object Reference" :default "/Game/ProjectLight/Characters/Hero/Input/IA_FocusLookTrigger.IA_FocusLookTrigger"))
  (bind _herocharacter (`self.HeroCharacter`))
  (:`Started`
    (bind _inventorycomponent (`/Game/ProjectLight/FunctionLibrary/BML_Common.GetInventoryComponent` _herocharacter)
      (:`IsValid`
        (bind _battlemodules (`/Game/ProjectLight/Characters/Components/BPC_InventoryComponent.BattleModules` _inventorycomponent)
          (:`then`
            (bind _opensuccess (`/Game/ProjectLight/Modules/BP_Module_Base.OpenModule` _battlemodules))
            (if _opensuccess
              (`/Engine/EditorBlueprintResources/StandardMacros.DoOnce` false :!label _label
                (:`Completed`
                  (add `/Game/ProjectLight/Modules/BP_Module_Base.OnModuleClose` _battlemodules (delegate `StopFocusOnMouse`))
                  (`self.FocusToMouse` true)))))
          (:`else`)))))
  (:`Completed`
    (`self.StopFocusOnMouse`)
    (bind _inventorycomponent_2 (`/Game/ProjectLight/FunctionLibrary/BML_Common.GetInventoryComponent` _herocharacter)
      (:`IsValid`
        (bind _battlemodules_2 (`/Game/ProjectLight/Characters/Components/BPC_InventoryComponent.BattleModules` _inventorycomponent_2)
          (:`then`
            (`/Game/ProjectLight/Modules/BP_Module_Base.CloseModule` _battlemodules_2)
            (goto _label :!via `Reset`))
          (:`else`))))))

(event `StopFocusOnMouse`
  (`self.FocusToMouse` false)
  (bind _inventorycomponent (`/Game/ProjectLight/FunctionLibrary/BML_Common.GetInventoryComponent` (`self.HeroCharacter`))
    (:`IsValid`
      (bind _battlemodules (`/Game/ProjectLight/Characters/Components/BPC_InventoryComponent.BattleModules` _inventorycomponent)
        (:`then`
          (clear `/Game/ProjectLight/Modules/BP_Module_Base.OnModuleClose` _battlemodules))
        (:`else`)))))

(event `EnhancedInput|/Game/ProjectLight/Characters/Hero/Input/IA_MeleeAttack`
  (params (ActionValue :type Boolean) (ElapsedSeconds :type "Float (double-precision)") (TriggeredSeconds :type "Float (double-precision)") (InputAction :type "InputAction Object Reference" :default "/Game/ProjectLight/Characters/Hero/Input/IA_MeleeAttack.IA_MeleeAttack"))
  (bind _herocharacter (`self.HeroCharacter`))
  (:`Triggered`
    (bind _inventorycomponent (`/Game/ProjectLight/FunctionLibrary/BML_Common.GetInventoryComponent` _herocharacter)
      (:`IsValid`
        (bind _meleemodule (`/Game/ProjectLight/Characters/Components/BPC_InventoryComponent.MeleeModule` _inventorycomponent)
          (:`then`
            (bind _opensuccess (`/Game/ProjectLight/Modules/BP_Module_Base.OpenModule` _meleemodule))
            (if _opensuccess
              (`/Engine/EditorBlueprintResources/StandardMacros.DoOnce` false :!label _label_2
                (:`Completed`
                  (`self.FocusToMouse` true)))))
          (:`else`)))))
  (:`Completed`
    (`self.FocusToMouse` false)
    (bind _inventorycomponent_2 (`/Game/ProjectLight/FunctionLibrary/BML_Common.GetInventoryComponent` _herocharacter)
      (:`IsValid`
        (bind _meleemodule_2 (`/Game/ProjectLight/Characters/Components/BPC_InventoryComponent.MeleeModule` _inventorycomponent_2)
          (:`then`
            (`/Game/ProjectLight/Modules/BP_Module_Base.CloseModule` _meleemodule_2)
            (goto _label_2 :!via `Reset`))
          (:`else`))))))

(fn `FocusToMouse`
  (params (FocusToMouse :type Boolean))
  (bind _output_get (set `self.FocusOnMouse` FocusToMouse))
  (message `/Game/ProjectLight/Characters/Interfaces/BPI_Character.SetMovementSpeedRate` (`self.K2_GetPawn`) (select `bool` _output_get :`false` 1.0 :`true` 0.5))
  (set `/Game/ProjectLight/Characters/Hero/BP_Character_Hero.FocusState` (select `bool` _output_get :`false` "NewEnumerator0" :`true` "NewEnumerator1" :!type "/Game/ProjectLight/Characters/Hero/Enum/EFocusState Enum") (`self.HeroCharacter`)))

(fn `GetRotationCharacterToCursor`
  (returns (Rotation :type "Rotator Structure"))
  (return (`KismetMathLibrary.MakeRotator` 0.0 0.0 (.yaw (`KismetMathLibrary.FindLookAtRotation` (`self.K2_GetActorLocation` (`self.K2_GetPawn`)) (`.Location` (`GameplayStatics.BreakHitResult` (`self.GetHitResultUnderCursorByChannel` "TraceTypeQuery1"))))))))

(fn `UserConstructionScript`)
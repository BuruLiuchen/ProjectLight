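; Inventory component that tracks its owner's registered modules and publishes the list of buildable buildings to the battle HUD.
; UpdateModuleList sorts modules by type: Melee, Produce and Battle assignments overwrite, while Storage and Assist collect unique entries.
; GetAllModules returns the non-assist modules, optionally appending the assist ones.
; BeginPlay polls on a short delay until the BattleHUD is valid, then pushes BuildingsCanBuild to it.
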(event `self.ReceiveBeginPlay`
  (bind _ashud_battle_sence (cast `/Game/ProjectLight/Blueprints/HUD_BattleSence` (`PlayerController.GetHUD` (`GameplayStatics.GetPlayerController` 0)) :!label _label))
  (`/Game/ProjectLight/Blueprints/HUD_BattleSence.BattleHUD` _ashud_battle_sence
    (:`then`
      (`self.UpdateDisplayOfBuildings`))
    (:`else`
      (`KismetSystemLibrary.Delay` 0.2)
      (goto _label))))

(fn `GetAllModules`
  (params (WithAssistModules :type Boolean))
  (returns (ModulesReturn :type "Array of /Game/ProjectLight/Modules/BP_Module_Base Object Reference"))
  (locals (Modules :type "Array of /Game/ProjectLight/Modules/BP_Module_Base Object Reference"))
  (`KismetArrayLibrary.Array_Append` (`local.Modules`) (`self.ModulesWithoutAssist`))
  (if WithAssistModules
    (`KismetArrayLibrary.Array_Append` (`local.Modules`) (`self.AssistModules`)))
  (return (`local.Modules`)))

(fn `UpdateDisplayOfBuildings`
  (bind _ashud_battle_sence (cast `/Game/ProjectLight/Blueprints/HUD_BattleSence` (`PlayerController.GetHUD` (`GameplayStatics.GetPlayerController` 0))))
  (bind _battlehud (`/Game/ProjectLight/Blueprints/HUD_BattleSence.BattleHUD` _ashud_battle_sence)
    (:`then`
      (`/Game/ProjectLight/UMG/UMG_HUD_Battle.UpdateBuildingList` _battlehud (`self.BuildingsCanBuild`)))
    (:`else`)))

(fn `UpdateModuleList`
  (params (ModuleToRegister :type "/Game/ProjectLight/Modules/BP_Module_Base Object Reference"))
  (bind (_basicinfo_size _basicinfo_rarity _basicinfo_moduletype) (break `/Game/ProjectLight/Modules/Struct/FModuleInfo_Base` (`/Game/ProjectLight/Modules/BP_Module_Base.BasicInfo` ModuleToRegister)))
  (bind _moduletoregister (`local.ModuleToRegister`))
  (switch `/Game/ProjectLight/Modules/EModuleType` _basicinfo_moduletype
    (:`NewEnumerator0`
      (set `self.MeleeModule` _moduletoregister))
    (:`NewEnumerator1`
      (set `self.ProduceModule` _moduletoregister))
    (:`NewEnumerator2`
      (`KismetArrayLibrary.Array_AddUnique` (`self.StorageModules`) _moduletoregister))
    (:`NewEnumerator3`
      (set `self.BattleModules` _moduletoregister))
    (:`NewEnumerator5`
      (`KismetArrayLibrary.Array_AddUnique` (`self.AssistModules`) _moduletoregister))))
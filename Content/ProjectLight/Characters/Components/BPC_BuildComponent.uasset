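; Building placement component that runs a three-stage state machine: choose a building, decide its location, then adjust its rotation.
; A preview actor follows or turns toward the cursor, with its cost read from DT_Buildings and shown on the battle HUD.
; Overlaps and resource checks drive a PreviewError material parameter collection value.
; Final confirm requires no overlaps and successful resource consumption; cancel steps back a stage.
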(fn `BuildActionCancel`
  (switch `/Game/ProjectLight/Characters/Hero/Enum/EBuildState` (`self.BuildState`)
    (:`NewEnumerator1`
      (set `self.BuildState` "NewEnumerator0")
      (bind _spawnedbuilding (`self.SpawnedBuilding`)
        (:`then`
          (`Actor.K2_DestroyActor` _spawnedbuilding)
          (`KismetArrayLibrary.Array_Clear` (`self.OverlapedActors`)))
        (:`else`)))
    (:`NewEnumerator2`
      (set `self.BuildState` "NewEnumerator1"))))

(fn `BuildActionConfirm`
  (switch `/Game/ProjectLight/Characters/Hero/Enum/EBuildState` (`self.BuildState`)
    (:`NewEnumerator0`
      (set `self.BuildState` "NewEnumerator1")
      (`KismetArrayLibrary.Array_Clear` (`self.OverlapedActors`)))
    (:`NewEnumerator1`
      (set `self.BuildState` "NewEnumerator2"))
    (:`NewEnumerator2`
      (if (`KismetArrayLibrary.Array_IsEmpty` (`self.OverlapedActors`))
        (bind _success (`self.TryToConsumeResource`))
        (if _success
          (set `self.BuildState` "NewEnumerator0")
          (bind _spawnedbuilding (`self.SpawnedBuilding`)
            (:`then`
              (`/Game/ProjectLight/Buildings/BP_Building_Base.BuildConfirm` _spawnedbuilding)
              (set `self.SpawnedBuilding` null))
            (:`else`)))))))

(fn `CursorLocationInput`
  (params (CursorLocation :type "Vector Structure"))
  (bind _spawnedbuilding (`self.SpawnedBuilding`))
  (bind (_returnvalue_roll _returnvalue_pitch _returnvalue_yaw) (`KismetMathLibrary.BreakRotator` (`KismetMathLibrary.FindLookAtRotation` (`self.BuildingLocation`) CursorLocation)))
  (bind (_returnvalue_roll_2 _returnvalue_pitch_2) (`KismetMathLibrary.BreakRotator` (`Actor.K2_GetActorRotation` _spawnedbuilding)))
  (`self.SpawnedBuilding`
    (:`then`
      (switch `/Game/ProjectLight/Characters/Hero/Enum/EBuildState` (`self.BuildState`)
        (:`NewEnumerator1`
          (bind _output_get (set `self.BuildingLocation` CursorLocation))
          (`Actor.K2_SetActorLocation` _spawnedbuilding (`KismetMathLibrary.MakeVector` (.x _output_get) (.y _output_get) (+ (.z _output_get) (`CapsuleComponent.GetScaledCapsuleHalfHeight` (`/Game/ProjectLight/Buildings/BP_Building_Base.Capsule` _spawnedbuilding)))) false false))
        (:`NewEnumerator2`
          (`Actor.K2_SetActorRotation` _spawnedbuilding (`KismetMathLibrary.MakeRotator` _returnvalue_roll_2 _returnvalue_pitch_2 _returnvalue_yaw) false))))
    (:`else`)))

(fn `ExitBuildMode`
  (set `self.BuildState` "NewEnumerator0")
  (bind _spawnedbuilding (`self.SpawnedBuilding`)
    (:`then`
      (`Actor.K2_DestroyActor` _spawnedbuilding)
      (`KismetArrayLibrary.Array_Clear` (`self.OverlapedActors`)))
    (:`else`)))

(fn `GetConsumeValue`
  (params (Type :type "/Game/ProjectLight/Components/Enum/EEnergyType Enum" :default "NewEnumerator0"))
  (returns (ValumeToConsume :type "Float (double-precision)"))
  (for _array_element (`self.Build Resource`)
    (bind (_type _volume) (break `/Game/ProjectLight/Components/Struct/FEnergyInfo` _array_element))
    (if (`|EnumEquality` Type _type)
      (return _volume)))
  (return 0.0))

(fn `SetOverlapedActors`
  (params (NewOverlapedActor :type "Actor Object Reference") (Remove :type Boolean))
  (bind _overlapedactors (`self.OverlapedActors`))
  (`self.SpawnedBuilding`
    (:`then`
      (if Remove
        (`KismetArrayLibrary.Array_RemoveItem` _overlapedactors NewOverlapedActor)
        (else
          (`KismetArrayLibrary.Array_AddUnique` _overlapedactors NewOverlapedActor)))
      (`self.UpdatePreviewState`))
    (:`else`)))

(fn `SpawnBuildingActor`
  (params (BuildingName :type Name))
  (bind _spawnedbuilding (`self.SpawnedBuilding`)
    (:`then`
      (`Actor.K2_DestroyActor` _spawnedbuilding))
    (:`else`
      _))
  (`self.UpdateResourceNeed` BuildingName)
  (bind _returnvalue (`|SpawnActorFromClass` "/Game/ProjectLight/Buildings/BP_Building_Base.BP_Building_Base_C" (`KismetMathLibrary.MakeTransform` (0.0 0.0 0.0)) "Undefined" "MultiplyWithRoot" null BuildingName null))
  (bind _output_get (set `self.SpawnedBuilding` _returnvalue))
  (`PrimitiveComponent.SetCollisionProfileName` (`/Game/ProjectLight/Buildings/BP_Building_Base.Capsule` _output_get) "PreviewBuilding" true)
  (bind _resourcecomponent (`/Game/ProjectLight/Blueprints/FunctionLibrary/BML_Common.GetResourceComponent` (`GameplayStatics.GetPlayerCharacter` 0))
    (:`IsValid`
      (add `/Game/ProjectLight/Characters/Components/BPC_ResourceComponent.OnCurrentStorageChange` _resourcecomponent (`|CreateDelegate` :!event `UpdatePreviewState`))
      (`self.UpdatePreviewState`))))

(fn `TryToConsumeResource`
  (returns (Success :type Boolean))
  (bind _resourcecomponent (`/Game/ProjectLight/Blueprints/FunctionLibrary/BML_Common.GetResourceComponent` (`self.GetOwner`))
    (:`IsValid`
      (for _array_element (`self.Build Resource`)
        (bind (_type _volume) (break `/Game/ProjectLight/Components/Struct/FEnergyInfo` _array_element))
        (bind _consumesucess (`/Game/ProjectLight/Characters/Components/BPC_ResourceComponent.ConsumeStorageValue` _resourcecomponent _type _volume))
        (if (not _consumesucess)
          (return false)))
      (return true))
    (:`IsNotValid`
      (return false))))

(fn `UpdatePreviewState`
  (bind _paracollection (`self.ParaCollection`))
  (`self.SpawnedBuilding`
    (:`then`
      (bind _resourcecomponent (`/Game/ProjectLight/Blueprints/FunctionLibrary/BML_Common.GetResourceComponent` (`self.GetOwner`))
        (:`IsValid`
          (bind _isenough (`/Game/ProjectLight/Characters/Components/BPC_ResourceComponent.CheckResourceIsEnough` _resourcecomponent (`self.Build Resource`)))
          (if _isenough
            (if (`KismetArrayLibrary.Array_IsEmpty` (`self.OverlapedActors`))
              (`KismetMaterialLibrary.SetScalarParameterValue` _paracollection "PreviewError" 0.0)
              (else
                (`KismetMaterialLibrary.SetScalarParameterValue` _paracollection "PreviewError" 1.0)))
            (else
              (`KismetMaterialLibrary.SetScalarParameterValue` (`self.ParaCollection`) "PreviewError" 1.0))))))
    (:`else`)))

(fn `UpdateResourceNeed`
  (params (RowName :type Name))
  (bind _returnvalue (`|GetDataTableRow` "/Game/ProjectLight/Buildings/Data/DT_Buildings.DT_Buildings" RowName)
    (:`then`
      (bind (_displayname _buildingtype _size _maxhealthpoint _assistmodulelimit _attachedmodules _connectrange _buildtime _buildresource) (break `/Game/ProjectLight/Buildings/Struct/FBuildingInfo` _returnvalue))
      (set `self.Build Resource` _buildresource)
      (bind _ashud_battle_sence (cast `/Game/ProjectLight/Blueprints/HUD_BattleSence` (`PlayerController.GetHUD` (`GameplayStatics.GetPlayerController` 0))))
      (bind _battlehud (`/Game/ProjectLight/Blueprints/HUD_BattleSence.BattleHUD` _ashud_battle_sence)
        (:`then`
          (`/Game/ProjectLight/UMG/UMG_HUD_Battle.UpdateConsumeText` _battlehud _buildresource))
        (:`else`)))))
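; Resource component that tracks and spends Electrical, Biomass and Tech resources.
; Electrical and Biomass storage modules register by energy type; queries sum their storage and capacity, optionally filtered by owner unit type, while Tech is one uncapped point counter.
; Spending checks the total, then drains modules in list order.
; Cost-list helpers check every entry, but ConsumeResources returns after consuming the first.
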(fn `ChangeTechPoint`
  (params (Delta :type "Float (double-precision)"))
  (bind _returnvalue (+ Delta (`self.TechPoint`)))
  (set `self.TechPoint` (`KismetMathLibrary.FClamp` _returnvalue 0.0 _returnvalue)))

(fn `CheckResourceIsEnough`
  (params (Resources :type "Array of /Game/ProjectLight/Components/Struct/FEnergyInfo Structure"))
  (returns (IsEnough :type Boolean))
  (for _array_element Resources
    (bind (_type _volume) (break `/Game/ProjectLight/Components/Struct/FEnergyInfo` _array_element))
    (if (not (>= (`self.GetStorageValue` _type) _volume))
      (return false)))
  (return true))

(fn `ConsumeResources`
  (params (Resources :type "Array of /Game/ProjectLight/Components/Struct/FEnergyInfo Structure"))
  (returns (ConsumeSucess :type Boolean))
  (for _array_element Resources
    (bind (_type _volume) (break `/Game/ProjectLight/Components/Struct/FEnergyInfo` _array_element))
    (bind _consumesucess (`self.ConsumeStorageValue` _type _volume))
    (return _consumesucess)))

(fn `ConsumeStorageValue`
  (params (EnergyType :type "/Game/ProjectLight/Components/Enum/EEnergyType Enum" :default "NewEnumerator0") (ValueToConsume :type "Float (double-precision)"))
  (returns (ConsumeSucess :type Boolean))
  (locals (TotalValue :type "Float (double-precision)") (ConsumeValue :type "Float (double-precision)"))
  (set `local.TotalValue` ValueToConsume)
  (if (>= (`self.GetStorageValue` EnergyType) ValueToConsume)
    (switch `/Game/ProjectLight/Components/Enum/EEnergyType` EnergyType
      (:`NewEnumerator1`
        (for _array_element (`self.StorageModules_Electrical`)
          (bind _output_get (set `local.ConsumeValue` (`KismetMathLibrary.FMin` (`local.TotalValue`) (`/Game/ProjectLight/Modules/BP_Module_Storage.CurrentStorage` _array_element))))
          (`/Game/ProjectLight/Modules/BP_Module_Storage.ChangeStorage` _array_element (* _output_get -1.0))
          (bind _output_get_2 (set `local.TotalValue` (- (`local.TotalValue`) (`local.ConsumeValue`))))
          (if (<= _output_get_2 0.0)
            (break)))
        (return true))
      (:`NewEnumerator2`
        (for _array_element_2 (`self.StorageModules_Biomass`)
          (bind _output_get_3 (set `local.ConsumeValue` (`KismetMathLibrary.FMin` (`local.TotalValue`) (`/Game/ProjectLight/Modules/BP_Module_Storage.CurrentStorage` _array_element_2))))
          (`/Game/ProjectLight/Modules/BP_Module_Storage.ChangeStorage` _array_element_2 (* _output_get_3 -1.0))
          (bind _output_get_4 (set `local.TotalValue` (- (`local.TotalValue`) (`local.ConsumeValue`))))
          (if (<= _output_get_4 0.0)
            (break)))
        (return true))
      (:`NewEnumerator3`
        (`self.ChangeTechPoint` (* (`local.TotalValue`) -1.0))))
    (else
      (return false))))

(fn `GetStorageValue`
  (params (EnergyType :type "/Game/ProjectLight/Components/Enum/EEnergyType Enum" :default "NewEnumerator0") (PlayerOnly :type Boolean))
  (returns (CurrentValue :type "Float (double-precision)") (ValueCap :type "Float (double-precision)"))
  (locals (CurrentValue_Local :type "Float (double-precision)") (ValueCap_Local :type "Float (double-precision)"))
  (bind _valuecap_local (`local.ValueCap_Local`))
  (bind _currentvalue_local (`local.CurrentValue_Local`))
  (switch `/Game/ProjectLight/Components/Enum/EEnergyType` EnergyType
    (:`NewEnumerator1`
      (for _array_element (`self.StorageModules_Electrical`)
        (`/Engine/EditorBlueprintResources/StandardMacros.IsValid` _array_element
          (:`Is Valid`
            (if (`local.PlayerOnly`)
              (bind _unittype (message `/Game/ProjectLight/Blueprints/Interfaces/BPI_Common.GetUnitType` (`/Game/ProjectLight/Modules/BP_Module_Base.ParentActor` _array_element)))
              (if (`|EnumEquality` _unittype "NewEnumerator0")
                (set `local.CurrentValue_Local` (+ (`local.CurrentValue_Local`) (`/Game/ProjectLight/Modules/BP_Module_Storage.CurrentStorage` _array_element)) :!label _label)
                (set `local.ValueCap_Local` (+ (`local.ValueCap_Local`) (`/Game/ProjectLight/Modules/BP_Module_Storage.Storage Cap` _array_element))))
              (else
                (goto _label))))))
      (return _currentvalue_local _valuecap_local))
    (:`NewEnumerator2`
      (for _array_element_2 (`self.StorageModules_Biomass`)
        (`/Engine/EditorBlueprintResources/StandardMacros.IsValid` _array_element_2
          (:`Is Valid`
            (if (`local.PlayerOnly`)
              (bind _unittype_2 (message `/Game/ProjectLight/Blueprints/Interfaces/BPI_Common.GetUnitType` (`/Game/ProjectLight/Modules/BP_Module_Base.ParentActor` _array_element_2)))
              (if (`|EnumEquality` _unittype_2 "NewEnumerator0")
                (set `local.CurrentValue_Local` (+ (`local.CurrentValue_Local`) (`/Game/ProjectLight/Modules/BP_Module_Storage.CurrentStorage` _array_element_2)) :!label _label_2)
                (set `local.ValueCap_Local` (+ (`local.ValueCap_Local`) (`/Game/ProjectLight/Modules/BP_Module_Storage.Storage Cap` _array_element_2))))
              (else
                (goto _label_2))))))
      (return _currentvalue_local _valuecap_local))
    (:`NewEnumerator3`
      (return (`self.TechPoint`) -1.0))))

(fn `RegisterStorageModule`
  (params (StorageModule :type "/Game/ProjectLight/Modules/BP_Module_Storage Object Reference"))
  (`/Engine/EditorBlueprintResources/StandardMacros.IsValid` StorageModule
    (:`Is Valid`
      (switch `/Game/ProjectLight/Components/Enum/EEnergyType` (`/Game/ProjectLight/Modules/BP_Module_Storage.Storage Energy` StorageModule)
        (:`NewEnumerator1`
          (`KismetArrayLibrary.Array_AddUnique` (`self.StorageModules_Electrical`) StorageModule))
        (:`NewEnumerator2`
          (`KismetArrayLibrary.Array_AddUnique` (`self.StorageModules_Biomass`) StorageModule))))))

(fn `TechPonintIsEnough`
  (params (ValueNeed :type "Float (double-precision)"))
  (returns (IsEnough :type Boolean))
  (return (>= (`self.TechPoint`) ValueNeed)))

(fn `UnregisterStorageModule`
  (params (StorageModule :type "/Game/ProjectLight/Modules/BP_Module_Storage Object Reference"))
  (`/Engine/EditorBlueprintResources/StandardMacros.IsValid` StorageModule
    (:`Is Valid`
      (switch `/Game/ProjectLight/Components/Enum/EEnergyType` (`/Game/ProjectLight/Modules/BP_Module_Storage.Storage Energy` StorageModule)
        (:`NewEnumerator1`
          (`KismetArrayLibrary.Array_RemoveItem` (`self.StorageModules_Electrical`) StorageModule))
        (:`NewEnumerator2`
          (`KismetArrayLibrary.Array_RemoveItem` (`self.StorageModules_Biomass`) StorageModule))))))
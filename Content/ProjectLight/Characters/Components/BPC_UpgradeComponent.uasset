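; Actor component that handles hero and building upgrades, plus an adjust mode showing building info for actors in range.
; Adjust mode binds to the owner's port-manager SenseRange overlaps, toggling its collision profile to refresh them, and closes messages on exit.
; TryToUpgrade spends resources, then builds a "Name_Lv_N" next-level name.
; That name upgrades the hero or MainTower directly; other buildings only get swapped in the inventory's buildable list.
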(event `EnterAdjustMode`
  (bind _portmanagecomp (`/Game/ProjectLight/Blueprints/FunctionLibrary/BML_Common.GetPortManageComp` (`self.GetOwner`))
    (:`IsValid`
      (bind _senserange (`/Game/ProjectLight/Components/BPC_PortManageComponent.SenseRange` _portmanagecomp)
        (:`then`
          (add `PrimitiveComponent.OnComponentBeginOverlap` _senserange (delegate `OnBeginOverlap`))
          (add `PrimitiveComponent.OnComponentEndOverlap` _senserange (delegate `OnEndOverlap`))
          (`self.RestartConnectRange`))
        (:`else`)))))

(event `OnBeginOverlap`
  (params (OverlappedComponent :type "PrimitiveComponent Object Reference") (OtherActor :type "Actor Object Reference") (OtherComp :type "PrimitiveComponent Object Reference") (OtherBodyIndex :type Integer) (bFromSweep :type Boolean) (SweepResult :type "HitResult Structure (by ref)"))
  (message `/Game/ProjectLight/Blueprints/Interfaces/BPI_Common.OpenBuildingInfo` OtherActor)
  (`KismetArrayLibrary.Array_AddUnique` (`self.OverlapedActors`) OtherActor))

(event `OnEndOverlap`
  (params (OverlappedComponent :type "PrimitiveComponent Object Reference") (OtherActor :type "Actor Object Reference") (OtherComp :type "PrimitiveComponent Object Reference") (OtherBodyIndex :type Integer))
  (message `/Game/ProjectLight/Blueprints/Interfaces/BPI_Common.CloseBuildingInfo` OtherActor)
  (`KismetArrayLibrary.Array_RemoveItem` (`self.OverlapedActors`) OtherActor))

(event `ExitAdjustMode`
  (bind _portmanagecomp (`/Game/ProjectLight/Blueprints/FunctionLibrary/BML_Common.GetPortManageComp` (`self.GetOwner`))
    (:`IsValid`
      (bind _senserange (`/Game/ProjectLight/Components/BPC_PortManageComponent.SenseRange` _portmanagecomp)
        (:`then`
          (remove `PrimitiveComponent.OnComponentBeginOverlap` _senserange (delegate `OnBeginOverlap`))
          (remove `PrimitiveComponent.OnComponentEndOverlap` _senserange (delegate `OnEndOverlap`))
          (for _array_element (`self.OverlapedActors`)
            (message `/Game/ProjectLight/Blueprints/Interfaces/BPI_Common.CloseBuildingInfo` _array_element)))
        (:`else`)))))

(fn `RestartConnectRange`
  (bind _portmanagecomp (`/Game/ProjectLight/Blueprints/FunctionLibrary/BML_Common.GetPortManageComp` (`self.GetOwner`))
    (:`IsValid`
      (bind _senserange (`/Game/ProjectLight/Components/BPC_PortManageComponent.SenseRange` _portmanagecomp))
      (`PrimitiveComponent.SetCollisionProfileName` _senserange "NoCollision" true)
      (`PrimitiveComponent.SetCollisionProfileName` _senserange "EnergyConnect" true))))

(fn `TryToUpgrade`
  (params (UnitType :type "/Game/ProjectLight/Blueprints/Enums/EUnitType Enum" :default "NewEnumerator0") (UnitName :type String) (CurrentLevel :type Integer) (UpgradeResource :type "Array of /Game/ProjectLight/Components/Struct/FEnergyInfo Structure"))
  (returns (UpgradeSuccess :type Boolean))
  (bind _returnvalue (`self.GetOwner`))
  (bind _unitname (`local.UnitName`))
  (bind _currentlevel (`local.CurrentLevel`))
  (bind _returnvalue_2 (`KismetStringLibrary.Conv_StringToName` (`KismetStringLibrary.Concat_StrStr` _unitname "_Lv_" (`KismetStringLibrary.Conv_IntToString` (+ _currentlevel 1)))))
  (bind _resourcecomponent (`/Game/ProjectLight/Blueprints/FunctionLibrary/BML_Common.GetResourceComponent` (`self.GetOwner`))
    (:`IsValid`
      (bind _isenough (`/Game/ProjectLight/Characters/Components/BPC_ResourceComponent.CheckResourceIsEnough` _resourcecomponent UpgradeResource))
      (if _isenough
        (bind _consumesucess (`/Game/ProjectLight/Characters/Components/BPC_ResourceComponent.ConsumeResources` _resourcecomponent UpgradeResource))
        (if _consumesucess
          (switch `/Game/ProjectLight/Blueprints/Enums/EUnitType` (`local.UnitType`)
            (:`NewEnumerator0`
              (bind _asbp_character_hero (cast `/Game/ProjectLight/Characters/Hero/BP_Character_Hero` _returnvalue))
              (set `/Game/ProjectLight/Characters/BP_Character_Base.CharacterName` _returnvalue_2 _asbp_character_hero)
              (`/Game/ProjectLight/Characters/Hero/BP_Character_Hero.CharacterUpgrade` _asbp_character_hero)
              (return true))
            (:`NewEnumerator2`
              (if (`KismetStringLibrary.EqualEqual_StrStr` _unitname "MainTower")
                (bind _returnvalue_3 (`GameplayStatics.GetActorOfClass` "/Game/ProjectLight/Buildings/BP_Building_MainTower.BP_Building_MainTower_C"))
                (`/Game/ProjectLight/Buildings/BP_Building_Base.UpgradeBuilding` _returnvalue_3 _returnvalue_2)
                (return true)
                (else
                  (bind _inventorycomponent (`/Game/ProjectLight/Blueprints/FunctionLibrary/BML_Common.GetInventoryComponent` _returnvalue)
                    (:`IsValid`
                      (bind _buildingscanbuild (`/Game/ProjectLight/Characters/Components/BPC_InventoryComponent.BuildingsCanBuild` _inventorycomponent))
                      (`KismetArrayLibrary.Array_RemoveItem` _buildingscanbuild (`KismetStringLibrary.Conv_StringToName` (`KismetStringLibrary.Concat_StrStr` _unitname "_Lv_" (`KismetStringLibrary.Conv_IntToString` _currentlevel))))
                      (`KismetArrayLibrary.Array_AddUnique` _buildingscanbuild _returnvalue_2)
                      (return true)))))))
          (else
            _)))
      (return false))))
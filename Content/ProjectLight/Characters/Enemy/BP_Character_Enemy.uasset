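; Base melee enemy character that loads health, speed, attack range, mesh, animation and montage from DT_EnemyList by CharacterName.
; SearchRange overlaps write living targets of a specific unit and building type to the AI Blackboard's TargetActor.
; Attack loops the montage, while MeleeAttack toggles a per-tick box trace that damages the target once per swing or drops it if missed.
; On death it launches biomass pickups upward and expires shortly after.
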(event `self.ReceiveTick`
  (params (DeltaSeconds :type "Float (single-precision)"))
  (bind _returnvalue (`self.K2_GetActorLocation`))
  (`parent.ReceiveTick` DeltaSeconds)
  (if (`self.IsAttacking`)
    (bind _outhits (`KismetSystemLibrary.BoxTraceMulti` _returnvalue (+ _returnvalue (* (`self.GetActorForwardVector`) (`self.AttackRange`))) (0.0 40.0 20.0) (`self.K2_GetActorRotation`) "TraceTypeQuery4"))
    (`self.CheckHitResult` _outhits)))

(event `Attack`
  (params (AttackTarget :type "Actor Object Reference"))
  (bind _output_get (set `self.AttackTarget` AttackTarget))
  (add `self.OnDestroyed` _output_get (delegate `TargetLose`))
  (`self.AttackTarget` :!label _label
    (:`then`
      (`|PlayMontage` (`self.Mesh`) (`self.AttackMontage`)
        (:`OnCompleted`
          (`self.OnAttackEnd` false)
          (goto _label))
        (:`OnInterrupted`
          (`self.OnAttackEnd` true))))
    (:`else`
      (`self.TargetLose` null))))

(event `TargetLose` :!signature `self.OnDestroyed`
  (params (DestroyedActor :type "Actor Object Reference"))
  (`self.OnTargetLosed`)
  (set `self.AttackTarget` null))

(event `/Game/ProjectLight/Characters/Interfaces/BPI_Character.MeleeAttack`
  (params (StartAttack :type Boolean))
  (set `self.IsAttacking` StartAttack)
  (`KismetArrayLibrary.Array_Clear` (`self.HitActors`)))

(event `self.CharacterDie`
  (`parent.CharacterDie`)
  (`self.SpawnResource`)
  (`self.SetLifeSpan` 3.0))

(event `self.SearchRange.OnComponentBeginOverlap`
  (params (OverlappedComponent :type "PrimitiveComponent Object Reference") (OtherActor :type "Actor Object Reference") (OtherComp :type "PrimitiveComponent Object Reference") (OtherBodyIndex :type Integer) (bFromSweep :type Boolean) (SweepResult :type "HitResult Structure (by ref)"))
  (bind _returnvalue (`AIBlueprintHelperLibrary.GetAIController` self))
  (bind (_righttarget _overlapedtarget) (`self.CheckOverlapedTarget` OtherActor))
  (if _righttarget
    (`/Engine/EditorBlueprintResources/StandardMacros.IsValid` _returnvalue
      (:`Is Valid`
        (`BlackboardComponent.SetValueAsObject` (`AIBlueprintHelperLibrary.GetBlackboard` _returnvalue) "TargetActor" _overlapedtarget)))))

(event `self.ReceiveBeginPlay`
  (bind _returnvalue (`|GetDataTableRow` "/Game/ProjectLight/Characters/Enemy/DT_EnemyList.DT_EnemyList" (`self.CharacterName`))
    (:`then`
      (`self.InitEnemyInfo` _returnvalue)
      (`parent.ReceiveBeginPlay`))))

(fn `ApplyDamage`
  (params (HitResult :type "HitResult Structure (by ref)") (HitSomthing :type Boolean))
  (locals (HitActor :type "Actor Object Reference"))
  (bind (_bblockinghit _binitialoverlap _time _distance _location _impactpoint _normal _impactnormal _physmat _hitactor) (`GameplayStatics.BreakHitResult` HitResult))
  (bind _hitactor_2 (`local.HitActor`))
  (if HitSomthing
    (set `local.HitActor` _hitactor)
    (if (and (!= (`GameplayStatics.GetObjectClass` _hitactor) (`GameplayStatics.GetObjectClass` self)) (not (`KismetArrayLibrary.Array_Contains` (`self.HitActors`) _hitactor)))
      (`KismetArrayLibrary.Array_AddUnique` (`self.HitActors`) _hitactor_2)
      (`GameplayStatics.ApplyDamage` _hitactor_2 (`self.BaseDamage`)))))

(fn `CheckAttackRange`
  (params (Target :type "Actor Object Reference"))
  (returns (InRange :type Boolean))
  (return (<= (`self.GetDistanceTo` Target self) (`self.AttackRange`))))

(fn `CheckHitResult`
  (params (TargetArray :type "Array of HitResult Structure (by ref)"))
  (locals (HasHitTarget :type Boolean))
  (if (`KismetArrayLibrary.Array_IsNotEmpty` TargetArray)
    (for _array_element TargetArray
      (if (== (`.HitActor` (`GameplayStatics.BreakHitResult` _array_element)) (`self.AttackTarget`))
        (set `local.HasHitTarget` true)
        (`self.ApplyDamage` _array_element true)))
    (if (not (`local.HasHitTarget`))
      (`self.TargetLose` null))
    (else
      (`self.TargetLose` null))))

(fn `CheckOverlapedTarget`
  (params (OtherActor :type "Actor Object Reference"))
  (returns (RightTarget :type Boolean) (OverlapedTarget :type "Actor Object Reference"))
  (bind _otheractor (`local.OtherActor`))
  (bind _unittype (message `/Game/ProjectLight/Blueprints/Interfaces/BPI_Common.GetUnitType` OtherActor))
  (if (`|EnumEquality` _unittype "NewEnumerator2")
    (bind _buildingtype (message `/Game/ProjectLight/Blueprints/Interfaces/BPI_Common.GetBuildingType` (`local.OtherActor`)))
    (if (`|EnumEquality` _buildingtype "NewEnumerator2")
      (bind _isliving (message `/Game/ProjectLight/Blueprints/Interfaces/BPI_Common.GetIsLiving` _otheractor))
      (return _isliving _otheractor))))

(fn `GetUnitType`
  (returns (UnitType :type "/Game/ProjectLight/Blueprints/Enums/EUnitType Enum"))
  (return "NewEnumerator1"))

(fn `InitEnemyInfo`
  (params (FEnemyInfo :type "/Game/ProjectLight/Characters/Enemy/FEnemyInfo Structure (by ref)"))
  (bind (_maxhealth _movespeed _attackrange _attackmontage _displayname _displayicon _mesh _animblueprint) (break `/Game/ProjectLight/Characters/Enemy/FEnemyInfo` FEnemyInfo))
  (bind _mesh_2 (`self.Mesh`))
  (`self.ChangeMaxHealth` _maxhealth)
  (set `self.InitalMovementSpeed` _movespeed)
  (set `self.AttackRange` _attackrange)
  (set `self.AttackMontage` _attackmontage)
  (`SkeletalMeshComponent.SetSkeletalMeshAsset` _mesh_2 _mesh)
  (`SkeletalMeshComponent.SetAnimInstanceClass` _mesh_2 _animblueprint))

(fn `SpawnResource`
  (bind _biomassvaluesingle (`self.BiomassValueSingle`))
  (bind _returnvalue (`KismetMathLibrary.FFloor` (/ (`self.TotalBiomassValue`) _biomassvaluesingle)))
  (for _ (range (+ (`KismetMathLibrary.Clamp` _returnvalue 1 _returnvalue) 1))
    (bind _returnvalue_2 (`|SpawnActorFromClass` "/Game/ProjectLight/Blueprints/BP_Item_Base.BP_Item_Base_C" (`KismetMathLibrary.MakeTransform` (`self.K2_GetActorLocation`)) "AdjustIfPossibleButAlwaysSpawn" "MultiplyWithRoot" null (make `/Game/ProjectLight/Components/Struct/FEnergyInfo` "NewEnumerator2" _biomassvaluesingle) null))
    (`/Engine/EditorBlueprintResources/StandardMacros.IsValid` _returnvalue_2
      (:`Is Valid`
        (bind _capsule (`/Game/ProjectLight/Blueprints/BP_Item_Base.Capsule` _returnvalue_2)
          (:`then`
            (`PrimitiveComponent.AddImpulse` _capsule (* (`KismetMathLibrary.RandomUnitVectorInConeInDegrees` (0.0 0.0 1.0) 45.0) 500.0) "None" true))
          (:`else`))))))

(fn `UserConstructionScript`
  (`parent.UserConstructionScript`))
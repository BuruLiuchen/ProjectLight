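; BP_Resource_Base is a base pickup actor for an energy resource, defined by an EnergyInfo type and volume.
; On PickedUp, it loops through the storage modules in the hero's inventory component, looking for non-full modules of the same energy type.
; A match receives the volume through ChangeStorage and the pickup destroys itself, though the loop has no break after that.
; Without a match, the actor stays in the world.
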(event `PickedUp`
  (params (HeroCharacter :type "/Game/ProjectLight/Characters/Hero/BP_Character_Hero Object Reference"))
  (bind (_type _volume) (break `/Game/ProjectLight/Components/Struct/FEnergyInfo` (`self.EnergyInfo`)))
  (bind _bpc_inventorycomponent (`/Game/ProjectLight/Characters/Hero/BP_Character_Hero.BPC_InventoryComponent` HeroCharacter)
    (:`then`
      (for _array_element (`/Game/ProjectLight/Characters/Components/BPC_InventoryComponent.StorageModules` _bpc_inventorycomponent)
        (bind _asbp_module_storage (cast `/Game/ProjectLight/Modules/BP_Module_Storage` _array_element))
        (if (and (not (`/Game/ProjectLight/Modules/BP_Module_Storage.StorageIsFull` _asbp_module_storage)) (`|EnumEquality` (`/Game/ProjectLight/Modules/BP_Module_Storage.Storage Energy` _asbp_module_storage) _type))
          (`/Game/ProjectLight/Modules/BP_Module_Storage.ChangeStorage` _asbp_module_storage _volume)
          (`self.K2_DestroyActor`))))
    (:`else`)))

(fn `UserConstructionScript`)
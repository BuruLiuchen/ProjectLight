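; BPL_Port is a Blueprint function library for querying energy port components on an actor.
; GetPortsByTypeAndEnergy gathers either the BPC_EnergyPort_Input or BPC_EnergyPort_Output components, chosen by the requested port type.
; It returns the unique ports whose energy type matches the one requested.
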(fn `GetPortsByTypeAndEnergy`
  (params (Actor :type "Actor Object Reference") (PortType :type "/Game/ProjectLight/Components/Enum/EEnergyPortType Enum" :default "NewEnumerator0") (EnergyType :type "/Game/ProjectLight/Components/Enum/EEnergyType Enum" :default "NewEnumerator0"))
  (returns (PortsForReturn :type "Array of /Game/ProjectLight/Components/BPC_EnergyPort Object Reference"))
  (locals (OutputPorts :type "Array of /Game/ProjectLight/Components/BPC_EnergyPort Object Reference"))
  (for _array_element (select `/Game/ProjectLight/Components/Enum/EEnergyPortType` PortType :`NewEnumerator0` (`Actor.K2_GetComponentsByClass` Actor "/Game/ProjectLight/Components/BPC_EnergyPort_Input.BPC_EnergyPort_Input_C") :`NewEnumerator1` (`Actor.K2_GetComponentsByClass` Actor "/Game/ProjectLight/Components/BPC_EnergyPort_Output.BPC_EnergyPort_Output_C") :!type "Array of /Game/ProjectLight/Components/BPC_EnergyPort Object Reference")
    (if (`|EnumEquality` (`/Game/ProjectLight/Components/BPC_EnergyPort.EnergyType` _array_element) (`local.EnergyType`))
      (`KismetArrayLibrary.Array_AddUnique` (`local.OutputPorts`) _array_element)))
  (return (`local.OutputPorts`)))
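; BPL_Light is a Blueprint function library providing ConeLineTrace, a horizontal fan-shaped hit query in front of an actor.
; Two arcs, each with its own angle and distance, are centred on the actor's forward vector by yaw rotation.
; Evenly spaced line traces join matching inner and outer arc points, drawing one-frame debug lines.
; It returns the unique hit results and whether anything was hit.
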(fn `ConeLineTrace`
  (params (Actor :type "Actor Object Reference") (ActorsIgnore :type "Array of Actor Object Reference") (LineNum :type Integer :default 10) (InnerAngle :type "Float (double-precision)" :default 30.0) (InnerDistance :type "Float (double-precision)" :default 20.0) (OuterAngle :type "Float (double-precision)" :default 90.0) (OuterDistance :type "Float (double-precision)" :default 300.0))
  (returns (OutHits :type "Array of HitResult Structure") (HasHitSomething :type Boolean))
  (locals (InnerAngle_Local :type "Vector Structure") (OuterAngle_Local :type "Vector Structure") (ActorLocation :type "Vector Structure" :default (0.0 0.0 0.0)) (HitResults :type "Array of HitResult Structure"))
  (bind _hitresults (`local.HitResults`))
  (set `local.ActorLocation` (`Actor.K2_GetActorLocation` Actor))
  (set `local.InnerAngle_Local` (`KismetMathLibrary.GreaterGreater_VectorRotator` (`Actor.GetActorForwardVector` Actor) (`KismetMathLibrary.MakeRotator` 0.0 0.0 (* InnerAngle -0.5))))
  (set `local.OuterAngle_Local` (`KismetMathLibrary.GreaterGreater_VectorRotator` (`Actor.GetActorForwardVector` Actor) (`KismetMathLibrary.MakeRotator` 0.0 0.0 (* OuterAngle -0.5))))
  (for _index (range (+ (`local.LineNum`) 1))
    (bind (_outhit _returnvalue) (`KismetSystemLibrary.LineTraceSingle` (`local.Actor`) (+ (`local.ActorLocation`) (* (`KismetMathLibrary.GreaterGreater_VectorRotator` (`local.InnerAngle_Local`) (`KismetMathLibrary.MakeRotator` 0.0 0.0 (* _index (/ (`local.InnerAngle`) (`local.LineNum`))))) (`local.InnerDistance`))) (+ (`local.ActorLocation`) (* (`KismetMathLibrary.GreaterGreater_VectorRotator` (`local.OuterAngle_Local`) (`KismetMathLibrary.MakeRotator` 0.0 0.0 (* _index (/ (`local.OuterAngle`) (`local.LineNum`))))) (`local.OuterDistance`))) "TraceTypeQuery3" false (`local.ActorsIgnore`) "ForOneFrame"))
    (if _returnvalue
      (`KismetArrayLibrary.Array_AddUnique` (`local.HitResults`) _outhit)))
  (return _hitresults (`KismetArrayLibrary.Array_IsNotEmpty` _hitresults)))
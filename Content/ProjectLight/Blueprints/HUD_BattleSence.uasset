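; Battle scene HUD that creates the battle overlay widget on begin play and controls the inventory and upgrade menus.
; The inventory action toggles its menu, passing the player character's inventory component when first creating the widget.
; The upgrade action opens or closes its menu from a boolean, refreshing the upgrade items when an existing menu is shown again.
; Both menus are created lazily, then reused by switching visibility, with flags tracking their open state.
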(event `self.ReceiveBeginPlay`
  (bind _returnvalue (`|CreateWidget` "/Game/ProjectLight/UMG/UMG_HUD_Battle.UMG_HUD_Battle_C"))
  (bind _output_get (set `self.BattleHUD` _returnvalue))
  (`UserWidget.AddToViewport` _output_get 0))

(event `InventoryMenuAction`
  (if (`self.HasOpenInventory`)
    (bind _inventorymenu (`self.InventoryMenu`)
      (:`then`
        (`Widget.SetVisibility` _inventorymenu "Collapsed")
        (set `self.HasOpenInventory` false))
      (:`else`))
    (else
      (set `self.HasOpenInventory` true)
      (bind _inventorymenu_2 (`self.InventoryMenu`)
        (:`then`
          (`Widget.SetVisibility` _inventorymenu_2 "Visible"))
        (:`else`
          (bind _inventorycomponent (`/Game/ProjectLight/Blueprints/FunctionLibrary/BML_Common.GetInventoryComponent` (`GameplayStatics.GetPlayerCharacter` 0))
            (:`IsValid`
              (bind _returnvalue (`|CreateWidget` "/Game/ProjectLight/UMG/UMG_InventoryMenu.UMG_InventoryMenu_C" null _inventorycomponent))
              (set `self.InventoryMenu` _returnvalue)
              (`UserWidget.AddToViewport` _returnvalue 0))))))))

(event `UpgradeMenuAction`
  (params (OpenMenu :type Boolean))
  (bind _hasopenupgrade (`self.HasOpenUpgrade`))
  (if OpenMenu
    (if (not _hasopenupgrade)
      (bind _upgrademenu (`self.UpgradeMenu`)
        (:`then`
          (`Widget.SetVisibility` _upgrademenu "Visible")
          (`/Game/ProjectLight/UMG/UMG_UpgradeMenu.UpdateUpgradeItem` _upgrademenu))
        (:`else`
          (bind _returnvalue (`|CreateWidget` "/Game/ProjectLight/UMG/UMG_UpgradeMenu.UMG_UpgradeMenu_C"))
          (bind _output_get (set `self.UpgradeMenu` _returnvalue))
          (`UserWidget.AddToViewport` _output_get 0)))
      (set `self.HasOpenUpgrade` true))
    (elif _hasopenupgrade
      (bind _upgrademenu_2 (`self.UpgradeMenu`)
        (:`then`
          (`Widget.SetVisibility` _upgrademenu_2 "Collapsed")
          (set `self.HasOpenUpgrade` false))
        (:`else`)))))

(fn `UserConstructionScript`)
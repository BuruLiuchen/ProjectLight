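; BP_Prop_Base is a base prop that, when living, can be damaged and broken down into biomass resource pickups.
; BeginPlay varies its biomass by up to 25%, and damage drains health until it hides, disables collision and expires shortly after.
; SpawnResource splits the biomass into BP_Resource_Base actors launched upward in a random cone.
; Destruction triggers a navigation rebuild console command, and the info getters return placeholder defaults.
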(event `self.ReceiveBeginPlay`
  (bind _totalbiomassvalue (`self.TotalBiomassValue`))
  (set `self.TotalBiomassValue` (+ _totalbiomassvalue (`KismetMathLibrary.RandomFloatInRange` (* _totalbiomassvalue -0.25) (* _totalbiomassvalue 0.25)))))

(event `self.ReceiveAnyDamage`
  (params (Damage :type "Float (single-precision)") (DamageType :type "DamageType Object Reference") (InstigatedBy :type "Controller Object Reference") (DamageCauser :type "Actor Object Reference"))
  (if (`self.IsLiving`)
    (`KismetSystemLibrary.PrintString` (`KismetStringLibrary.Conv_DoubleToString` Damage))
    (bind _output_get (set `self.HealthPoint` (`KismetMathLibrary.FClamp` (- (`self.HealthPoint`) Damage) 0.0 (`self.MaxHealthPoint`))))
    (if (<= _output_get 0.0)
      (`self.SetLifeSpan` 0.5)
      (`self.SetActorHiddenInGame` true)
      (`self.SetActorEnableCollision` false)
      (`self.SpawnResource`))))

(event `self.ReceiveDestroyed`
  (`KismetSystemLibrary.ExecuteConsoleCommand` "RebuildNavigation" null))

(fn `GetBuildingType`
  (returns (BuildingType :type "/Game/ProjectLight/Buildings/EBuildingType Enum"))
  (return "NewEnumerator0"))

(fn `GetIsActive`
  (returns (IsActive :type Boolean))
  (return false))

(fn `GetIsLiving`
  (returns (IsLiving :type Boolean))
  (return false))

(fn `GetName`
  (returns (ReturnName :type Name))
  (return "None"))

(fn `GetUnitType`
  (returns (UnitType :type "/Game/ProjectLight/Blueprints/Enums/EUnitType Enum"))
  (return "NewEnumerator1"))

(fn `GetVolumeForDispaly`
  (returns (Volume :type "Float (double-precision)") (MaxVolume :type "Float (double-precision)"))
  (return 0.0 0.0))

(fn `SpawnResource`
  (bind _biomassvaluesingle (`self.BiomassValueSingle`))
  (bind _returnvalue (`KismetMathLibrary.FFloor` (/ (`self.TotalBiomassValue`) _biomassvaluesingle)))
  (for _ (range (+ (`KismetMathLibrary.Clamp` _returnvalue 1 _returnvalue) 1))
    (bind _returnvalue_2 (`|SpawnActorFromClass` "/Game/ProjectLight/Blueprints/BP_Resource_Base.BP_Resource_Base_C" (`KismetMathLibrary.MakeTransform` (`self.K2_GetActorLocation`)) "AdjustIfPossibleButAlwaysSpawn" "MultiplyWithRoot" null (make `/Game/ProjectLight/Components/Struct/FEnergyInfo` "NewEnumerator2" _biomassvaluesingle) null))
    (`/Engine/EditorBlueprintResources/StandardMacros.IsValid` _returnvalue_2
      (:`Is Valid`
        (bind _capsule (`/Game/ProjectLight/Blueprints/BP_Resource_Base.Capsule` _returnvalue_2)
          (:`then`
            (`PrimitiveComponent.AddImpulse` _capsule (* (`KismetMathLibrary.RandomUnitVectorInConeInDegrees` (0.0 0.0 1.0) 45.0) 500.0) "None" true))
          (:`else`))))))

(fn `UserConstructionScript`)
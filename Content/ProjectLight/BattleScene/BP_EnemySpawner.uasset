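; Enemy spawner for the battle stage that registers itself with GM_BattleStage on BeginPlay.
; TryToSpawnEnemy starts a looping timer that spawns named BP_Character_Enemy instances one at a time at random navigable points around the spawner.
; Requests made while busy wait in the SpawnList map, keyed by enemy name, so a repeated name overwrites its queued count.
; Each finished batch fires OnSpawnFInished, which the spawner itself handles to start the next queued entry.
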(event `self.ReceiveBeginPlay`
  (add `self.OnSpawnFInished` (delegate `OnSpawnFInished_Event`))
  (bind _asgm_battle_stage (cast `/Game/ProjectLight/BattleScene/GM_BattleStage` (`GameplayStatics.GetGameMode`)))
  (`KismetArrayLibrary.Array_AddUnique` (`/Game/ProjectLight/BattleScene/GM_BattleStage.EnemySpawners` _asgm_battle_stage) self))

(event `OnSpawnFInished_Event`
  (`self.CheckSpawnList`))

(event `TryToSpawnEnemy`
  (params (EnemyName :type Name) (SpawnNum :type Integer))
  (if (`self.IsSpawning`)
    (`BlueprintMapLibrary.Map_Add` (`self.SpawnList`) EnemyName SpawnNum)
    (else
      (set `self.Enemy Name` EnemyName)
      (set `self.IsSpawning` true)
      (set `self.SpawnNum` SpawnNum)
      (set `self.NumHasSpawn` 0)
      (bind _returnvalue (`KismetSystemLibrary.K2_SetTimerDelegate` (delegate `SpawnEnemy`) 0.5 true))
      (set `self.SpwanTimer` _returnvalue))))

(event `SpawnEnemy`
  (bind _randomlocation (`NavigationSystemV1.K2_GetRandomLocationInNavigableRadius` (`self.K2_GetActorLocation`) 200.0 null null))
  (`|SpawnActorFromClass` "/Game/ProjectLight/Characters/Enemy/BP_Character_Enemy.BP_Character_Enemy_C" (`KismetMathLibrary.MakeTransform` _randomlocation) "Undefined" "MultiplyWithRoot" null (`self.Enemy Name`) null)
  (bind _output_get (set `self.NumHasSpawn` (+ (`self.NumHasSpawn`) 1)))
  (if (>= _output_get (`self.SpawnNum`))
    (set `self.IsSpawning` false)
    (`KismetSystemLibrary.K2_ClearAndInvalidateTimerHandle` (`self.SpwanTimer`))
    (`self.OnSpawnFInished`)))

(fn `CheckSpawnList`
  (locals (EnemyName_Local :type Name))
  (bind _spawnlist (`self.SpawnList`))
  (if (`BlueprintMapLibrary.Map_IsNotEmpty` _spawnlist)
    (bind _keys (`BlueprintMapLibrary.Map_Keys` _spawnlist))
    (bind _output_get (set `local.EnemyName_Local` (`|GetArrayItem` _keys)))
    (`self.TryToSpawnEnemy` _output_get (`BlueprintMapLibrary.Map_Find` (`self.SpawnList`) _output_get))
    (`BlueprintMapLibrary.Map_Remove` (`self.SpawnList`) (`local.EnemyName_Local`))))

(fn `UserConstructionScript`)
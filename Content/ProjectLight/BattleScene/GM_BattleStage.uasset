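; Battle stage game mode that runs the day/night cycle, feeding sunlight energy to units by day and spawning enemies at night.
; Timings and light power come from DT_DayTime, and looping timers advance the day, pitch the directional light and send energy to registered BPI_Energy units.
; Sun power rises linearly to midday and falls toward dusk, scaling both pitch and energy.
; Night pauses those timers and periodically spawns zombies at random spawners until day resumes.
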(event `self.ReceiveBeginPlay`
  (`self.UpdateDayTimeInfo` "NormalDay")
  (`self.ChangeGamePhase` (struct :`TagName` "Gameplay.Phase.Day"))
  (bind _returnvalue (`GameplayStatics.GetActorOfClass` "/Script/Engine.DirectionalLight"))
  (set `self.SunLight` _returnvalue)
  (set `self.SpendDayTime` (* (`self.DayTime`) 0.3))
  (bind _returnvalue_2 (`KismetSystemLibrary.K2_SetTimerDelegate` (`|CreateDelegate` :!event `SpreadLight`) (`self.SpreadInterval`) true true))
  (set `self.SunLigthTimer` _returnvalue_2)
  (bind _returnvalue_3 (`KismetSystemLibrary.K2_SetTimerDelegate` (`|CreateDelegate` :!event `DayToNight`) (`self.TimeInterval`) true true))
  (set `self.IntoNightTimer` _returnvalue_3))

(event `SpreadLight`
  (if (`KismetArrayLibrary.Array_IsNotEmpty` (`self.UnitsNeedLight`))
    (for _array_element (`self.UnitsNeedLight`)
      (`/Engine/EditorBlueprintResources/StandardMacros.IsValid` _array_element
        (:`Is Valid`
          (message `/Game/ProjectLight/Components/Interfaces/BPI_Energy.EnergyPass_UDP` _array_element (make `/Game/ProjectLight/Components/Struct/FEnergyInfo` "NewEnumerator0" (* (* (`self.LightPower`) (`self.SpreadInterval`)) (`self.GetSunPower`))) "NewEnumerator0"))))))

(event `DayToNight`
  (bind _sunlight (`self.SunLight`))
  (bind (_returnvalue_roll _returnvalue_pitch _returnvalue_yaw) (`KismetMathLibrary.BreakRotator` (`self.K2_GetActorRotation` _sunlight)))
  (bind _output_get (set `self.SpendDayTime` (+ (`self.SpendDayTime`) (`self.TimeInterval`))))
  (if (>= _output_get (`self.DayTime`))
    (`/Game/ProjectLight/Blueprints/FunctionLibrary/BPL_Common.PauseTimer` (`self.IntoNightTimer`) self)
    (`/Game/ProjectLight/Blueprints/FunctionLibrary/BPL_Common.PauseTimer` (`self.SunLigthTimer`) self)
    (`self.ChangeGamePhase` (struct :`TagName` "Gameplay.Phase.Night"))
    (`self.NightProcess`)
    ;[1 1 1] NightTime
    (bind _returnvalue (`KismetSystemLibrary.K2_SetTimerDelegate` (delegate `NightToDay`) (`self.NightTime`)))
    (set `self.IntoDayTimer` _returnvalue)
    (else
      (`self.K2_SetActorRotation` _sunlight (`KismetMathLibrary.MakeRotator` _returnvalue_roll (`KismetMathLibrary.Lerp` 4.0 -60.0 (`self.GetSunPower`)) _returnvalue_yaw) false))))

(event `NightToDay`
  ;[1 1 1] NightTime
  (set `self.SpendDayTime` 0.0)
  (`/Game/ProjectLight/Blueprints/FunctionLibrary/BPL_Common.UnpauseTimer` (`self.IntoNightTimer`) self)
  (`/Game/ProjectLight/Blueprints/FunctionLibrary/BPL_Common.UnpauseTimer` (`self.SunLigthTimer`) self)
  (`self.ChangeGamePhase` (struct :`TagName` "Gameplay.Phase.Day")))

(event `SpawnEnemy`
  (params (EnemyName :type Name) (EnemyNum :type Integer))
  (bind _outitem (`KismetArrayLibrary.Array_Random` (`self.EnemySpawners`)))
  (`/Engine/EditorBlueprintResources/StandardMacros.IsValid` _outitem
    (:`Is Valid`
      (`/Game/ProjectLight/BattleScene/BP_EnemySpawner.TryToSpawnEnemy` _outitem EnemyName EnemyNum))))

(fn `ChangeGamePhase`
  (params (NewGamePhase :type "GameplayTag Structure"))
  (bind _output_get (set `self.GamePhase` NewGamePhase))
  (if (`BlueprintGameplayTagLibrary.MatchesTag` _output_get (struct :`TagName` "Gameplay.Phase.Day"))
    (`KismetSystemLibrary.K2_ClearAndInvalidateTimerHandle` (`self.EnemySpawnTimer`))))

(fn `GetSunPower`
  (returns (ReturnValue :type "Float (double-precision)"))
  (bind _spenddaytime (`self.SpendDayTime`))
  (return (/ (select `bool` (>= (`self.SpendDayTime`) (/ (`self.DayTime`) 2.0)) :`false` _spenddaytime :`true` (- (`self.DayTime`) _spenddaytime)) (/ (`self.DayTime`) 2.0))))

(fn `NightProcess`
  (bind _returnvalue (`KismetSystemLibrary.K2_SetTimerDelegate` (`|CreateDelegate` :!event `SpwanEnemyByData`) 10.0 true))
  (set `self.EnemySpawnTimer` _returnvalue))

(fn `RegisterToUnitList`
  (params (NewUnit :type "Actor Object Reference"))
  (if (`KismetSystemLibrary.DoesImplementInterface` NewUnit "/Game/ProjectLight/Components/Interfaces/BPI_Energy.BPI_Energy_C")
    (`KismetArrayLibrary.Array_AddUnique` (`self.UnitsNeedLight`) NewUnit)))

(fn `SpwanEnemyByData`
  (`self.SpawnEnemy` "Zombie" 5))

(fn `UpdateDayTimeInfo`
  (params (Name :type Name))
  (bind _returnvalue (`|GetDataTableRow` "/Game/ProjectLight/BattleScene/Data/DT_DayTime.DT_DayTime" Name)
    (:`then`
      (bind (_daytime _lightpower _nighttime) (break `/Game/ProjectLight/BattleScene/Struct/FDayTimeInfo` _returnvalue))
      (set `self.DayTime` _daytime)
      (set `self.LightPower` _lightpower)
      (set `self.NightTime` _nighttime))))

(fn `UserConstructionScript`)